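; Stage 02 fire hazard trigger that lets the black hole ability switch linked fires on or off.
; When a BP_BlackHole_ForAbility begins overlapping the Trigger component, it loops through the TargetBP array and inverts each element's Fire state through FireOn or FireOff.
; A FlipFlop sits inside the loop, but both of its branches run the same check, so it has no effect on the result.
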(event OnComponentBeginOverlap(Trigger)
  (params (OverlappedComponent :type Primitive%20Component%20Object%20Reference) (OtherActor :type Actor%20Object%20Reference) (OtherComp :type Primitive%20Component%20Object%20Reference) (OtherBodyIndex :type Integer) (bFromSweep :type Boolean) (SweepResult :type Hit%20Result%20Structure%20%28by%20ref%29))
  (Utilities|Casting|CastToBP_BlackHole_ForAbility OtherActor)
  (for _array_element (Variables|Default|GetTargetBP)
    (Utilities|FlowControl|FlipFlop
      (:A
        (if (Variables|/Game/01_Blueprint/InteractiveObject/BP_Firehazard.BP_Firehazard_C|GetFire _array_element)
          (Default|FireOff _array_element)
          (else
            (Default|Fireon _array_element))))
      (:B
        (if (Variables|/Game/01_Blueprint/InteractiveObject/BP_Firehazard.BP_Firehazard_C|GetFire _array_element)
          (Default|FireOff _array_element)
          (else
            (Default|Fireon _array_element)))))))

(fn ConstructionScript)