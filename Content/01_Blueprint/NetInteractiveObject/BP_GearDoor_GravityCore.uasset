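; Networked gear puzzle door that opens when a BP_Gear_GravityCore actor enters its trigger.
; The server destroys that gear and sets GearAttached, whose RepNotify reveals the fitted gear and button mesh, changes audio and raises the door through a timeline.
; Tick always rotates two gear meshes and turns the rest of the train once the gear is attached.
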(event OnComponentBeginOverlap(Trigger)
  (params (OverlappedComponent :type Primitive%20Component%20Object%20Reference) (OtherActor :type Actor%20Object%20Reference) (OtherComp :type Primitive%20Component%20Object%20Reference) (OtherBodyIndex :type Integer) (bFromSweep :type Boolean) (SweepResult :type Hit%20Result%20Structure%20%28by%20ref%29))
  (Networking|SwitchHasAuthority
    (:Authority
      (bind _asbp_gear_gravity_core (Utilities|Casting|CastToBP_Gear_GravityCore OtherActor)
        (:then
          (Variables|Default|SetGearAttached true)
          (Actor|DestroyActor _asbp_gear_gravity_core))
        (:CastFailed
          (Development|PrintString "Hello"))))))

(event Custom|PlayGearAttachedFX
  (Rendering|SetVisibility (Variables|Default|Get1_button_science) true false)
  (Rendering|SetVisibility (Variables|Default|GetGearVisible) true false)
  (Variables|Default|SetDoorLoc (Transformation|GetRelativeTransform (Variables|Default|GetDoorMesh1)))
  (Audio|PlaySoundatLocation "/Game/40_Audio/03_SFX/MetaSounds/Objects/MS_SFX_Cardboard_Puzzle_Solved_01.MS_SFX_Cardboard_Puzzle_Solved_01" "0, 0, 0" "0, 0, 0" 1.0 1.0 0.0 0 0 0 0)
  (Audio|Components|Audio|SetSound (Variables|Default|GetAudio) "/Game/40_Audio/03_SFX/MetaSounds/Objects/MS_SFX_Cardboard_Puzzle_02.MS_SFX_Cardboard_Puzzle_02")
  (bind _lerp (Timeline|Timeline_1 Play)
    (:Update
      (Transformation|SetRelativeLocation (Variables|Default|GetDoorMesh1) (Math|Vector|MakeVector 0.0 -83.8 (.z (.location (Math|Transform|Lerp(Transform) (Variables|Default|GetDoorLoc) (Math|Transform|MakeTransform (Math|Vector|MakeVector 0.0 0.0 7e+02) "0, 0, 0" "1.000000,1.000000,1.000000") _lerp)))) false false))))

(event EventBeginPlay
  (Audio|Components|Audio|SetSound (Variables|Default|GetAudio) "/Game/40_Audio/03_SFX/MetaSounds/Objects/MS_SFX_Cardboard_Puzzle_01.MS_SFX_Cardboard_Puzzle_01"))

(event Collision|EventActorBeginOverlap
  (params (OtherActor :type Actor%20Object%20Reference)))

(event EventTick
  (params (DeltaSeconds :type Float%20%28single-precision%29))
  (Transformation|AddLocalRotation (Variables|Default|GetGearMesh1) "0.000000,1.000000,0.000000" false false)
  (Transformation|AddLocalRotation (Variables|Default|GetGearMesh) "0.000000,1.000000,0.000000" false false)
  (if (Variables|Default|GetGearAttached)
    (Transformation|AddLocalRotation (Variables|Default|GetGearMesh) "0.000000,1.000000,0.000000" false false)
    (Transformation|AddLocalRotation (Variables|Default|GetGearMesh2) "0.000000,1.000000,0.000000" false false)
    (Transformation|AddLocalRotation (Variables|Default|GetGearMesh4) "0.000000,1.000000,0.000000" false false)
    (Transformation|AddLocalRotation (Variables|Default|GetGearVisible) "0.000000,-1.000000,0.000000" false false)
    (Transformation|AddLocalRotation (Variables|Default|GetGearMesh6) "0.000000,0.000000,-1.000000" false false)
    (Transformation|AddLocalRotation (Variables|Default|GetGearMesh5) "0.000000,0.000000,-1.000000" false false)))

(fn ConstructionScript)

(fn OnRepGearAttached
  (if (Variables|Default|GetGearAttached)
    (CallFunction|PlayGearAttachedFX)))