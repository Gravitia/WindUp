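; BP_MeshRepeatBH is a Stage 2 interactive object that switches between an on mesh and an off mesh, making the on mesh solid or passable.
; BeginPlay sets mesh visibility and MeshOn collision from the initial IsVisible flag; MeshOff collision is never changed.
; VisiblityOn and VisiblityOff, which have no caller in this Blueprint, switch the state only when it differs and print a debug message.
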(event Custom|VisiblityOn
  (if (not (Variables|Default|GetIsVisible))
    (Rendering|SetVisibility (Variables|Default|GetMeshOff) false false)
    (Rendering|SetVisibility (Variables|Default|GetMeshOn) true false)
    (Collision|SetCollisionEnabled (Variables|Default|GetMeshOn) "QueryAndPhysics")
    (Variables|Default|SetIsVisible true)
    (Development|PrintString "비지빌리티 ON !@@!@#!@#!@#@!#!@#!@")))

(event Custom|VisiblityOff
  (if (Variables|Default|GetIsVisible)
    (Rendering|SetVisibility (Variables|Default|GetMeshOff) true false)
    (Rendering|SetVisibility (Variables|Default|GetMeshOn) false false)
    (Collision|SetCollisionEnabled (Variables|Default|GetMeshOn) "NoCollision")
    (Variables|Default|SetIsVisible false)
    (Development|PrintString "비지빌리티 OFF !@@!@#!@#!@#@!#!@#!@")))

(event EventBeginPlay
  (if (Variables|Default|GetIsVisible)
    (Rendering|SetVisibility (Variables|Default|GetMeshOff) false false)
    (Rendering|SetVisibility (Variables|Default|GetMeshOn) true false)
    (Collision|SetCollisionEnabled (Variables|Default|GetMeshOn) "QueryAndPhysics")
    (else
      (Rendering|SetVisibility (Variables|Default|GetMeshOff) true false)
      (Rendering|SetVisibility (Variables|Default|GetMeshOn) false false)
      (Collision|SetCollisionEnabled (Variables|Default|GetMeshOn) "NoCollision"))))

(fn ConstructionScript)