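; BP_UpPlatform is a Stage 02 interactive platform that moves its mesh when a BP_GravityCoreBattery is placed in its capsule.
; A battery entering an otherwise battery-free capsule snaps to the Cylinder's location, and after a short delay its PropNumber selects one of three timelines and target vectors.
; A battery leaving runs another timeline back to the relative origin.
; Each timeline lerps from the mesh's current relative location.
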(event OnComponentBeginOverlap(Capsule)
  (params (OverlappedComponent :type Primitive%20Component%20Object%20Reference) (OtherActor :type Actor%20Object%20Reference) (OtherComp :type Primitive%20Component%20Object%20Reference) (OtherBodyIndex :type Integer) (bFromSweep :type Boolean) (SweepResult :type Hit%20Result%20Structure%20%28by%20ref%29))
  (bind _asbp_gravity_core_battery (Utilities|Casting|CastToBP_GravityCoreBattery OtherActor))
  (if (== (Utilities|Array|Length (Collision|GetOverlappingActors (Variables|Default|GetCapsule) "/Game/01_Blueprint/InteractiveObject/Stage02_Objects/BP_GravityCoreBattery.BP_GravityCoreBattery_C" :!class /Script/Engine.PrimitiveComponent)) 1)
    (Transformation|SetActorRelativeLocation _asbp_gravity_core_battery (Transformation|GetWorldLocation (Variables|Default|GetCylinder)))
    (Utilities|FlowControl|Delay 1.0)
    (switch int (Variables|/Game/01_Blueprint/InteractiveObject/Stage02_Objects/BP_GravityCoreBattery.BP_GravityCoreBattery_C|GetProp%20Number _asbp_gravity_core_battery)
      (:0
        (bind _newtrack_0 (Timeline|Move01 PlayFromStart)
          (:Update
            (Transformation|SetRelativeLocation (Variables|Default|GetStaticMesh) (Math|Vector|Lerp(Vector) (Variables|/Script/Engine.SceneComponent|GetRelativeLocation (Variables|Default|GetStaticMesh)) (Variables|Default|GetVector01) _newtrack_0) false false))))
      (:1
        (bind _newtrack_0_2 (Timeline|Move02 PlayFromStart)
          (:Update
            (Transformation|SetRelativeLocation (Variables|Default|GetStaticMesh) (Math|Vector|Lerp(Vector) (Variables|/Script/Engine.SceneComponent|GetRelativeLocation (Variables|Default|GetStaticMesh)) (Variables|Default|GetVector02) _newtrack_0_2) false false))))
      (:2
        (bind _newtrack_0_3 (Timeline|Move03 PlayFromStart)
          (:Update
            (Transformation|SetRelativeLocation (Variables|Default|GetStaticMesh) (Math|Vector|Lerp(Vector) (Variables|/Script/Engine.SceneComponent|GetRelativeLocation (Variables|Default|GetStaticMesh)) (Variables|Default|GetVector03) _newtrack_0_3) false false)))))))

(event OnComponentEndOverlap(Capsule)
  (params (OverlappedComponent :type Primitive%20Component%20Object%20Reference) (OtherActor :type Actor%20Object%20Reference) (OtherComp :type Primitive%20Component%20Object%20Reference) (OtherBodyIndex :type Integer))
  (Utilities|Casting|CastToBP_GravityCoreBattery OtherActor)
  (bind _newtrack_0 (Timeline|Timeline PlayFromStart)
    (:Update
      (Transformation|SetRelativeLocation (Variables|Default|GetStaticMesh) (Math|Vector|Lerp(Vector) (Variables|/Script/Engine.SceneComponent|GetRelativeLocation (Variables|Default|GetStaticMesh)) "0, 0, 0" _newtrack_0) false false))))

(event EventBeginPlay)

(event Collision|EventActorBeginOverlap
  (params (OtherActor :type Actor%20Object%20Reference)))

(event EventTick
  (params (DeltaSeconds :type Float%20%28single-precision%29)))

(fn ConstructionScript)