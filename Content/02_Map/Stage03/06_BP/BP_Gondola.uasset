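; BP_Gondola is a Stage03 gondola that travels along a spline once a player triggers it.
; The first BP_CharacterPlayer overlap with TriggerBox sets a one-time flag, then starts GondolaTimeline after a short delay.
; Timeline alpha scales the spline length, passes through a vector-distance node, and samples the local spline position used to move GondolaMesh without sweeping.
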(event OnComponentBeginOverlap(TriggerBox)
  (params (OverlappedComponent :type Primitive%20Component%20Object%20Reference) (OtherActor :type Actor%20Object%20Reference) (OtherComp :type Primitive%20Component%20Object%20Reference) (OtherBodyIndex :type Integer) (bFromSweep :type Boolean) (SweepResult :type Hit%20Result%20Structure%20%28by%20ref%29))
  (Utilities|Casting|CastToBP_CharacterPlayer OtherActor)
  (if (not (Variables|Default|GetbHasStarted))
    (Variables|Default|SetbHasStarted true)
    (Utilities|FlowControl|Delay 2.0)
    (bind _alpha (Timeline|GondolaTimeline Play)
      (:Update
        (Transformation|SetRelativeLocation (Variables|Default|GetGondolaMesh) (Spline|GetLocationatDistanceAlongSpline (Variables|Default|GetSpline) (Math|Vector|Distance(Vector) (* (Spline|GetSplineLength (Variables|Default|GetSpline)) _alpha) "0, 0, 0") "Local") false false)))))

(event EventBeginPlay)

(event Collision|EventActorBeginOverlap
  (params (OtherActor :type Actor%20Object%20Reference)))

(event EventTick
  (params (DeltaSeconds :type Float%20%28single-precision%29)))

(fn ConstructionScript)