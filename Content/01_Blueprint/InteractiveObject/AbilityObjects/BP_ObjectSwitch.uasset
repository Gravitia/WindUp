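; BP_ObjectSwitch is an interactive switch that toggles the visibility of a target mesh object.
; Its Trigger responds only to BP_CustomGObject_04 actors, on both begin and end overlap.
; Each event checks whether TargetMesh is visible and calls its VisiblityOff or VisiblityOn function to flip that state, so leaving the trigger toggles it again.
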(event OnComponentBeginOverlap(Trigger)
  (params (OverlappedComponent :type Primitive%20Component%20Object%20Reference) (OtherActor :type Actor%20Object%20Reference) (OtherComp :type Primitive%20Component%20Object%20Reference) (OtherBodyIndex :type Integer) (bFromSweep :type Boolean) (SweepResult :type Hit%20Result%20Structure%20%28by%20ref%29))
  (bind _targetmesh (Variables|Default|GetTargetMesh))
  (Utilities|Casting|CastToBP_CustomGObject_04 OtherActor)
  (if (Variables|/Game/01_Blueprint/InteractiveObject/BP_SwitchToggleMesh_01.BP_SwitchToggleMesh_01_C|GetIsVisible _targetmesh)
    (Default|VisiblityOff _targetmesh)
    (else
      (Default|Visiblityon _targetmesh))))

(event OnComponentEndOverlap(Trigger)
  (params (OverlappedComponent :type Primitive%20Component%20Object%20Reference) (OtherActor :type Actor%20Object%20Reference) (OtherComp :type Primitive%20Component%20Object%20Reference) (OtherBodyIndex :type Integer))
  (bind _targetmesh (Variables|Default|GetTargetMesh))
  (Utilities|Casting|CastToBP_CustomGObject_04 OtherActor)
  (if (Variables|/Game/01_Blueprint/InteractiveObject/BP_SwitchToggleMesh_01.BP_SwitchToggleMesh_01_C|GetIsVisible _targetmesh)
    (Default|VisiblityOff _targetmesh)
    (else
      (Default|Visiblityon _targetmesh))))

(fn ConstructionScript)