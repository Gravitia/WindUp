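; Volume actor for the EasySaveGameUI system that pauses auto saves while the player character is inside its box.
; After a short delay on BeginPlay, it caches the SaveGameOperationsManager and checks for characters already overlapping the box.
; Begin overlap shares that check, storing the player character and pausing auto saves through the manager.
; End overlap resumes auto saves when that stored actor leaves.
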(event OnComponentBeginOverlap(Box)
  (params (OverlappedComponent :type Primitive%20Component%20Object%20Reference) (OtherActor :type Actor%20Object%20Reference) (OtherComp :type Primitive%20Component%20Object%20Reference) (OtherBodyIndex :type Integer) (bFromSweep :type Boolean) (SweepResult :type Hit%20Result%20Structure%20%28by%20ref%29))
  (CallFunction|SetVariablesandDisableAutoSaves OtherActor))

(event OnComponentEndOverlap(Box)
  (params (OverlappedComponent :type Primitive%20Component%20Object%20Reference) (OtherActor :type Actor%20Object%20Reference) (OtherComp :type Primitive%20Component%20Object%20Reference) (OtherBodyIndex :type Integer))
  (if (== OtherActor (Variables|Components|GetOverlappedActor))
    (Default|PauseorResumeAutoSaves (Variables|Default|GetSaveGameOperationsManager) false)))

(event EventBeginPlay
  (Utilities|FlowControl|Delay 0.2)
  (Variables|Default|SetSaveGameOperationsManager (CallFunction|GetSaveGameOperationsManager))
  (for _array_element (Collision|GetOverlappingActors (Variables|Default|GetBox) "/Script/Engine.Character" :!class /Script/Engine.PrimitiveComponent)
    (CallFunction|SetVariablesandDisableAutoSaves _array_element)))

(fn ConstructionScript)

(fn SetVariablesandDisableAutoSaves
  (params (InActor :type Actor%20Object%20Reference))
  (if (== InActor (Game|GetPlayerCharacter 0))
    (Variables|Components|SetOverlappedActor InActor)
    (Default|PauseorResumeAutoSaves (Variables|Default|GetSaveGameOperationsManager) true)))