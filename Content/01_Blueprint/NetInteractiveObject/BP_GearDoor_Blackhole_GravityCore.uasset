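; Networked gear-puzzle door that opens once both a Gravity Core gear and a Black Hole gear are inserted.
; Server-side trigger overlaps destroy the delivered gear and set replicated flags, whose OnReps reveal the mounted gear and button mesh.
; With both attached, a timeline raises the door and puzzle audio changes.
; Tick spins the gear train progressively as gears attach, deriving steps from server world time to stay synchronized.
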(event OnComponentBeginOverlap(GravityCore_Trigger)
  (params (OverlappedComponent :type Primitive%20Component%20Object%20Reference) (OtherActor :type Actor%20Object%20Reference) (OtherComp :type Primitive%20Component%20Object%20Reference) (OtherBodyIndex :type Integer) (bFromSweep :type Boolean) (SweepResult :type Hit%20Result%20Structure%20%28by%20ref%29))
  (Networking|SwitchHasAuthority
    (:Authority
      (bind _asbp_gear_gravity_core (Utilities|Casting|CastToBP_Gear_GravityCore OtherActor))
      (Variables|Default|SetGravityCore_GearAttached true)
      (Actor|DestroyActor _asbp_gear_gravity_core))))

(event OnComponentBeginOverlap(BlackHole_Trigger)
  (params (OverlappedComponent :type Primitive%20Component%20Object%20Reference) (OtherActor :type Actor%20Object%20Reference) (OtherComp :type Primitive%20Component%20Object%20Reference) (OtherBodyIndex :type Integer) (bFromSweep :type Boolean) (SweepResult :type Hit%20Result%20Structure%20%28by%20ref%29))
  (Networking|SwitchHasAuthority
    (:Authority
      (bind _asbp_gear_blackhole (Utilities|Casting|CastToBP_Gear_Blackhole OtherActor))
      (Variables|Default|SetBlackHole_GearAttached true)
      (Actor|DestroyActor _asbp_gear_blackhole))))

(event Custom|PlayGravityCoreAttachedFX
  (Rendering|SetVisibility (Variables|Default|GetGravityCore_GearVisible) true false)
  (Rendering|SetVisibility (Variables|Default|Get1_button_science) true false)
  (if (Variables|Default|GetBlackHole_GearAttached)
    (if (Variables|Default|GetGravityCore_GearAttached)
      (Variables|Default|SetDoorLoc (Transformation|GetRelativeTransform (Variables|Default|GetDoorMesh1)))
      (Audio|PlaySoundatLocation "/Game/40_Audio/03_SFX/MetaSounds/Objects/MS_SFX_Cardboard_Puzzle_Solved_01.MS_SFX_Cardboard_Puzzle_Solved_01" "0, 0, 0" "0, 0, 0" 1.0 1.0 0.0 0 0 0 0)
      (Audio|Components|Audio|SetSound (Variables|Default|GetAudio) "/Game/40_Audio/03_SFX/MetaSounds/Objects/MS_SFX_Cardboard_Puzzle_02.MS_SFX_Cardboard_Puzzle_02")
      (bind _lerp (Timeline|Timeline_1 Play)
        (:Update
          (Transformation|SetRelativeLocation (Variables|Default|GetDoorMesh1) (Math|Vector|MakeVector 0.0 -83.8 (.z (.location (Math|Transform|Lerp(Transform) (Variables|Default|GetDoorLoc) (Math|Transform|MakeTransform (Math|Vector|MakeVector 0.0 0.0 7e+02) "0, 0, 0" "1.000000,1.000000,1.000000") _lerp)))) false false))))))

(event Custom|PlayBlackHoleAttachedFX
  (Rendering|SetVisibility (Variables|Default|GetBlackHole_GearVisible) true false)
  (Rendering|SetVisibility (Variables|Default|Get1_button_magic) true false)
  (if (Variables|Default|GetBlackHole_GearAttached)
    (if (Variables|Default|GetGravityCore_GearAttached)
      (Variables|Default|SetDoorLoc (Transformation|GetRelativeTransform (Variables|Default|GetDoorMesh1)))
      (Audio|PlaySoundatLocation "/Game/40_Audio/03_SFX/MetaSounds/Objects/MS_SFX_Cardboard_Puzzle_Solved_01.MS_SFX_Cardboard_Puzzle_Solved_01" "0, 0, 0" "0, 0, 0" 1.0 1.0 0.0 0 0 0 0)
      (Audio|Components|Audio|SetSound (Variables|Default|GetAudio) "/Game/40_Audio/03_SFX/MetaSounds/Objects/MS_SFX_Cardboard_Puzzle_02.MS_SFX_Cardboard_Puzzle_02")
      (bind _lerp (Timeline|Timeline_1 Play)
        (:Update
          (Transformation|SetRelativeLocation (Variables|Default|GetDoorMesh1) (Math|Vector|MakeVector 0.0 -83.8 (.z (.location (Math|Transform|Lerp(Transform) (Variables|Default|GetDoorLoc) (Math|Transform|MakeTransform (Math|Vector|MakeVector 0.0 0.0 7e+02) "0, 0, 0" "1.000000,1.000000,1.000000") _lerp)))) false false))))))

(event EventBeginPlay
  (Audio|Components|Audio|SetSound (Variables|Default|GetAudio) "/Game/40_Audio/03_SFX/MetaSounds/Objects/MS_SFX_Cardboard_Puzzle_01.MS_SFX_Cardboard_Puzzle_01"))

(event Collision|EventActorBeginOverlap
  (params (OtherActor :type Actor%20Object%20Reference)))

(event EventTick
  (params (DeltaSeconds :type Float%20%28single-precision%29))
  (bind (_spinyaw _spinyawinv _spinrollinv) (CallFunction|UpdateGearSpin))
  (Transformation|AddLocalRotation (Variables|Default|Get11_GearMesh) _spinyaw false false)
  (if (Variables|Default|GetGravityCore_GearAttached)
    (Transformation|AddLocalRotation (Variables|Default|GetGravityCore_GearVisible) _spinyawinv false false)
    (Transformation|AddLocalRotation (Variables|Default|Get13_GearMesh) _spinyaw false false)
    (if (Variables|Default|GetBlackHole_GearAttached)
      (Transformation|AddLocalRotation (Variables|Default|Get14_GearMesh) _spinyaw false false)
      (Transformation|AddLocalRotation (Variables|Default|GetBlackHole_GearVisible) _spinyawinv false false)
      (Transformation|AddLocalRotation (Variables|Default|Get16_GearMesh) _spinrollinv false false))))

(fn ConstructionScript)

(fn OnRepBlackHoleGearAttached
  (if (Variables|Default|GetBlackHole_GearAttached)
    (CallFunction|PlayBlackHoleAttachedFX)))

(fn OnRepGravityCoreGearAttached
  (if (Variables|Default|GetGravityCore_GearAttached)
    (CallFunction|PlayGravityCoreAttachedFX)))

(fn UpdateGearSpin
  (Variables|Default|SetGearSpinStep (- (* (Math|Float|MakeLiteralFloat 6e+01) (GameState|GetServerWorldTimeSeconds (Game|GetGameState))) (Variables|Default|GetGearSpinAccum)))
  (Variables|Default|SetGearSpinAccum (+ (Variables|Default|GetGearSpinAccum) (Variables|Default|GetGearSpinStep)))
  (return (Math|Rotator|MakeRotator 0.0 0.0 (Variables|Default|GetGearSpinStep)) (Math|Rotator|MakeRotator 0.0 0.0 (- 0.0 (Variables|Default|GetGearSpinStep))) (Math|Rotator|MakeRotator (- 0.0 (Variables|Default|GetGearSpinStep)) 0.0 0.0)))