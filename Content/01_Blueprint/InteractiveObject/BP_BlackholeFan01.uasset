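; Interactive fan obstacle that spins around its yaw axis and opens its blocking collision when a black hole ability actor enters its trigger.
; Tick applies the frame-time-scaled rotation speed, which two timelines drive.
; Trigger entry plays the first timeline, whose updates set the speed and disable blocking.
; Trigger exit waits a short delay, restores full blocking, then plays the second timeline to change the speed again.
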(event OnComponentBeginOverlap(Trigger)
  (params (OverlappedComponent :type Primitive%20Component%20Object%20Reference) (OtherActor :type Actor%20Object%20Reference) (OtherComp :type Primitive%20Component%20Object%20Reference) (OtherBodyIndex :type Integer) (bFromSweep :type Boolean) (SweepResult :type Hit%20Result%20Structure%20%28by%20ref%29))
  (Utilities|Casting|CastToBP_BlackHole_ForAbility OtherActor)
  (bind _newtrack_3 (Timeline|Timeline Play)
    (:Update
      (Variables|Default|SetRotation%20Speed _newtrack_3)
      (Collision|SetCollisionEnabled (Variables|Default|GetBlocking) "NoCollision"))))

(event OnComponentEndOverlap(Trigger)
  (params (OverlappedComponent :type Primitive%20Component%20Object%20Reference) (OtherActor :type Actor%20Object%20Reference) (OtherComp :type Primitive%20Component%20Object%20Reference) (OtherBodyIndex :type Integer))
  (bind _blocking (Variables|Default|GetBlocking))
  (Utilities|Casting|CastToBP_BlackHole_ForAbility OtherActor)
  (Utilities|FlowControl|Delay 3.0)
  (Collision|SetCollisionEnabled _blocking "QueryAndPhysics")
  (Collision|SetCollisionResponsetoAllChannels _blocking "ECR_Block")
  (bind _newtrack_3 (Timeline|Timeline_0 Play)
    (:Update
      (Variables|Default|SetRotation%20Speed _newtrack_3))))

(event EventTick
  (params (DeltaSeconds :type Float%20%28single-precision%29))
  (Transformation|AddActorLocalRotation (Math|Rotator|MakeRotator 0.0 0.0 (* DeltaSeconds (Variables|Default|GetRotation%20Speed))) false false))

(fn ConstructionScript)