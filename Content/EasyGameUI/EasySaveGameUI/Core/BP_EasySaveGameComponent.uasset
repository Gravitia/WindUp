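; Actor component that makes its owner saveable in the EasySaveGame system by registering the actor, and optionally its destruction, with the game instance.
; SaveOrLoadVariables round-trips a JSON string holding component settings, the actor transform (optionally keyed by level name) and custom variables exchanged through a dispatcher.
; Restoring component settings re-triggers registration.
; It can relay the operations manager's save/load start and end events, and pull stored persistent-actor data on request.
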(event Custom|RetriggerRegistration
  ;[1 0.5587 0.2081] Init + Registration
  (|InitialRegistration)
  (Variables|Default|SetRegistered? true))

(event EventBeginPlay
  ;[1 0.5587 0.2081] Init + Registration
  (|GetBaseActorInfos)
  (Utilities|FlowControl|DelayUntilNextTick)
  (|SaveGameOperationEventsBinding)
  (if (not (Variables|Default|GetRegistered?))
    (|InitialRegistration)
    (Variables|Default|SetRegistered? true)))

(event EventEndPlay
  (params (EndPlayReason :type EEndPlayReason%20Enum :default "Destroyed"))
  ;[0.5436 1 0.3684] Destruction Registration
  (if (and (Utilities|Enum|Equal(Enum) EndPlayReason "Destroyed") (Variables|EasyConfig|GetRegisterDestruction?))
    (if (|CheckIfRequireNewGUID)
      (|DestructionRegistrationWithNewGUID)
      (else
        (|DestructionRegistration)))
    (Variables|Default|SetRegistered? true)))

(fn RequestLoadVariables
  (if (and (Utilities|Enum|Equal(Enum) (Variables|EasyConfig|GetActorSaveType) "NewEnumerator0") (not (Variables|EasyConfig|GetRegisterDestruction?)))
    (bind _output_get (LocalVariables|SetSaveGameOprationsManager (CallFunction|GetSaveGameOperationsManager)))
    (if (and (Variables|/Game/EasyGameUI/EasySaveGameUI/Core/BP_EasySaveGameOperationsManager.BP_EasySaveGameOperationsManager_C|GetWorldInitialized? _output_get) (not (Variables|/Game/EasyGameUI/EasySaveGameUI/Core/BP_EasySaveGameOperationsManager.BP_EasySaveGameOperationsManager_C|GetIsSavingOrLoading? _output_get)))
      (CallFunction|SaveorLoadVariables "NewEnumerator1" (.Value (Utilities|Map|Find (Variables|/Game/EasyGameUI/EasySaveGameUI/Core/BP_EasySaveGameOperationsManager.BP_EasySaveGameOperationsManager_C|GetPersistentActors _output_get) (Variables|Default|GetOwnerActorRef)))))))

(fn SaveorLoadVariables
  (params (OperationType :type E_SaveGameOperationType%20Enum :default "NewEnumerator0") (SavedVariables :type String))
  (switch Utilities|FlowControl|Switch|SwitchonE_SaveGameOperationType OperationType
    (:NewEnumerator0
      ;[1 0 0.243] Save Actor
      (bind _outjsonobject (Class|JsonBlueprintFunctionLibrary|FromString "{}")) ; Load an empty JSON to clear all variables
      (Variables|Default|SetJsonObject _outjsonobject)
      (Utilities|FlowControl|Sequence
        (:then_0
          (|SaveOrLoadComponentState :!label _label))
        (:then_1
          (|SaveVariables)
          (|SaveTransform)
          (bind _outjsonstring (Class|JsonBlueprintFunctionLibrary|ToString (Variables|Default|GetJsonObject)))
          (return (Variables|Default|GetOwnerActorRef) _outjsonstring (Variables|Default|GetActorUniqueID)))))
    (:NewEnumerator1
      ;[0 1 0.1932] Load Actor
      (bind _outjsonobject_2 (Class|JsonBlueprintFunctionLibrary|FromString SavedVariables))
      (Variables|Default|SetJsonObject _outjsonobject_2)
      (Utilities|FlowControl|Sequence
        (:then_0
          (goto _label))
        (:then_1
          (|LoadTransform)
          (|LoadVariables))))))

(event Custom|SaveGameOperationStarted_Event
  (params (Operation :type S%20Save%20Operation%20Infos%20Structure))
  (Default|CallSaveGameOperationStarted Operation))

(event Custom|SaveGameOperationEnded_Event
  (params (Operation :type S%20Save%20Operation%20Infos%20Structure))
  (Default|CallSaveGameOperationEnded Operation))