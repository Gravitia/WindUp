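; Interactive lift that takes a gravity core battery and moves to the level selected by that battery's PropNumber.
; A lone battery overlapping the capsule has its gravity mesh component disabled, is attached to the battery slot, and triggers the matching montage and keyed movement.
; If its number differs from the lift's, after a delay the montage plays in reverse, the battery is released and the lift returns to its initial state.
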(event OnComponentBeginOverlap(Capsule)
  (params (OverlappedComponent :type Primitive%20Component%20Object%20Reference) (OtherActor :type Actor%20Object%20Reference) (OtherComp :type Primitive%20Component%20Object%20Reference) (OtherBodyIndex :type Integer) (bFromSweep :type Boolean) (SweepResult :type Hit%20Result%20Structure%20%28by%20ref%29))
  (bind _2_lift_sk (Variables|Default|Get2_lift_SK))
  (bind _returnvalue (Components|SkeletalMesh|GetAnimInstance _2_lift_sk))
  (Components|Timeline|SetPlayRate (Variables|Default|Get2_lift_SK) 1.0)
  (bind _asbp_gravity_core_battery (Utilities|Casting|CastToBP_GravityCoreBattery OtherActor))
  (if (== (Utilities|Array|Length (Collision|GetOverlappingActors (Variables|Default|GetCapsule) "/Game/01_Blueprint/InteractiveObject/Stage02_Objects/BP_GravityCoreBattery.BP_GravityCoreBattery_C" :!class /Script/Engine.PrimitiveComponent)) 1)
    (Variables|Default|SetComponentMeshAffected (Actor|GetComponentbyClass _asbp_gravity_core_battery "/Script/ChronoSpace.CSMeshAffectedByGravityCore"))
    (Class|CSMeshAffectedbyGravityCore|SetEnable (Actor|GetComponentbyClass _asbp_gravity_core_battery "/Script/ChronoSpace.CSMeshAffectedByGravityCore") false)
    (bind _returnvalue_2 (Class|CSActorAttachmentComponent|AttachActortoSlot (Variables|Default|GetActorAttachment) "battery" _asbp_gravity_core_battery))
    (if _returnvalue_2
      (switch int (Variables|/Game/01_Blueprint/InteractiveObject/Stage02_Objects/BP_GravityCoreBattery.BP_GravityCoreBattery_C|GetProp%20Number _asbp_gravity_core_battery)
        (:Default
          _)
        (:0
          (Animation|Montage|MontagePlay _returnvalue "/Game/21_Animation/Prop/CH2/Lift/IdleToL1_Montage.IdleToL1_Montage" 1.0 "MontageLength" 0.0 true)
          (Variables|Default|SetLastMontage "/Game/21_Animation/Prop/CH2/Lift/IdleToL1_Montage.IdleToL1_Montage"))
        (:1
          (Animation|Montage|MontagePlay _returnvalue "/Game/21_Animation/Prop/CH2/Lift/IdleToL2_Montage.IdleToL2_Montage" 1.0 "MontageLength" 0.0 true)
          (Variables|Default|SetLastMontage "/Game/21_Animation/Prop/CH2/Lift/IdleToL2_Montage.IdleToL2_Montage"))
        (:2
          (Animation|Montage|MontagePlay _returnvalue "/Game/21_Animation/Prop/CH2/Lift/IdleToL3_Montage.IdleToL3_Montage" 1.0 "MontageLength" 0.0 true)
          (Variables|Default|SetLastMontage "/Game/21_Animation/Prop/CH2/Lift/IdleToL3_Montage.IdleToL3_Montage")))
      (Class|CSTransformMover|PlayMovement (Utilities|String|StringToName (Utilities|String|ToString(Integer) (Variables|/Game/01_Blueprint/InteractiveObject/Stage02_Objects/BP_GravityCoreBattery.BP_GravityCoreBattery_C|GetProp%20Number _asbp_gravity_core_battery))))
      (if (== (Variables|Default|GetpropNumber) (Variables|/Game/01_Blueprint/InteractiveObject/Stage02_Objects/BP_GravityCoreBattery.BP_GravityCoreBattery_C|GetProp%20Number _asbp_gravity_core_battery))
        (Development|PrintString "Up Platform Success")
        (else
          (Utilities|FlowControl|Delay (Variables|Default|Getdelay))
          (Animation|Montage|MontagePlay (Components|SkeletalMesh|GetAnimInstance (Variables|Default|Get2_lift_SK)) (Variables|Default|GetLastMontage) -1.0 "MontageLength" 1.667 true)
          (Class|CSActorAttachmentComponent|DetachActorfromSlot (Variables|Default|GetActorAttachment) "Battery")
          (Class|CSMeshAffectedbyGravityCore|SetEnable (Variables|Default|GetComponentMeshAffected) true)
          (Class|CSTransformMover|ReturntoInitial))))))

(event Custom|OnMovementStarted_Event
  (params (MovementKey :type Name)))

(fn ConstructionScript)