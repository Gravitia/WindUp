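; BP_CollapsePlatform_02 is an interactive platform that tilts as if collapsing when a Character enters its triggers.
; Trigger1 and Trigger2 each fire once, each playing its own timeline that drives the StaticMesh's relative roll.
; Every timeline update also starts a camera shake for players 0 and 1.
; When the second timeline finishes, the mesh snaps to a fixed world-space roll.
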(event OnComponentBeginOverlap(Trigger1)
  (params (OverlappedComponent :type Primitive%20Component%20Object%20Reference) (OtherActor :type Actor%20Object%20Reference) (OtherComp :type Primitive%20Component%20Object%20Reference) (OtherBodyIndex :type Integer) (bFromSweep :type Boolean) (SweepResult :type Hit%20Result%20Structure%20%28by%20ref%29))
  (Utilities|Casting|CastToCharacter OtherActor)
  (Utilities|FlowControl|DoOnce false
    (:Completed
      (bind _newtrack_1 (Timeline|Timeline01 Play)
        (:Update
          (Transformation|SetRelativeRotation (Variables|Default|GetStaticMesh) (Math|Rotator|MakeRotator (.x _newtrack_1) 0.0 0.0) false false)
          (CameraShakes|StartCameraShake (Game|GetPlayerCameraManager 0) "/Game/01_Blueprint/Camera/BP_CameraShake.BP_CameraShake_C" 1.0 "CameraLocal" "0, 0, 0")
          (CameraShakes|StartCameraShake (Game|GetPlayerCameraManager 1) "/Game/01_Blueprint/Camera/BP_CameraShake.BP_CameraShake_C" 1.0 "CameraLocal" "0, 0, 0"))))))

(event OnComponentBeginOverlap(Trigger2)
  (params (OverlappedComponent :type Primitive%20Component%20Object%20Reference) (OtherActor :type Actor%20Object%20Reference) (OtherComp :type Primitive%20Component%20Object%20Reference) (OtherBodyIndex :type Integer) (bFromSweep :type Boolean) (SweepResult :type Hit%20Result%20Structure%20%28by%20ref%29))
  (Utilities|Casting|CastToCharacter OtherActor)
  (Utilities|FlowControl|DoOnce false
    (:Completed
      (bind _newtrack_0 (Timeline|Timeline02 Play)
        (:Update
          (Transformation|SetRelativeRotation (Variables|Default|GetStaticMesh) (Math|Rotator|MakeRotator (.x _newtrack_0) 0.0 0.0) false false)
          (CameraShakes|StartCameraShake (Game|GetPlayerCameraManager 0) "/Game/01_Blueprint/Camera/BP_CameraShake.BP_CameraShake_C" 1.0 "CameraLocal" "0, 0, 0")
          (CameraShakes|StartCameraShake (Game|GetPlayerCameraManager 1) "/Game/01_Blueprint/Camera/BP_CameraShake.BP_CameraShake_C" 1.0 "CameraLocal" "0, 0, 0"))
        (:Finished
          (Transformation|SetWorldRotation (Variables|Default|GetStaticMesh) (Math|Rotator|MakeRotator 15.0 0.0 0.0) false false))))))

(fn ConstructionScript)