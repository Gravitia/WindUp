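; Trigger volume that starts a save in a new slot of its save type when the player character enters it.
; If a save or load is running at BeginPlay, it waits for completion; a player found inside must exit before it can fire.
; It can disable itself after one activation, persisting that state through its EasySaveGame component and restoring disabled collision on load.
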(event OnComponentBeginOverlap(Box)
  (params (OverlappedComponent :type Primitive%20Component%20Object%20Reference) (OtherActor :type Actor%20Object%20Reference) (OtherComp :type Primitive%20Component%20Object%20Reference) (OtherBodyIndex :type Integer) (bFromSweep :type Boolean) (SweepResult :type Hit%20Result%20Structure%20%28by%20ref%29))
  (if (Math|Boolean|ANDBoolean (== OtherActor (Game|GetPlayerCharacter 0)) (not (Variables|Default|GetActivated?)) (Variables|Default|GetCanTrigger?))
    (bind _saveuniquename (CallFunction|FindAvailableIndexforSaveType (Variables|EasyConfig|GetSaveType) 99))
    (Class|BPIEGUIGameInstanceInterface|StartSaveGameOperation(Message) (Game|GetGameInstance) (Utilities|Struct|MakeS_SaveOperationInfos _saveuniquename "NewEnumerator0" "NewEnumerator0" false) false (Variables|EasyConfig|GetForceSaveOperation?))
    (if (Variables|EasyConfig|GetDisableAfterActivation?)
      (Variables|Default|SetActivated? true)
      (Collision|SetCollisionEnabled (Variables|Default|GetBox) "NoCollision"))))

(event OnComponentEndOverlap(Box)
  (params (OverlappedComponent :type Primitive%20Component%20Object%20Reference) (OtherActor :type Actor%20Object%20Reference) (OtherComp :type Primitive%20Component%20Object%20Reference) (OtherBodyIndex :type Integer))
  (if (and (== OtherActor (Game|GetPlayerCharacter 0)) (Variables|Default|GetWaitForPlayerToExit?))
    (Variables|Default|SetCanTrigger? true)
    (Variables|Default|SetWaitForPlayerToExit? false)))

(event LoadingorSavingVariables(BP_EasySaveGameComponent)
  (params (OperationType :type E_SaveGameOperationType%20Enum :default "NewEnumerator0") (JsonObject :type Json%20Object%20Wrapper%20Structure))
  (bind _loadedvalue (Utilities|SaveorLoadVariable OperationType JsonObject "Activation" (Variables|Default|GetActivated?))
    (:Loaded
      (bind _output_get (Variables|Default|SetActivated? _loadedvalue))
      (if _output_get
        (Collision|SetCollisionEnabled (Variables|Default|GetBox) "NoCollision")))))

(event Custom|LoadEnded
  (params (Operation :type S%20Save%20Operation%20Infos%20Structure))
  (EventDispatchers|UnbindEventfromSaveGameOperationEnded (CallFunction|GetSaveGameOperationsManager) (delegate Custom|LoadEnded))
  (|CheckIfPlayerHasSpawnedInsidetheVolume))

(event EventBeginPlay
  (bind _savegameoperationmanager (CallFunction|GetSaveGameOperationsManager))
  (Utilities|FlowControl|DelayUntilNextTick)
  (if (Variables|/Game/EasyGameUI/EasySaveGameUI/Core/BP_EasySaveGameOperationsManager.BP_EasySaveGameOperationsManager_C|GetIsSavingOrLoading? _savegameoperationmanager)
    (Variables|Default|SetCanTrigger? false)
    (EventDispatchers|BindEventtoSaveGameOperationEnded _savegameoperationmanager (delegate Custom|LoadEnded))
    (else
      (Variables|Default|SetCanTrigger? true))))

(fn ConstructionScript
  (Variables|/Game/EasyGameUI/EasySaveGameUI/Core/BP_EasySaveGameComponent.BP_EasySaveGameComponent_C|SetHasVariablesToSave? (Variables|Default|GetBP_EasySaveGameComponent) (Variables|EasyConfig|GetDisableAfterActivation?)))