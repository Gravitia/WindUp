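; BP_GravityTowerWater is a water hazard, apparently for a gravity tower, that damages the player character on overlap.
; On overlap with BP_CharacterPlayer, it applies the BPGE_GravityTowerWaterDamage gameplay effect to that player's ability system component.
; It then disables its static mesh collision and a timer restores query-only collision half a second later, so the overlap can fire again as a repeating damage tick.
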(event EventBeginPlay)

(event Collision|EventActorBeginOverlap
  (params (OtherActor :type Actor%20Object%20Reference))
  (bind _asbp_character_player (Utilities|Casting|CastToBP_CharacterPlayer OtherActor))
  (bind _returnvalue (Spec|MakeSpecHandle(ByClass) "/Game/01_Blueprint/GA/GE/BPGE_GravityTowerWaterDamage.BPGE_GravityTowerWaterDamage_C" 0))
  (GameplayEffects|ApplyGameplayEffectSpecToTarget (Variables|Default|GetAbilitySystem) _returnvalue (Ability|GetAbilitySystemComponent _asbp_character_player))
  (CallFunction|Reactivate))

(event EventTick
  (params (DeltaSeconds :type Float%20%28single-precision%29)))

(fn ConstructionScript)

(fn Reactivate
  (Collision|SetCollisionEnabled (Variables|Default|GetStaticMesh) "NoCollision")
  (Utilities|Time|SetTimerbyFunctionName 0 "Activate" 0.5))

(fn Activate
  (Collision|SetCollisionEnabled (Variables|Default|GetStaticMesh) "QueryOnly"))