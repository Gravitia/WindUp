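; Spawner actor that records a referenced actor's starting transform and can return that actor to it on demand.
; BeginPlay caches the transform of the SpawnActor reference as SpawnPoint, and RespawnActor teleports the same actor back to that location and rotation.
; It moves the existing instance rather than creating a new one; the spawn and relative-transform nodes are left unconnected.
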(event Custom|RespawnActor
  (bind _spawnpoint (Variables|Default|GetSpawnPoint))
  (Transformation|Teleport (Variables|Default|GetSpawnActor) (.location _spawnpoint) (.rotation _spawnpoint)))

(event EventBeginPlay
  (Variables|Default|SetSpawnPoint (Transformation|GetActorTransform (Variables|Default|GetSpawnActor))))

(fn ConstructionScript)