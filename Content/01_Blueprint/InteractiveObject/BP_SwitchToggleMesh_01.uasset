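; BP_SwitchToggleMesh_01 is an interactive object that swaps between an "on" mesh and an "off" mesh.
; BeginPlay applies the initial state from IsVisible, enabling collision on MeshOn only when it is shown; MeshOff collision is never changed.
; VisiblityOn and VisiblityOff flip the meshes and IsVisible, each behind its own DoOnce that only RESET_ON or RESET_OFF re-arms.
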(event Custom|VisiblityOn
  (Utilities|FlowControl|DoOnce false
    (:Completed
      (if (not (Variables|Default|GetIsVisible))
        (Rendering|SetVisibility (Variables|Default|GetMeshOff) false false)
        (Rendering|SetVisibility (Variables|Default|GetMeshOn) true false)
        (Collision|SetCollisionEnabled (Variables|Default|GetMeshOn) "QueryAndPhysics")
        (Variables|Default|SetIsVisible true)))))

(event Custom|VisiblityOff
  (Utilities|FlowControl|DoOnce false
    (:Completed
      (if (Variables|Default|GetIsVisible)
        (Rendering|SetVisibility (Variables|Default|GetMeshOff) true false)
        (Rendering|SetVisibility (Variables|Default|GetMeshOn) false false)
        (Collision|SetCollisionEnabled (Variables|Default|GetMeshOn) "NoCollision")
        (Variables|Default|SetIsVisible false)))))

(event Custom|RESET_OFF
  (Utilities|FlowControl|DoOnce false) ; enters at Reset
)

(event Custom|RESET_ON
  (Utilities|FlowControl|DoOnce false) ; enters at Reset
)

(event EventBeginPlay
  (if (Variables|Default|GetIsVisible)
    (Rendering|SetVisibility (Variables|Default|GetMeshOff) false false)
    (Rendering|SetVisibility (Variables|Default|GetMeshOn) true false)
    (Collision|SetCollisionEnabled (Variables|Default|GetMeshOn) "QueryAndPhysics")
    (else
      (Rendering|SetVisibility (Variables|Default|GetMeshOff) true false)
      (Rendering|SetVisibility (Variables|Default|GetMeshOn) false false)
      (Collision|SetCollisionEnabled (Variables|Default|GetMeshOn) "NoCollision"))))

(fn ConstructionScript)