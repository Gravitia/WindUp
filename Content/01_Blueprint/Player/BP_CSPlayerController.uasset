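; BP_CSPlayerController is a player controller that manages the main menu widget.
; On BeginPlay it creates WBP_MenuMain for player 0, adds it to the viewport and keeps a reference to it.
; The M key toggles that same widget between visible and hidden, tracking the state in a MenuOpened flag.
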(event EventBeginPlay
  (bind _returnvalue (UserInterface|CreateWidget "/Game/MENU_GRAPHICS/Widgets/WBP_MenuMain.WBP_MenuMain_C" (Game|GetPlayerController 0)))
  (UserInterface|Viewport|AddtoViewport _returnvalue 0)
  (Variables|Default|SetMenuMainObject _returnvalue))

(event EventTick
  (params (DeltaSeconds :type Float%20%28single-precision%29)))

(event Input|KeyboardEvents|M
  (params (Key :type Key%20Structure :default "None"))
  (:Pressed
    (if (Variables|Default|GetbMenuOpened)
      (Widget|SetVisibility (Variables|Default|GetMenuMainObject) "Hidden")
      (Variables|Default|SetbMenuOpened false)
      (else
        (Widget|SetVisibility (Variables|Default|GetMenuMainObject) "Visible")
        (Variables|Default|SetbMenuOpened true)))))

(fn ConstructionScript)