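; Black hole pair switch, a puzzle object that toggles a linked TargetMesh's visibility when it and its PairSwitch are both active.
; Only BP_BlackHole_ForAbility overlaps activate its trigger.
; If the target is flagged DoOnce, completing the pair disables both triggers' collision.
; Otherwise, ending an overlap deactivates the switch and toggles the mesh again, whatever the partner's state.
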(event OnComponentBeginOverlap(Trigger)
  (params (OverlappedComponent :type Primitive%20Component%20Object%20Reference) (OtherActor :type Actor%20Object%20Reference) (OtherComp :type Primitive%20Component%20Object%20Reference) (OtherBodyIndex :type Integer) (bFromSweep :type Boolean) (SweepResult :type Hit%20Result%20Structure%20%28by%20ref%29))
  (bind _targetmesh (Variables|Default|GetTargetMesh))
  (Utilities|Casting|CastToBP_BlackHole_ForAbility OtherActor)
  (Variables|Components|SetIsActivate true)
  (if (and (Variables|Components|GetIsActivate) (Variables|/Game/01_Blueprint/InteractiveObject/AbilityObjects/BP_GravityCoreSwitch_Pair.BP_GravityCoreSwitch_Pair_C|GetIsActivate (Variables|Default|GetPairSwitch)))
    (Utilities|FlowControl|Delay 0.0)
    (if (Rendering|IsVisible (Variables|/Game/01_Blueprint/InteractiveObject/BP_SwitchToggleMesh_01.BP_SwitchToggleMesh_01_C|GetMeshOn _targetmesh))
      (Default|VisiblityOff _targetmesh)
      (else
        (Default|Visiblityon _targetmesh)))
    (if (Variables|/Game/01_Blueprint/InteractiveObject/BP_SwitchToggleMesh_01.BP_SwitchToggleMesh_01_C|GetDo%20once? (Variables|Default|GetTargetMesh))
      (Collision|SetCollisionEnabled (Variables|Default|GetTrigger) "NoCollision"))))

(event OnComponentEndOverlap(Trigger)
  (params (OverlappedComponent :type Primitive%20Component%20Object%20Reference) (OtherActor :type Actor%20Object%20Reference) (OtherComp :type Primitive%20Component%20Object%20Reference) (OtherBodyIndex :type Integer))
  (bind _targetmesh (Variables|Default|GetTargetMesh))
  (Utilities|Casting|CastToBP_BlackHole_ForAbility OtherActor)
  (if (not (Variables|/Game/01_Blueprint/InteractiveObject/BP_SwitchToggleMesh_01.BP_SwitchToggleMesh_01_C|GetDo%20once? (Variables|Default|GetTargetMesh)))
    (Variables|Components|SetIsActivate false)
    (if (not (Variables|Components|GetIsActivate))
      (if (Variables|/Game/01_Blueprint/InteractiveObject/AbilityObjects/BP_GravityCoreSwitch_Pair.BP_GravityCoreSwitch_Pair_C|GetIsActivate (Variables|Default|GetPairSwitch))
        _
        (else
          _))
      (if (Rendering|IsVisible (Variables|/Game/01_Blueprint/InteractiveObject/BP_SwitchToggleMesh_01.BP_SwitchToggleMesh_01_C|GetMeshOn _targetmesh))
        (Default|VisiblityOff _targetmesh)
        (else
          (Default|Visiblityon _targetmesh))))))

(fn ConstructionScript)