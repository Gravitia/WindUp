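; Lobby player controller that sets up the lobby screen for the local player.
; On BeginPlay it creates and stores the EOS lobby widget, enables the cursor with Game and UI input, and switches the view to the first actor tagged "Cine".
; A timeline applies a subtle pitch offset to that actor around its starting rotation.
; OnSwitchLobbyWidget forwards to the widget's game start button handler.
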(event EventBeginPlay
  (bind _returnvalue (Game|GetPlayerController 0))
  (if (Pawn|IsLocalController)
    (bind _returnvalue_2 (UserInterface|CreateWidget "/Game/01_Blueprint/UI/Main/WBP_EOSLobby.WBP_EOSLobby_C"))
    (bind _asbp_cslobby_player_controller (Utilities|Casting|CastToBP_CSLobbyPlayerController (Game|GetPlayerController 0)))
    (Variables|BP_CSLobbyPlayerController_C|SetLobbyWidgetRef _asbp_cslobby_player_controller _returnvalue_2)
    (UserInterface|Viewport|AddtoViewport _returnvalue_2 0)
    (Input|SetInputModeGameandUI _returnvalue _returnvalue_2 "DoNotLock" true false)
    (Variables|/Script/Engine.PlayerController|SetbShowMouseCursor _returnvalue true)
    (Variables|Default|SetbFindCameraComponentWhenViewTarget true)
    (bind _outactors (Actor|GetAllActorswithTag "Cine"))
    (Game|Player|SetViewTargetwithBlend (Game|GetPlayerController 0) (Utilities|Array|Get(acopy) _outactors) 0.0 "VTBlend_Linear" 0.0 false)
    (Variables|Default|SetBaseRotation (Transformation|GetActorRotation (Utilities|Array|Get(acopy) _outactors)))
    (bind _output (Timeline|Timeline PlayFromStart)
      (:Update
        (Transformation|SetActorRotation (Utilities|Array|Get(acopy) _outactors) (Math|Rotator|MakeRotator (.roll (Variables|Default|GetBaseRotation)) (+ (Math|Float|Lerp 0.1 -0.1 _output) (.pitch (Variables|Default|GetBaseRotation))) (.yaw (Variables|Default|GetBaseRotation))))))))

(event EventTick
  (params (DeltaSeconds :type Float%20%28single-precision%29)))

(event EventOnSwitchLobbyWidget
  (params (NewIndex :type Integer))
  (Default|OnClickGameStartButton (Variables|Default|GetLobbyWidgetRef)))

(fn ConstructionScript)