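; BP_MeshOnce01 is a Stage 2 interactive object that swaps between an "on" mesh and an "off" mesh.
; The construction script uses IsVisible to set the starting mesh visibility and enables collision on MeshOn only when it is shown.
; VisiblityOn and VisiblityOff events perform the swap and print debug text.
; Both check IsVisible without updating it, so only the change away from the starting state takes effect.
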(event Custom|VisiblityOn
  (if (not (Variables|Default|GetIsVisible))
    (Rendering|SetVisibility (Variables|Default|GetMeshOff) false false)
    (Rendering|SetVisibility (Variables|Default|GetMeshOn) true false)
    (Collision|SetCollisionEnabled (Variables|Default|GetMeshOn) "QueryAndPhysics")
    (Development|PrintString "비지빌리티 ON !@@!@#!@#!@#@!#!@#!@")))

(event Custom|VisiblityOff
  (if (Variables|Default|GetIsVisible)
    (Rendering|SetVisibility (Variables|Default|GetMeshOff) true false)
    (Rendering|SetVisibility (Variables|Default|GetMeshOn) false false)
    (Collision|SetCollisionEnabled (Variables|Default|GetMeshOn) "NoCollision")
    (Development|PrintString "비지빌리티 OFF !@@!@#!@#!@#@!#!@#!@")))

(event EventBeginPlay)

(fn ConstructionScript
  (if (Variables|Default|GetIsVisible)
    (Rendering|SetVisibility (Variables|Default|GetMeshOff) false false)
    (Rendering|SetVisibility (Variables|Default|GetMeshOn) true false)
    (Collision|SetCollisionEnabled (Variables|Default|GetMeshOn) "QueryAndPhysics")
    (else
      (Rendering|SetVisibility (Variables|Default|GetMeshOff) true false)
      (Rendering|SetVisibility (Variables|Default|GetMeshOn) false false)
      (Collision|SetCollisionEnabled (Variables|Default|GetMeshOn) "NoCollision"))))