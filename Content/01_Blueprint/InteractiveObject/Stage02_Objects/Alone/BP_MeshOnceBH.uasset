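; Interactive Stage 02 object that swaps between two meshes, MeshOn and MeshOff, when its reactor trigger changes.
; An active trigger shows MeshOff and hides MeshOn with collision disabled; an inactive one reverses this, restoring MeshOn's query and physics collision.
; The construction script calls the same event with the inverse of IsVisible to set the initial state.
; Both branches set Used and print debug text, and nothing here checks Used.
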(event EventOnReactorTriggerChanged
  (params (bActive :type Boolean))
  (if bActive
    (Rendering|SetVisibility (Variables|Default|GetMeshOff) true false)
    (Rendering|SetVisibility (Variables|Default|GetMeshOn) false false)
    (Collision|SetCollisionEnabled (Variables|Default|GetMeshOn) "NoCollision")
    (Variables|Default|SetUsed? true)
    (Development|PrintString "비지빌리티 OFF !@@!@#!@#!@#@!#!@#!@")
    (else
      (Rendering|SetVisibility (Variables|Default|GetMeshOff) false false)
      (Rendering|SetVisibility (Variables|Default|GetMeshOn) true false)
      (Collision|SetCollisionEnabled (Variables|Default|GetMeshOn) "QueryAndPhysics")
      (Variables|Default|SetUsed? true)
      (Development|PrintString "비지빌리티 ON !@@!@#!@#!@#@!#!@#!@"))))

(event EventBeginPlay)

(fn ConstructionScript
  (if (Variables|Default|GetIsVisible)
    (CallFunction|OnReactorTriggerChanged false)
    (else
      (CallFunction|OnReactorTriggerChanged true))))