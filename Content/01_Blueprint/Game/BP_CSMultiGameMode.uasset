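; Game mode for local multiplayer that spawns and removes additional local players at runtime.
; BeginPlay creates a local player with its own controller, without storing a reference to it.
; AdjustPlayer acts as a toggle: it removes Player2Controller and its pawn if valid.
; Otherwise it switches the default pawn to BPC_CharacterPlayer_02 and creates players for active platform users lacking a controller, storing the last as Player2Controller.
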(event Custom|AdjustPlayer
  (bind _player2controller (Variables|Default|GetPlayer2Controller)
    (:then
      (Class|GameplayStatics|RemovePlayer _player2controller true))
    (:else
      (Variables|Default|SetDefaultPawnClass "/Game/01_Blueprint/Character/BPC_CharacterPlayer_02.BPC_CharacterPlayer_02_C")
      (bind _outusers (Class|InputDeviceLibrary|GetAllActiveUsers))
      (for _array_element _outusers
        (Utilities|IsValid (Class|GameplayStatics|GetPlayerControllerfromPlatformUser _array_element)
          (:Is%20Not%20Valid
            (bind _returnvalue (Class|GameplayStatics|CreatePlayerfromPlatformUser _array_element))
            (Variables|Default|SetPlayer2Controller _returnvalue)))))))

(event EventBeginPlay
  (Class|GameplayStatics|CreatePlayer -1))

(fn ConstructionScript)