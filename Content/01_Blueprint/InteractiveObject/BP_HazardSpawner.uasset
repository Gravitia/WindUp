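; Server-authoritative spawner that fills a box area with randomly rotated and scaled hazard actors of a configurable class.
; Spawning runs on BeginPlay if its CSProgressActivatable starts active, or when Activate fires.
; Two overlap areas recycle BP_BlackholeHazard_01 actors by teleporting them to their initial state.
; After Deactivate sets a flag, those areas destroy the hazards instead, so they drain as they arrive.
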(event OnComponentBeginOverlap(Destroy_Area01)
  (params (OverlappedComponent :type Primitive%20Component%20Object%20Reference) (OtherActor :type Actor%20Object%20Reference) (OtherComp :type Primitive%20Component%20Object%20Reference) (OtherBodyIndex :type Integer) (bFromSweep :type Boolean) (SweepResult :type Hit%20Result%20Structure%20%28by%20ref%29))
  (Networking|SwitchHasAuthority
    (:Authority
      (bind _asbp_blackhole_hazard_01 (Utilities|Casting|CastToBP_BlackholeHazard_01 OtherActor))
      (if (Variables|Default|GetbDeactivated)
        (Actor|DestroyActor _asbp_blackhole_hazard_01)
        (Development|PrintString "Deestroy")
        (else
          (Default|TeleporttoInit _asbp_blackhole_hazard_01))))))

(event OnComponentBeginOverlap(Destroy_Area02)
  (params (OverlappedComponent :type Primitive%20Component%20Object%20Reference) (OtherActor :type Actor%20Object%20Reference) (OtherComp :type Primitive%20Component%20Object%20Reference) (OtherBodyIndex :type Integer) (bFromSweep :type Boolean) (SweepResult :type Hit%20Result%20Structure%20%28by%20ref%29))
  (Networking|SwitchHasAuthority
    (:Authority
      (bind _asbp_blackhole_hazard_01 (Utilities|Casting|CastToBP_BlackholeHazard_01 OtherActor))
      (if (Variables|Default|GetbDeactivated)
        (Actor|DestroyActor _asbp_blackhole_hazard_01)
        (Development|PrintString "Deestroy")
        (else
          (Default|TeleporttoInit _asbp_blackhole_hazard_01))))))

(event EventActivate
  (params (InstigatorActor :type Actor%20Object%20Reference) (TriggerId :type Name :default "None"))
  (bind _scalemin (Variables|Default|GetScaleMin))
  (bind _scalemax (Variables|Default|GetScaleMax))
  (bind _returnvalue (Math|Random|RandomFloatinRange _scalemin _scalemax))
  (Networking|SwitchHasAuthority
    (:Authority
      (for _index (range 0 (Variables|Default|GetAmount))
        (Game|SpawnActorfromClass (Variables|Default|GetClass) (Math|Transform|MakeTransform (Math|Random|RandomPointinBoundingBox (Transformation|GetWorldLocation (Variables|Default|GetSpawn_Area)) (Components|Box|GetScaledBoxExtent (Variables|Default|GetSpawn_Area))) (Math|Random|RandomRotator false) (Math|Vector|MakeVector _returnvalue _returnvalue _returnvalue)) "Undefined" "MultiplyWithRoot" 0 0)))))

(event EventDeactivate
  (params (InstigatorActor :type Actor%20Object%20Reference) (TriggerId :type Name :default "None"))
  (Variables|Default|SetbDeactivated true))

(event EventBeginPlay
  (bind _scalemin (Variables|Default|GetScaleMin))
  (bind _scalemax (Variables|Default|GetScaleMax))
  (bind _returnvalue (Math|Random|RandomFloatinRange _scalemin _scalemax))
  (Networking|SwitchHasAuthority
    (:Authority
      (if (Variables|/Script/ChronoSpace.CSProgressActivatableComponent|GetbStartActive (Variables|Default|GetCSProgressActivatable))
        (for _index (range 0 (Variables|Default|GetAmount))
          (Game|SpawnActorfromClass (Variables|Default|GetClass) (Math|Transform|MakeTransform (Math|Random|RandomPointinBoundingBox (Transformation|GetWorldLocation (Variables|Default|GetSpawn_Area)) (Components|Box|GetScaledBoxExtent (Variables|Default|GetSpawn_Area))) (Math|Random|RandomRotator false) (Math|Vector|MakeVector _returnvalue _returnvalue _returnvalue)) "Undefined" "MultiplyWithRoot" 0 0))))))

(fn ConstructionScript)