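; BP_RESET is a Stage 02 trigger volume that resets three target objects when the player enters its box.
; On overlap with BP_CharacterPlayer, a sequence moves each target to its stored relative location without sweeping.
; Each branch feeds one shared CollisionEnable call on all three targets, so that call runs three times per trigger.
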(event OnComponentBeginOverlap(Box)
  (params (OverlappedComponent :type Primitive%20Component%20Object%20Reference) (OtherActor :type Actor%20Object%20Reference) (OtherComp :type Primitive%20Component%20Object%20Reference) (OtherBodyIndex :type Integer) (bFromSweep :type Boolean) (SweepResult :type Hit%20Result%20Structure%20%28by%20ref%29))
  (bind _target01 (Variables|Default|GetTarget01))
  (Utilities|Casting|CastToBP_CharacterPlayer OtherActor)
  (Utilities|FlowControl|Sequence
    (:then_0
      (Transformation|SetActorRelativeLocation _target01 (Variables|Default|GetTarget01%20location)))
    (:then_1
      (Transformation|SetActorRelativeLocation (Variables|Default|GetTarget02) (Variables|Default|GetTarget02%20location)))
    (:then_2
      (Transformation|SetActorRelativeLocation (Variables|Default|GetTarget03) (Variables|Default|GetTarget03%20location))))
  (Default|CollisionEnable _target01))

(event EventBeginPlay)

(event Collision|EventActorBeginOverlap
  (params (OtherActor :type Actor%20Object%20Reference)))

(event EventTick
  (params (DeltaSeconds :type Float%20%28single-precision%29)))

(fn ConstructionScript)