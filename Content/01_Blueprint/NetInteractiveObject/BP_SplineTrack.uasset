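; BP_SplineTrack is a visual track actor that builds itself along an editable spline in the construction script, with no runtime logic.
; It places a scaled end-cap mesh at both spline ends.
; Spline length divided by the mesh's Z bounds sets the number of Z-forward spline mesh segments, floored with a minimum of one.
; Segments take tangents from the spline and share material and scale; all generated meshes have collision disabled.
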(event EventBeginPlay)

(event Collision|EventActorBeginOverlap
  (params (OtherActor :type Actor%20Object%20Reference)))

(event EventTick
  (params (DeltaSeconds :type Float%20%28single-precision%29)))

(fn ConstructionScript
  (bind _spline (Variables|Default|GetSpline))
  (bind _endcapmesh (Variables|Default|GetEndCapMesh))
  (bind _endcapscale (Variables|Default|GetEndCapScale))
  (bind _mesh (Variables|Default|GetMesh))
  (bind _meshscale (Variables|Default|GetMeshScale))
  (bind _returnvalue (StaticMesh|GetBoundingBox _mesh))
  (bind _returnvalue_2 (Spline|GetSplineLength _spline))
  (bind _returnvalue_3 (Math|Vector|MakeVector _endcapscale _endcapscale _endcapscale))
  (bind (_min _max) (Utilities|Struct|BreakBox _returnvalue))
  (bind _returnvalue_4 (- _max _min))
  (bind _z (Math|Vector|BreakVector _returnvalue_4))
  (Spline|UpdateSpline _spline)
  (bind _returnvalue_5 (AddComponent|AddStaticMeshComponent false (Math|Transform|MakeTransform (Spline|GetLocationatDistanceAlongSpline _spline 0.0 "Local") "0, 0, 0" _returnvalue_3)))
  (Components|StaticMesh|SetStaticMesh _returnvalue_5 _endcapmesh)
  (Collision|SetCollisionEnabled _returnvalue_5 "NoCollision")
  (bind _returnvalue_6 (AddComponent|AddStaticMeshComponent false (Math|Transform|MakeTransform (Spline|GetLocationatDistanceAlongSpline _spline _returnvalue_2 "Local") "0, 0, 0" _returnvalue_3)))
  (Components|StaticMesh|SetStaticMesh _returnvalue_6 _endcapmesh)
  (Collision|SetCollisionEnabled _returnvalue_6 "NoCollision")
  (Utilities|IsValid _mesh
    (:Is%20Valid
      (for _index (range 0 (- (Math|Integer|Max(Integer) (Math|Float|Floor (/ _returnvalue_2 _z)) 1) (Class|KismetSystemLibrary|MakeLiteralInteger 1)))
        (bind _returnvalue_7 (AddComponent|AddSplineMeshComponent false))
        (Components|StaticMesh|SetStaticMesh _returnvalue_7 _mesh)
        (Rendering|Material|SetMaterial _returnvalue_7 0 (Variables|Default|GetMaterial))
        (SplineMesh|SetForwardAxis _returnvalue_7 "Z" true)
        (SplineMesh|SetStartandEnd _returnvalue_7 (Spline|GetLocationatDistanceAlongSpline _spline (* _index _z) "Local") (* (Spline|GetDirectionatDistanceAlongSpline _spline (* _index _z) "Local") _z) (Spline|GetLocationatDistanceAlongSpline _spline (Math|Float|Min(Float) (* (+ _index (Class|KismetSystemLibrary|MakeLiteralInteger 1)) _z) _returnvalue_2) "Local") (* (Spline|GetDirectionatDistanceAlongSpline _spline (Math|Float|Min(Float) (* (+ _index (Class|KismetSystemLibrary|MakeLiteralInteger 1)) _z) _returnvalue_2) "Local") _z) true :!class /Script/Engine.SplineMeshComponent)
        (SplineMesh|SetStartScale _returnvalue_7 _meshscale true :!class /Script/Engine.SplineMeshComponent)
        (SplineMesh|SetEndScale _returnvalue_7 _meshscale true :!class /Script/Engine.SplineMeshComponent)
        (Collision|SetCollisionEnabled _returnvalue_7 "NoCollision")))))