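; BP_ActorSpawner is a tool actor that periodically spawns random actors inside a box area and destroys actors that enter a destroy area.
; A looping timer picks a class from an array and spawns it with random location, rotation and per-axis scale while SpawnCondition is false, recording each instance.
; An overlap on the destroy area destroys everything overlapping it.
; Player-proximity toggling, teleport reset and count-limit logic are left unconnected.
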(event OnComponentBeginOverlap(Destroy_Area)
  (params (OverlappedComponent :type Primitive%20Component%20Object%20Reference) (OtherActor :type Actor%20Object%20Reference) (OtherComp :type Primitive%20Component%20Object%20Reference) (OtherBodyIndex :type Integer) (bFromSweep :type Boolean) (SweepResult :type Hit%20Result%20Structure%20%28by%20ref%29))
  (Actor|DestroyActor (Collision|GetOverlappingActors (Variables|Default|GetDestroy_Area) 0 :!class /Script/Engine.PrimitiveComponent)))

(event OnComponentBeginOverlap(PC_Area)
  (params (OverlappedComponent :type Primitive%20Component%20Object%20Reference) (OtherActor :type Actor%20Object%20Reference) (OtherComp :type Primitive%20Component%20Object%20Reference) (OtherBodyIndex :type Integer) (bFromSweep :type Boolean) (SweepResult :type Hit%20Result%20Structure%20%28by%20ref%29)))

(event OnComponentEndOverlap(PC_Area)
  (params (OverlappedComponent :type Primitive%20Component%20Object%20Reference) (OtherActor :type Actor%20Object%20Reference) (OtherComp :type Primitive%20Component%20Object%20Reference) (OtherBodyIndex :type Integer)))

(event Custom|Spawn
  (bind _scalemin (Variables|Default|GetScaleMin))
  (bind _scalemax (Variables|Default|GetScaleMax))
  (bind _returnvalue (Math|Random|RandomFloatinRange _scalemin _scalemax))
  (if (not (Variables|Default|GetSpawnCondition))
    (if true
      (bind _returnvalue_2 (Game|SpawnActorfromClass (.OutItem (Utilities|Array|Random (Variables|Default|GetSpawnActor))) (Math|Transform|MakeTransform (Math|Random|RandomPointinBoundingBox (Transformation|GetWorldLocation (Variables|Default|GetSpawn_Area)) (Components|Box|GetScaledBoxExtent (Variables|Default|GetSpawn_Area))) (Math|Random|RandomRotator false) (Math|Vector|MakeVector _returnvalue _returnvalue _returnvalue)) "AdjustIfPossibleButAlwaysSpawn" "MultiplyWithRoot" 0 0))
      (Variables|Default|SetInitTransform (Transformation|GetActorTransform _returnvalue_2))
      (Utilities|Array|Add (Variables|Default|GetSpawnedActor) _returnvalue_2))))

(event EventBeginPlay
  (Utilities|Time|SetTimerbyEvent (delegate Custom|Spawn) (Variables|Default|GetInterval) true))

(fn ConstructionScript)