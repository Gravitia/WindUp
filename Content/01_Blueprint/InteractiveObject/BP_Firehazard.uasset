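; BP_Firehazard is a fire obstacle that a reactor trigger toggles on or off.
; Each activation flips the Fire flag, switching the Niagara effect, the BP_CSKillZone child actor's active state and Box collision together.
; The construction script sets visibility from Fire but enables the kill zone and collision either way, as its disabling nodes never run.
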(event EventOnReactorTriggerChanged
  (params (bActive :type Boolean))
  (bind _niagara (Variables|Default|GetNiagara))
  (bind _box (Variables|Default|GetBox))
  (bind _killzone1 (Variables|Default|GetKillzone1))
  (bind _childactor (Variables|/Script/Engine.ChildActorComponent|GetChildActor _killzone1))
  (if bActive
    (if (Variables|Default|GetFire)
      (Variables|Default|SetFire false)
      (Rendering|SetVisibility _niagara false false)
      (bind _asbp_cskill_zone (Utilities|Casting|CastToBP_CSKillZone _childactor))
      (Variables|/Script/ChronoSpace.CSKillZone|SetbIsActive _asbp_cskill_zone false)
      (Collision|SetCollisionEnabled _box "NoCollision")
      (else
        (Variables|Default|SetFire true)
        (Rendering|SetVisibility _niagara true false)
        (bind _asbp_cskill_zone_2 (Utilities|Casting|CastToBP_CSKillZone _childactor))
        (Variables|/Script/ChronoSpace.CSKillZone|SetbIsActive _asbp_cskill_zone_2 true)
        (Collision|SetCollisionEnabled _box "QueryAndPhysics")))))

(fn ConstructionScript
  (bind _killzone1 (Variables|Default|GetKillzone1))
  (if (Variables|Default|GetFire)
    (Rendering|SetVisibility _killzone1 true false)
    (else
      (Rendering|SetVisibility _killzone1 false false)))
  (bind _asbp_cskill_zone (Utilities|Casting|CastToBP_CSKillZone (Variables|/Script/Engine.ChildActorComponent|GetChildActor (Variables|Default|GetKillzone1))))
  (Variables|/Script/ChronoSpace.CSKillZone|SetbIsActive _asbp_cskill_zone true)
  (Collision|SetCollisionEnabled (Variables|Default|GetBox) "QueryAndPhysics")
  (Collision|SetCollisionEnabled (Variables|/Script/ChronoSpace.CSKillZone|GetKillVolume _asbp_cskill_zone) "QueryAndPhysics"))