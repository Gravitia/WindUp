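; BP_BlackholeHazard_02 is an interactive hazard object with reset logic for its physics-simulated static mesh.
; TeleportToInit runs on the authority and, unless InBlackhole is set, suspends physics, teleports to InitTransform, resumes physics and re-arms a looping ResetTime timer.
; BeginPlay is empty; the logic that records InitTransform and starts the timer is disconnected, so nothing in this graph starts the reset cycle.
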(event Custom|TeleportToInit
  (bind _staticmesh (Variables|Default|GetStaticMesh))
  (Networking|SwitchHasAuthority
    (:Authority
      (if (not (Variables|Default|GetbInBlackhole))
        (Physics|SetSimulatePhysics _staticmesh false)
        (Transformation|SetActorTransform (Variables|Default|GetInitTransform) false true)
        (Physics|SetSimulatePhysics _staticmesh true)
        (Utilities|Time|SetTimerbyEvent (delegate Custom|TeleportToInit) (Variables|Default|GetResetTime) true)))))

(event EventBeginPlay)

(fn ConstructionScript)