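; BP_UpPlatform_new is a Stage 2 interactive platform whose movement is driven by inserting a gravity core battery.
; When a lone battery overlaps the capsule, its gravity-affected mesh component is disabled and it attaches to the battery slot.
; The platform then plays the movement named after the battery's prop number.
; A mismatched number causes a delayed detach, re-enabling of that component and a return to the initial state.
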(event OnComponentBeginOverlap(Capsule)
  (params (OverlappedComponent :type Primitive%20Component%20Object%20Reference) (OtherActor :type Actor%20Object%20Reference) (OtherComp :type Primitive%20Component%20Object%20Reference) (OtherBodyIndex :type Integer) (bFromSweep :type Boolean) (SweepResult :type Hit%20Result%20Structure%20%28by%20ref%29))
  (bind _asbp_gravity_core_battery (Utilities|Casting|CastToBP_GravityCoreBattery OtherActor))
  (if (== (Utilities|Array|Length (Collision|GetOverlappingActors (Variables|Default|GetCapsule) "/Game/01_Blueprint/InteractiveObject/Stage02_Objects/BP_GravityCoreBattery.BP_GravityCoreBattery_C" :!class /Script/Engine.PrimitiveComponent)) 1)
    (Variables|Default|SetComponentMeshAffected (Actor|GetComponentbyClass _asbp_gravity_core_battery "/Script/ChronoSpace.CSMeshAffectedByGravityCore"))
    (Class|CSMeshAffectedbyGravityCore|SetEnable (Actor|GetComponentbyClass _asbp_gravity_core_battery "/Script/ChronoSpace.CSMeshAffectedByGravityCore") false)
    (bind _returnvalue (Class|CSActorAttachmentComponent|AttachActortoSlot (Variables|Default|GetActorAttachment) "battery" _asbp_gravity_core_battery))
    (if _returnvalue
      (Class|CSTransformMover|PlayMovement (Utilities|String|StringToName (Utilities|String|ToString(Integer) (Variables|/Game/01_Blueprint/InteractiveObject/Stage02_Objects/BP_GravityCoreBattery.BP_GravityCoreBattery_C|GetProp%20Number _asbp_gravity_core_battery))))
      (if (== (Variables|Default|GetpropNumber) (Variables|/Game/01_Blueprint/InteractiveObject/Stage02_Objects/BP_GravityCoreBattery.BP_GravityCoreBattery_C|GetProp%20Number _asbp_gravity_core_battery))
        (Development|PrintString "Up Platform Success")
        (else
          (Utilities|FlowControl|Delay (Variables|Default|Getdelay))
          (Class|CSActorAttachmentComponent|DetachActorfromSlot (Variables|Default|GetActorAttachment) "Battery")
          (Class|CSMeshAffectedbyGravityCore|SetEnable (Variables|Default|GetComponentMeshAffected) true)
          (Class|CSTransformMover|ReturntoInitial))))))

(event OnComponentEndOverlap(Capsule)
  (params (OverlappedComponent :type Primitive%20Component%20Object%20Reference) (OtherActor :type Actor%20Object%20Reference) (OtherComp :type Primitive%20Component%20Object%20Reference) (OtherBodyIndex :type Integer)))

(fn ConstructionScript)