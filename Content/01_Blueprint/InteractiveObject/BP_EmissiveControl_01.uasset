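; BP_EmissiveControl_01 is an interactive object that animates the emissive intensity of a target mesh when something overlaps its Box trigger.
; On BeginPlay it creates a dynamic material instance from the target mesh's first material slot and assigns it back to that slot.
; Any overlap plays a timeline whose float track drives the material's EMI scalar parameter, with no actor filter or end-overlap reversal.
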(event OnComponentBeginOverlap(Box)
  (params (OverlappedComponent :type Primitive%20Component%20Object%20Reference) (OtherActor :type Actor%20Object%20Reference) (OtherComp :type Primitive%20Component%20Object%20Reference) (OtherBodyIndex :type Integer) (bFromSweep :type Boolean) (SweepResult :type Hit%20Result%20Structure%20%28by%20ref%29))
  (bind _newtrack_0 (Timeline|Timeline Play)
    (:Update
      (Rendering|Material|SetScalarParameterValue (Variables|Default|GetMaterialInstance) "EMI" _newtrack_0 :!class /Script/Engine.MaterialInstanceDynamic))))

(event EventBeginPlay
  (bind _returnvalue (Rendering|Material|CreateDynamicMaterialInstance (Rendering|Material|GetMaterial (Variables|/Script/Engine.StaticMeshActor|GetStaticMeshComponent (Variables|Default|GetTargetMesh)) 0) "None" "None" :!class /Script/Engine.KismetMaterialLibrary))
  (Variables|Default|SetMaterialInstance _returnvalue)
  (Rendering|Material|SetMaterial (Variables|/Script/Engine.StaticMeshActor|GetStaticMeshComponent (Variables|Default|GetTargetMesh)) 0 (Variables|Default|GetMaterialInstance)))

(fn ConstructionScript)