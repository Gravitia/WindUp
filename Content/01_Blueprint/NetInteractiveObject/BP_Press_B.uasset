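; BP_Press_B is a press trap that moves its press head and cylinder in response to trap step events.
; The Second step saves the head's starting transform, then a timeline lerps its relative Z to a target while scaling the cylinder along Z to follow.
; The Third step runs another timeline that returns the head to the saved origin and scales the cylinder back to a fixed Z value.
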(event EventOnTrapStep
  (params (StepSlot :type ETrapStepSlot%20Enum :default "First"))
  (switch Utilities|FlowControl|Switch|SwitchonETrapStepSlot StepSlot
    (:Second
      (Variables|Default|SetPressOrigin (Transformation|GetRelativeTransform (Variables|Default|GetPressA)))
      (bind _lerp (Timeline|Timeline PlayFromStart)
        (:Update
          (Transformation|SetRelativeScale3D (Variables|Default|GetPressCylinder) (Math|Vector|MakeVector 2.0 2.0 (.z (.scale (Math|Transform|Lerp(Transform) (Variables|Default|GetPressOrigin) (Math|Transform|MakeTransform (Math|Vector|MakeVector 0.0 0.0 (Variables|Default|GetB%20Location%20Z)) "0, 0, 0" (Math|Vector|MakeVector 2.0 2.0 (Variables|Default|GetA%20Scale%20Z))) _lerp)))))
          (Transformation|SetRelativeLocation (Variables|Default|GetPressA) (Math|Vector|MakeVector 0.0 0.0 (.z (.location (Math|Transform|Lerp(Transform) (Variables|Default|GetPressOrigin) (Math|Transform|MakeTransform (Math|Vector|MakeVector 0.0 0.0 (Variables|Default|GetB%20Location%20Z)) "0, 0, 0" (Math|Vector|MakeVector 2.0 2.0 (Variables|Default|GetA%20Scale%20Z))) _lerp)))) false false))))
    (:Third
      (Variables|Default|SetPressLoc (Transformation|GetRelativeTransform (Variables|Default|GetPressA)))
      (bind _lerp_2 (Timeline|Timeline_0 PlayFromStart)
        (:Update
          (Transformation|SetRelativeScale3D (Variables|Default|GetPressCylinder) (.scale (Math|Transform|Lerp(Transform) (Math|Transform|MakeTransform "0, 0, 0" "0, 0, 0" (Math|Vector|MakeVector 2.0 2.0 (Variables|Default|GetA%20Scale%20Z))) (Math|Transform|MakeTransform "0, 0, 0" "0, 0, 0" (Math|Vector|MakeVector 2.0 2.0 -3.0)) _lerp_2)))
          (Transformation|SetRelativeLocation (Variables|Default|GetPressA) (Math|Vector|MakeVector 0.0 0.0 (.z (.location (Math|Transform|Lerp(Transform) (Variables|Default|GetPressLoc) (Variables|Default|GetPressOrigin) _lerp_2)))) false false))))))

(fn ConstructionScript)