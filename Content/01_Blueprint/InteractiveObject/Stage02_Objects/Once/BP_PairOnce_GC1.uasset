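; BP_PairOnce_GC1 is a paired one-shot switch that changes a target mesh's visibility when activated by a gravity core ability sphere.
; Its Trigger sets IsActivate while a BP_GravityCoreSphere_ForAbility overlaps it and clears it when the sphere leaves.
; On entry, if PairSwitch is also active, it calls VisiblityOff or VisiblityOn on TargetMesh according to its current visibility.
; Each direction has its own DoOnce, with no reset wired.
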(event OnComponentBeginOverlap(Trigger)
  (params (OverlappedComponent :type Primitive%20Component%20Object%20Reference) (OtherActor :type Actor%20Object%20Reference) (OtherComp :type Primitive%20Component%20Object%20Reference) (OtherBodyIndex :type Integer) (bFromSweep :type Boolean) (SweepResult :type Hit%20Result%20Structure%20%28by%20ref%29))
  (bind _targetmesh (Variables|Default|GetTargetMesh))
  (Utilities|Casting|CastToBP_GravityCoreSphere_ForAbility OtherActor)
  (Variables|Default|SetIsActivate true)
  (if (Variables|/Game/01_Blueprint/InteractiveObject/Stage02_Objects/Once/BP_PairOnce_BH1.BP_PairOnce_BH1_C|GetIsActivate (Variables|Default|GetPairSwitch))
    (if (Variables|/Game/01_Blueprint/InteractiveObject/Stage02_Objects/Once/BP_MeshOnce01.BP_MeshOnce01_C|GetIsVisible (Variables|Default|GetTargetMesh))
      (Utilities|FlowControl|DoOnce false
        (:Completed
          (Default|VisiblityOff _targetmesh)))
      (else
        (Utilities|FlowControl|DoOnce false
          (:Completed
            (Default|Visiblityon _targetmesh)))))))

(event OnComponentEndOverlap(Trigger)
  (params (OverlappedComponent :type Primitive%20Component%20Object%20Reference) (OtherActor :type Actor%20Object%20Reference) (OtherComp :type Primitive%20Component%20Object%20Reference) (OtherBodyIndex :type Integer))
  (Utilities|Casting|CastToBP_GravityCoreSphere_ForAbility OtherActor)
  (Variables|Default|SetIsActivate false))

(fn ConstructionScript)