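; BP_GearDoor is a gear-driven door that opens when a BP_Gear actor enters its trigger.
; The overlap destroys that gear, reveals the built-in GearVisible mesh and plays a timeline that slides DoorMesh1 along relative Y and Z.
; Tick constantly spins two gear meshes; once the gear is attached, it also turns the rest of the train and speeds up GearMesh, using fixed per-frame rotations.
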(event OnComponentBeginOverlap(Trigger)
  (params (OverlappedComponent :type Primitive%20Component%20Object%20Reference) (OtherActor :type Actor%20Object%20Reference) (OtherComp :type Primitive%20Component%20Object%20Reference) (OtherBodyIndex :type Integer) (bFromSweep :type Boolean) (SweepResult :type Hit%20Result%20Structure%20%28by%20ref%29))
  (bind _doormesh1 (Variables|Default|GetDoorMesh1))
  (bind _asbp_gear (Utilities|Casting|CastToBP_Gear OtherActor))
  (Variables|Default|SetGearAttached true)
  (Actor|DestroyActor _asbp_gear)
  (Rendering|SetVisibility (Variables|Default|GetGearVisible) true false)
  (Variables|Default|SetDoorLoc (Transformation|GetRelativeTransform _doormesh1))
  (bind _lerp (Timeline|Timeline_1 Play)
    (:Update
      (Transformation|SetRelativeLocation _doormesh1 (Math|Vector|MakeVector 0.0 (.y (.location (Math|Transform|Lerp(Transform) (Variables|Default|GetDoorLoc) (Math|Transform|MakeTransform (Math|Vector|MakeVector 0.0 5e+02 7e+02) "0, 0, 0" "1.000000,1.000000,1.000000") _lerp))) (.z (.location (Math|Transform|Lerp(Transform) (Variables|Default|GetDoorLoc) (Math|Transform|MakeTransform (Math|Vector|MakeVector 0.0 5e+02 7e+02) "0, 0, 0" "1.000000,1.000000,1.000000") _lerp)))) false false))))

(event Collision|EventActorBeginOverlap
  (params (OtherActor :type Actor%20Object%20Reference)))

(event EventTick
  (params (DeltaSeconds :type Float%20%28single-precision%29))
  (Transformation|AddLocalRotation (Variables|Default|GetGearMesh1) "0.000000,1.000000,0.000000" false false)
  (Transformation|AddLocalRotation (Variables|Default|GetGearMesh) "0.000000,1.000000,0.000000" false false)
  (if (Variables|Default|GetGearAttached)
    (Transformation|AddLocalRotation (Variables|Default|GetGearMesh) "0.000000,1.000000,0.000000" false false)
    (Transformation|AddLocalRotation (Variables|Default|GetGearMesh2) "0.000000,1.000000,0.000000" false false)
    (Transformation|AddLocalRotation (Variables|Default|GetGearMesh4) "0.000000,1.000000,0.000000" false false)
    (Transformation|AddLocalRotation (Variables|Default|GetGearVisible) "0.000000,-1.000000,0.000000" false false)
    (Transformation|AddLocalRotation (Variables|Default|GetGearMesh6) "0.000000,0.000000,-1.000000" false false)
    (Transformation|AddLocalRotation (Variables|Default|GetGearMesh5) "0.000000,0.000000,-1.000000" false false)))

(fn ConstructionScript)