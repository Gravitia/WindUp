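; BP_SwitchToggleMesh is an actor that switches between an "on" mesh and an "off" mesh.
; The VisibilityOn and VisibilityOff events swap which mesh is shown and enable query and physics collision on MeshOn only while it is visible.
; BeginPlay applies the on state if IsVisible is set, and MeshOff's collision is never changed.
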(event Custom|VisibilityOn
  (Rendering|SetVisibility (Variables|Default|GetMeshOff) false false)
  (Rendering|SetVisibility (Variables|Default|GetMeshOn) true false)
  (Collision|SetCollisionEnabled (Variables|Default|GetMeshOn) "QueryAndPhysics"))

(event Custom|VisibilityOff
  (Rendering|SetVisibility (Variables|Default|GetMeshOff) true false)
  (Rendering|SetVisibility (Variables|Default|GetMeshOn) false false)
  (Collision|SetCollisionEnabled (Variables|Default|GetMeshOn) "NoCollision"))

(event EventBeginPlay
  (if (Variables|Default|GetIsVisible)
    (CallFunction|Visibilityon)))

(fn ConstructionScript)