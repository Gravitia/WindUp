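; BP_CameraControl is a placeable trigger volume that shifts the player's follow camera while BP_CharacterPlayer is inside it.
; On overlap begin, the TimelineCloser track drives the FollowCamera's relative location with sweep; on overlap end, TimelineOuter does the same with its own track.
; The construction script sizes the Trigger from the TriggerScale variable.
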(event OnComponentBeginOverlap(Trigger)
  (params (OverlappedComponent :type Primitive%20Component%20Object%20Reference) (OtherActor :type Actor%20Object%20Reference) (OtherComp :type Primitive%20Component%20Object%20Reference) (OtherBodyIndex :type Integer) (bFromSweep :type Boolean) (SweepResult :type Hit%20Result%20Structure%20%28by%20ref%29))
  (bind _asbp_character_player (Utilities|Casting|CastToBP_CharacterPlayer OtherActor))
  (bind _newtrack_0 (Timeline|TimelineCloser PlayFromStart)
    (:Update
      (Transformation|SetRelativeLocation (Variables|/Script/ChronoSpace.CSCharacterPlayer|GetFollowCamera _asbp_character_player) _newtrack_0 true false))))

(event OnComponentEndOverlap(Trigger)
  (params (OverlappedComponent :type Primitive%20Component%20Object%20Reference) (OtherActor :type Actor%20Object%20Reference) (OtherComp :type Primitive%20Component%20Object%20Reference) (OtherBodyIndex :type Integer))
  (bind _asbp_character_player (Utilities|Casting|CastToBP_CharacterPlayer OtherActor))
  (bind _newtrack_0 (Timeline|TimelineOuter PlayFromStart)
    (:Update
      (Transformation|SetRelativeLocation (Variables|/Script/ChronoSpace.CSCharacterPlayer|GetFollowCamera _asbp_character_player) _newtrack_0 true false))))

(fn ConstructionScript
  (Transformation|SetWorldScale3D (Variables|Default|GetTrigger) (Variables|Default|GetTriggerScale)))