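; BP_ActorSpawnOnce is a tool actor that spawns a single actor of a configurable class when SpawnStart is called.
; A DoOnce gate limits the spawn, which uses a random point inside the SpawnArea box and independently randomized per-axis scale.
; Despite its name, Destroy_Area's begin overlap teleports the first found actor of that class to SpawnArea's center.
; An overlap-count check is left unconnected.
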(event OnComponentBeginOverlap(Destroy_Area)
  (params (OverlappedComponent :type Primitive%20Component%20Object%20Reference) (OtherActor :type Actor%20Object%20Reference) (OtherComp :type Primitive%20Component%20Object%20Reference) (OtherBodyIndex :type Integer) (bFromSweep :type Boolean) (SweepResult :type Hit%20Result%20Structure%20%28by%20ref%29))
  (bind _returnvalue (Actor|GetActorOfClass (Variables|Default|GetClass)))
  (Transformation|SetActorLocation _returnvalue (Transformation|GetWorldLocation (Variables|Default|GetSpawn_Area)) false false))

(event EventSpawnStart
  (bind _scalemin (Variables|Default|GetScaleMin))
  (bind _scalemax (Variables|Default|GetScaleMax))
  (bind _returnvalue (Math|Random|RandomFloatinRange _scalemin _scalemax))
  (Utilities|FlowControl|DoOnce false
    (:Completed
      (Game|SpawnActorfromClass (Variables|Default|GetClass) (Math|Transform|MakeTransform (Math|Random|RandomPointinBoundingBox (Transformation|GetWorldLocation (Variables|Default|GetSpawn_Area)) (Components|Box|GetScaledBoxExtent (Variables|Default|GetSpawn_Area))) "0, 0, 0" (Math|Vector|MakeVector _returnvalue _returnvalue _returnvalue)) "AdjustIfPossibleButAlwaysSpawn" "MultiplyWithRoot" 0 0))))

(fn ConstructionScript)