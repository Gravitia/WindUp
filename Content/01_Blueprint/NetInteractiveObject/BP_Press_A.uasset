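; BP_Press_A is a step-driven press trap that destroys barrels and breaks down after enough hits.
; On the Second trap step a timeline moves PressA to a target relative Z, and on the Third another returns it to its recorded origin.
; BP_PressBarrel overlaps on PressTigger destroy the barrel and decrement PressHealth.
; At zero health it is flagged destroyed, and the return timeline then blocks further steps.
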(event OnComponentBeginOverlap(PressTigger)
  (params (OverlappedComponent :type Primitive%20Component%20Object%20Reference) (OtherActor :type Actor%20Object%20Reference) (OtherComp :type Primitive%20Component%20Object%20Reference) (OtherBodyIndex :type Integer) (bFromSweep :type Boolean) (SweepResult :type Hit%20Result%20Structure%20%28by%20ref%29))
  (bind _asbp_press_barrel (Utilities|Casting|CastToBP_PressBarrel OtherActor))
  (Default|DestroyBarrel _asbp_press_barrel)
  (bind _result (Math|Integer|DecrementInt (Variables|Default|GetPressHealth))
    (:%20%20
      (if (== _result 0)
        (Variables|Default|SetIsDestroyed true)))))

(event EventOnTrapStep
  (params (StepSlot :type ETrapStepSlot%20Enum :default "First"))
  (if (not (Variables|Default|GetbStopAfterOperation))
    (switch Utilities|FlowControl|Switch|SwitchonETrapStepSlot StepSlot
      (:Second
        (Variables|Default|SetPressOrigin (Transformation|GetRelativeTransform (Variables|Default|GetPressA)))
        (bind _lerp (Timeline|Timeline PlayFromStart)
          (:Update
            (Transformation|SetRelativeLocation (Variables|Default|GetPressA) (Math|Vector|MakeVector 0.0 0.0 (.z (.location (Math|Transform|Lerp(Transform) (Variables|Default|GetPressOrigin) (Math|Transform|MakeTransform (Math|Vector|MakeVector 0.0 0.0 (Variables|Default|GetB%20Location%20Z)) "0, 0, 0" "1.000000,1.000000,1.000000") _lerp)))) false false))))
      (:Third
        (Variables|Default|SetPressLoc (Transformation|GetRelativeTransform (Variables|Default|GetPressA)))
        (bind _lerp_2 (Timeline|Timeline_0 PlayFromStart)
          (:Update
            (Transformation|SetRelativeLocation (Variables|Default|GetPressA) (Math|Vector|MakeVector 0.0 0.0 (.z (.location (Math|Transform|Lerp(Transform) (Variables|Default|GetPressLoc) (Variables|Default|GetPressOrigin) _lerp_2)))) false false)
            (if (Variables|Default|GetIsDestroyed)
              (Variables|Default|SetbStopAfterOperation true))))))))

(fn ConstructionScript)