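; BP_StageCurtain is a networked stage curtain that opens while both players' buttons are pressed, with an option to stay open afterwards.
; NotifyButtonState records each player's button on the authority and updates IsOpen, whose RepNotify plays or reverses a Timeline.
; BeginPlay caches the closed positions and scales the Timeline's play rate to OpenDuration.
; ApplyCurtainAlpha, wired to the Timeline update, slides the two halves apart along local Y by OpenDistance.
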(event EventBeginPlay
  (CallFunction|InitCurtain))

(fn ConstructionScript)

(fn OnRepBIsOpen
  (CallFunction|UpdateCurtainMotion))

(fn InitCurtain
  (bind _timeline (Variables|Default|GetTimeline))
  (bind _openduration (Variables|CSEditable|StageCurtain|GetOpenDuration))
  (bind _returnvalue (Components|Timeline|GetTimelineLength _timeline))
  (Variables|Default|SetLeftClosedLocation (Variables|/Script/Engine.SceneComponent|GetRelativeLocation (Variables|Default|GetCurtainLeft)))
  (Variables|Default|SetRightClosedLocation (Variables|/Script/Engine.SceneComponent|GetRelativeLocation (Variables|Default|GetCurtainRight)))
  (Components|Timeline|SetPlayRate _timeline (/ _returnvalue (select (> _openduration (Math|Float|MakeLiteralFloat 0.05)) _openduration (Math|Float|MakeLiteralFloat 0.05))))
  (if (Variables|Default|GetbIsOpen)
    (Components|Timeline|SetPlaybackPosition _timeline _returnvalue false true)))

(fn ApplyCurtainAlpha
  (params (Alpha :type Float%20%28double-precision%29))
  (bind _opendistance (Variables|CSEditable|StageCurtain|GetOpenDistance))
  (bind _returnvalue (* _opendistance Alpha))
  (bind _returnvalue_2 (Math|Vector|MakeVector 0.0 _returnvalue 0.0))
  (Transformation|SetRelativeLocation (Variables|Default|GetCurtainLeft) (- (Variables|Default|GetLeftClosedLocation) _returnvalue_2) false false)
  (Transformation|SetRelativeLocation (Variables|Default|GetCurtainRight) (+ (Variables|Default|GetRightClosedLocation) _returnvalue_2) false false))

(fn UpdateCurtainMotion
  (bind _timeline (Variables|Default|GetTimeline))
  (if (Variables|Default|GetbIsOpen)
    (Audio|Components|Audio|Play _timeline)
    (else
      (Utilities|String|Reverse _timeline))))

(fn NotifyButtonState
  (params (bIsPlayer2 :type Boolean) (bPressed :type Boolean))
  (if (Ability|HasAuthority self)
    (if bIsPlayer2
      (Variables|Default|SetbButton2Pressed bPressed)
      (else
        (Variables|Default|SetbButton1Pressed bPressed)))
    (if (!= (or (and (Variables|Default|GetbButton1Pressed) (Variables|Default|GetbButton2Pressed)) (and (Variables|CSEditable|StageCurtain|GetbStayOpen) (Variables|Default|GetbIsOpen))) (Variables|Default|GetbIsOpen))
      (Variables|Default|SetbIsOpen (or (and (Variables|Default|GetbButton1Pressed) (Variables|Default|GetbButton2Pressed)) (and (Variables|CSEditable|StageCurtain|GetbStayOpen) (Variables|Default|GetbIsOpen)))))))