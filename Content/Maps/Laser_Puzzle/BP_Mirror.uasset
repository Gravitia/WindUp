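; BP_Mirror is a rotatable mirror for the laser puzzle, turned in quarter-turn yaw steps.
; A box overlap enables or disables the first player controller's input on the actor.
; Rotate advances the target angle and plays a timeline that lerps the mirror's relative rotation to it.
; A Rotation flag clears after a delay, but its guard branch is disconnected, so Rotate never checks it.
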(event OnComponentBeginOverlap(Box)
  (params (OverlappedComponent :type Primitive%20Component%20Object%20Reference) (OtherActor :type Actor%20Object%20Reference) (OtherComp :type Primitive%20Component%20Object%20Reference) (OtherBodyIndex :type Integer) (bFromSweep :type Boolean) (SweepResult :type Hit%20Result%20Structure%20%28by%20ref%29))
  (Input|EnableInput (Game|GetPlayerController 0)))

(event OnComponentEndOverlap(Box)
  (params (OverlappedComponent :type Primitive%20Component%20Object%20Reference) (OtherActor :type Actor%20Object%20Reference) (OtherComp :type Primitive%20Component%20Object%20Reference) (OtherBodyIndex :type Integer))
  (Input|DisableInput (Game|GetPlayerController 0)))

(event Custom|Rotate
  (Variables|Default|SetRotation? true)
  (Variables|Default|SetProp%20Angle (+ (Variables|Default|GetProp%20Angle) 9e+01))
  (bind _newtrack_0 (Timeline|Timeline PlayFromStart)
    (:Update
      (Transformation|SetRelativeRotation (Variables|Default|GetMirror) (Math|Rotator|Lerp(Rotator) (Math|Rotator|MakeRotator 0.0 0.0 (- (Variables|Default|GetProp%20Angle) 9e+01)) (Math|Rotator|MakeRotator 0.0 0.0 (Variables|Default|GetProp%20Angle)) _newtrack_0) false false)
      (Utilities|FlowControl|Delay 1.2)
      (Variables|Default|SetRotation? false))))

(fn ConstructionScript)