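; BP_CurtainButton is a networked pressure button that only responds to one designated player slot and reports its state to a target curtain.
; On trigger overlap begin and end, the authority checks the character's PlayerSlot against ForPlayer2, then sets the pressed state and notifies TargetCurtain.
; The pressed state's RepNotify lowers or restores the button mesh relative to the rest location cached at BeginPlay.
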(event OnComponentBeginOverlap(Trigger)
  (params (OverlappedComponent :type Primitive%20Component%20Object%20Reference) (OtherActor :type Actor%20Object%20Reference) (OtherComp :type Primitive%20Component%20Object%20Reference) (OtherBodyIndex :type Integer) (bFromSweep :type Boolean) (SweepResult :type Hit%20Result%20Structure%20%28by%20ref%29))
  (CallFunction|HandleTriggerChange OtherActor true))

(event OnComponentEndOverlap(Trigger)
  (params (OverlappedComponent :type Primitive%20Component%20Object%20Reference) (OtherActor :type Actor%20Object%20Reference) (OtherComp :type Primitive%20Component%20Object%20Reference) (OtherBodyIndex :type Integer))
  (CallFunction|HandleTriggerChange OtherActor false))

(event EventBeginPlay
  (Variables|Default|SetMeshRestLocation (Variables|/Script/Engine.SceneComponent|GetRelativeLocation (Variables|Default|GetButtonMesh))))

(fn ConstructionScript)

(fn OnRepBIsPressed
  (CallFunction|ApplyPressVisual))

(fn IsRequiredPlayer
  (params (TestActor :type Actor%20Object%20Reference))
  (bind _ascscharacter_player (Utilities|Casting|CastToCSCharacterPlayer TestActor)
    (:then
      (bind _ascsplayer_state (Utilities|Casting|CastToCSPlayerState (Variables|/Script/Engine.Pawn|GetPlayerState _ascscharacter_player))
        (:then
          (switch Utilities|FlowControl|Switch|SwitchonECSPlayerSlot (Variables|/Script/ChronoSpace.CSPlayerState|GetPlayerSlot _ascsplayer_state)
            (:Player0
              (return (not (Variables|CSEditable|StageCurtain|GetbForPlayer2))))
            (:Player1
              (return (Variables|CSEditable|StageCurtain|GetbForPlayer2)))))
        (:CastFailed
          (return false))))
    (:CastFailed
      (return false))))

(fn ApplyPressVisual
  (Transformation|SetRelativeLocation (Variables|Default|GetButtonMesh) (- (Variables|Default|GetMeshRestLocation) (Math|Vector|MakeVector 0.0 0.0 (select (Variables|Default|GetbIsPressed) (Variables|CSEditable|StageCurtain|GetPressedDepth) (Math|Float|MakeLiteralFloat 0.0)))) false false))

(fn HandleTriggerChange
  (params (TestActor :type Actor%20Object%20Reference) (bEntered :type Boolean))
  (bind _targetcurtain (Variables|CSEditable|StageCurtain|GetTargetCurtain))
  (if (Ability|HasAuthority self)
    (bind _bmatched (CallFunction|IsRequiredPlayer TestActor))
    (if _bmatched
      (Variables|Default|SetbIsPressed bEntered)
      (Utilities|IsValid _targetcurtain
        (:Is%20Valid
          (Default|NotifyButtonState _targetcurtain (Variables|CSEditable|StageCurtain|GetbForPlayer2) bEntered))))))