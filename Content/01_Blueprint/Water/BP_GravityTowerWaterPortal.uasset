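; Water portal for the gravity tower that sends the game to L_Main as a listen server when a player character overlaps it while activated.
; BeginPlay clears IsActivated, and nothing in this Blueprint sets it to true.
; Reactivate turns the static mesh collision off, then a short timer calls Activate to restore query-only collision.
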(event EventBeginPlay
  (Variables|Default|SetIsActivated false))

(event Collision|EventActorBeginOverlap
  (params (OtherActor :type Actor%20Object%20Reference))
  (Utilities|Casting|CastToCSCharacterPlayer OtherActor)
  (if (Variables|Default|GetIsActivated)
    (Class|AdvancedSessionsLibrary|ServerTravel "L_Main?listen" false false)))

(event EventTick
  (params (DeltaSeconds :type Float%20%28single-precision%29)))

(fn ConstructionScript)

(fn Reactivate
  (Collision|SetCollisionEnabled (Variables|Default|GetStaticMesh) "NoCollision")
  (Utilities|Time|SetTimerbyFunctionName 0 "Activate" 0.5))

(fn Activate
  (Collision|SetCollisionEnabled (Variables|Default|GetStaticMesh) "QueryOnly"))