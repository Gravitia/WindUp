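; BP_CCTV_Watcher is a CCTV camera actor with a patrol-colored spotlight that sweeps its view and can test for the player.
; A timeline yaws the pivot around its initial rotation while the state enum holds its first value.
; IsPlayerInSight combines cone angle, range and a debug-drawn visibility trace from the spotlight to the player pawn.
; No graph here calls that check or changes the state.
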(event EventBeginPlay
  ;[0.15 0.15 0.15 0.5] CCTV_HedMove
  (Variables|Cache|SetTargetPlayer (Game|Player|GetPlayerPawn 0))
  (Variables|Cache|SetInitialPivotRotation (Variables|/Script/Engine.SceneComponent|GetRelativeRotation (Variables|Default|GetPivotScene)))
  (Rendering|Components|Light|SetLightColor (Variables|Default|GetSpotLight) (Variables|Visual|GetPatrolColor) true)
  (bind _scanalpha (Timeline|ScanTimeline Play)
    (:Update
      (if (Utilities|Enum|Equal(Enum) (Variables|State|GetCurrentState) "NewEnumerator0")
        (Transformation|SetRelativeRotation (Variables|Default|GetPivotScene) (Math|Rotator|CombineRotators (Variables|Cache|GetInitialPivotRotation) (Math|Rotator|MakeRotator 0.0 0.0 (* _scanalpha (Variables|Patrol|GetScanAngle)))) false false)))))

(event Collision|EventActorBeginOverlap
  (params (OtherActor :type Actor%20Object%20Reference)))

(event EventTick
  (params (DeltaSeconds :type Float%20%28single-precision%29)))

(fn ConstructionScript)

(fn IsPlayerinSight
  (bind _targetplayer (Variables|Cache|GetTargetPlayer))
  (bind _spotlight (Variables|Default|GetSpotLight))
  (bind _returnvalue (Transformation|GetActorLocation _targetplayer))
  (bind _returnvalue_2 (Transformation|GetWorldLocation _spotlight))
  (bind _outhit (Collision|LineTraceByChannel _returnvalue_2 _returnvalue "TraceTypeQuery1" false 0 "ForDuration"))
  (return (and (and (<= (Class|KismetMathLibrary|DegAcos (Math|Vector|DotProduct (Math|Vector|Normalize (- _returnvalue _returnvalue_2)) (Math|Vector|GetForwardVector _spotlight))) (Variables|Detection|GetDetectionConeAngle)) (<= (Math|Vector|Distance(Vector) _returnvalue _returnvalue_2) (Variables|Detection|GetDetectionRange))) (== (.HitActor (Collision|BreakHitResult _outhit)) (Variables|Cache|GetTargetPlayer)))))