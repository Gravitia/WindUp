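; Stage 2 interactive object that shows its TargetMesh while an ability black hole (BP_BlackHole_ForAbility) overlaps its Trigger.
; Begin and end overlaps set separate flags for the gravity sphere and the event horizon, treating any component other than the gravity sphere as the horizon.
; The mesh turns on at the first overlap and turns off only once both flags are clear.
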(event OnComponentBeginOverlap(Trigger)
  (params (OverlappedComponent :type Primitive%20Component%20Object%20Reference) (OtherActor :type Actor%20Object%20Reference) (OtherComp :type Primitive%20Component%20Object%20Reference) (OtherBodyIndex :type Integer) (bFromSweep :type Boolean) (SweepResult :type Hit%20Result%20Structure%20%28by%20ref%29))
  (bind _targetmesh (Variables|Default|GetTargetMesh))
  (bind _asbp_black_hole_for_ability (Utilities|Casting|CastToBP_BlackHole_ForAbility OtherActor))
  (if (== OtherComp (Variables|/Script/ChronoSpace.CSBlackHole|GetGravitySphereTrigger _asbp_black_hole_for_ability))
    (Variables|Default|SetbGravitySphereTrigger true)
    (else
      (Variables|Default|SetbEventHorizonSphereTrigger true)))
  (if (not (Variables|/Game/01_Blueprint/InteractiveObject/Stage02_Objects/Alone/BP_MeshRepeatBH.BP_MeshRepeatBH_C|GetIsVisible _targetmesh))
    (Default|Visiblityon _targetmesh)))

(event OnComponentEndOverlap(Trigger)
  (params (OverlappedComponent :type Primitive%20Component%20Object%20Reference) (OtherActor :type Actor%20Object%20Reference) (OtherComp :type Primitive%20Component%20Object%20Reference) (OtherBodyIndex :type Integer))
  (bind _targetmesh (Variables|Default|GetTargetMesh))
  (bind _asbp_black_hole_for_ability (Utilities|Casting|CastToBP_BlackHole_ForAbility OtherActor))
  (if (== OtherComp (Variables|/Script/ChronoSpace.CSBlackHole|GetGravitySphereTrigger _asbp_black_hole_for_ability))
    (Variables|Default|SetbGravitySphereTrigger false)
    (else
      (Variables|Default|SetbEventHorizonSphereTrigger false)))
  (if (Variables|/Game/01_Blueprint/InteractiveObject/Stage02_Objects/Alone/BP_MeshRepeatBH.BP_MeshRepeatBH_C|GetIsVisible _targetmesh)
    (if (Math|Boolean|NORBoolean (Variables|Default|GetbGravitySphereTrigger) (Variables|Default|GetbEventHorizonSphereTrigger))
      (Default|VisiblityOff _targetmesh))))

(fn ConstructionScript)