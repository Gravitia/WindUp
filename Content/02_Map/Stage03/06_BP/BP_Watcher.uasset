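; BP_Watcher is a Stage03 pawn that chases the player as soon as play begins.
; BeginPlay sets IsChasing and turns its point light red as an alert color.
; While the flag is set, Tick reissues AIMoveTo toward player 0 every frame, printing a debug string when the move fails.
; Nothing in the file clears the flag, so the chase never stops.
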(event Custom|StartChasing
  (Variables|Default|SetbIsChasing true)
  (Development|PrintString "start go"))

(event Custom|SetAlertColor
  (Rendering|Components|Light|SetLightColor (Variables|Default|GetPointLight) "(R=1.000000,G=0.000000,B=0.000000,A=1.000000)" true))

(event EventBeginPlay
  (CallFunction|StartChasing)
  (CallFunction|SetAlertColor))

(event EventTick
  (params (DeltaSeconds :type Float%20%28single-precision%29))
  (if (Variables|Default|GetbIsChasing)
    (AI|AIMoveTo self "0, 0, 0" (Game|GetPlayerCharacter 0) 1.2e+02 false
      (:OnFail
        (Development|PrintString "start stop")))))

(fn ConstructionScript)