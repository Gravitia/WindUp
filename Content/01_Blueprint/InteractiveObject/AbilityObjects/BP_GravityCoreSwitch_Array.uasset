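; BP_GravityCoreSwitch_Array is a switch that flips the visibility of multiple target meshes when a gravity core ability sphere overlaps its trigger.
; On begin overlap, each TargetMesh element inverts its current visibility through VisiblityOn or VisiblityOff.
; On end overlap, each element inverts again and also receives the matching RESETON or RESETOFF call.
; Toggling is relative to each element's current state, so mixed arrays swap visible and hidden members.
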(event OnComponentBeginOverlap(Trigger)
  (params (OverlappedComponent :type Primitive%20Component%20Object%20Reference) (OtherActor :type Actor%20Object%20Reference) (OtherComp :type Primitive%20Component%20Object%20Reference) (OtherBodyIndex :type Integer) (bFromSweep :type Boolean) (SweepResult :type Hit%20Result%20Structure%20%28by%20ref%29))
  (Utilities|Casting|CastToBP_GravityCoreSphere_ForAbility OtherActor)
  (for _array_element (Variables|Default|GetTargetMesh)
    (if (Variables|/Game/01_Blueprint/InteractiveObject/BP_SwitchToggleMesh_01.BP_SwitchToggleMesh_01_C|GetIsVisible _array_element)
      (Default|VisiblityOff _array_element)
      (else
        (Default|Visiblityon _array_element)))))

(event OnComponentEndOverlap(Trigger)
  (params (OverlappedComponent :type Primitive%20Component%20Object%20Reference) (OtherActor :type Actor%20Object%20Reference) (OtherComp :type Primitive%20Component%20Object%20Reference) (OtherBodyIndex :type Integer))
  (Utilities|Casting|CastToBP_GravityCoreSphere_ForAbility OtherActor)
  (for _array_element (Variables|Default|GetTargetMesh)
    (if (Variables|/Game/01_Blueprint/InteractiveObject/BP_SwitchToggleMesh_01.BP_SwitchToggleMesh_01_C|GetIsVisible _array_element)
      (Default|VisiblityOff _array_element)
      (Default|RESETOFF _array_element)
      (else
        (Default|Visiblityon _array_element)
        (Default|RESETON _array_element)))))

(fn ConstructionScript)