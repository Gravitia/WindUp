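; BP_ConveyorBelt is an interactive-object Blueprint that simulates a looping conveyor belt from repeated static mesh segments.
; BeginPlay spawns BeltCount mesh components spaced BeltLength apart along local X.
; Tick slides each segment by BeltSpeed and teleports segments that pass the belt's end back by its total length.
; When ShowPreview is set, the construction script lays out dummy conveyor instances as an editor preview, hidden in game and without collision.
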(event EventBeginPlay
  (for _index (range 0 (- (Variables|Default|GetBeltCount) 1))
    (bind _returnvalue (AddComponent|AddStaticMeshComponent false))
    (Transformation|SetRelativeLocation _returnvalue (Math|Vector|MakeVector (* _index (Variables|Default|GetBeltLength)) 0.0 0.0) false false)
    (Utilities|Array|Add (Variables|Default|GetBeltMesh) _returnvalue)))

(event EventTick
  (params (DeltaSeconds :type Float%20%28single-precision%29))
  (bind _beltcount (Variables|Default|GetBeltCount))
  (bind _beltlength (Variables|Default|GetBeltLength))
  (bind _returnvalue (* _beltcount _beltlength))
  (for _array_element (Variables|Default|GetBeltMesh)
    (Transformation|SetRelativeLocation _array_element (Math|Vector|MakeVector (+ (.x (.location (Transformation|GetRelativeTransform _array_element))) (* DeltaSeconds (Variables|Default|GetBeltSpeed))) 0.0 0.0) false false)
    (if (> (+ (.x (.location (Transformation|GetRelativeTransform _array_element))) (* DeltaSeconds (Variables|Default|GetBeltSpeed))) _returnvalue)
      (Transformation|SetRelativeLocation _array_element (Math|Vector|MakeVector (- (+ (.x (.location (Transformation|GetRelativeTransform _array_element))) (* DeltaSeconds (Variables|Default|GetBeltSpeed))) _returnvalue) 0.0 0.0) false true))))

(fn ConstructionScript
  (bind _instancedstaticmesh (Variables|Default|GetInstancedStaticMesh))
  (if (Variables|Default|GetShowPreview)
    (Components|StaticMesh|SetStaticMesh (Variables|Default|GetInstancedStaticMesh) "/Game/30_Mesh/LDProps/StaticMeshes/DummyProps/SM_DummyConveyor_01.SM_DummyConveyor_01")
    (for _index (range 0 (- (Variables|Default|GetBeltCount) 1))
      (Components|InstancedStaticMesh|AddInstance (Variables|Default|GetInstancedStaticMesh) (Math|Transform|MakeTransform (Math|Vector|MakeVector (* _index (Variables|Default|GetBeltLength)) 0.0 0.0) "0, 0, 0" "1.000000,1.000000,1.000000") false)
      (Development|SetHiddeninGame _instancedstaticmesh true false)
      (Collision|SetCollisionEnabled _instancedstaticmesh "NoCollision"))))