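; CCTV camera watcher that sweeps a spotlight and detects the player pawn, changing the light color between patrol and alert.
; A timeline yaws the pivot while Patrolling, and Tick runs a Patrolling/Alerted/Searching state machine.
; IsPlayerInSight combines range, cone angle and a visibility trace from the spotlight.
; Searching lasts one tick, either nudging yaw toward a reacquired player and re-alerting, or restarting the patrol sweep.
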(event EventBeginPlay
  ;[0.15 0.15 0.15 0.5] CCTV_HedMove
  (Variables|Cache|SetTargetPlayer (Game|Player|GetPlayerPawn 0))
  (Variables|Cache|SetInitialPivotRotation (Variables|/Script/Engine.SceneComponent|GetRelativeRotation (Variables|Default|GetPivotScene)))
  (Rendering|Components|Light|SetLightColor (Variables|Default|GetSpotLight) (Variables|Visual|GetPatrolColor) true)
  (bind _scanalpha (Timeline|ScanTimeline Play)
    (:Update
      (if (Utilities|Enum|Equal(Enum) (Variables|State|GetCurrentState) "NewEnumerator0")
        (Transformation|SetRelativeRotation (Variables|Default|GetPivotScene) (Math|Rotator|CombineRotators (Variables|Cache|GetInitialPivotRotation) (Math|Rotator|MakeRotator 0.0 0.0 (* _scanalpha (Variables|Patrol|GetScanAngle)))) false false)))))

(event EventTick
  (params (DeltaSeconds :type Float%20%28single-precision%29))
  (bind _pivotscene (Variables|Default|GetPivotScene))
  (switch Utilities|FlowControl|Switch|SwitchonE_CCTVState (Variables|State|GetCurrentState)
    (:NewEnumerator0
      (bind _bisvisible (CallFunction|IsPlayerinSight))
      (if _bisvisible
        (Variables|State|SetCurrentState "NewEnumerator1")
        (Rendering|Components|Light|SetLightColor (Variables|Default|GetSpotLight) (Variables|Visual|GetAlertColor) true)))
    (:NewEnumerator1
      (bind _bisvisible_2 (CallFunction|IsPlayerinSight))
      (if (not _bisvisible_2)
        (Variables|State|SetCurrentState "NewEnumerator2")))
    (:NewEnumerator2
      (bind _bisvisible_3 (CallFunction|IsPlayerinSight))
      (if _bisvisible_3
        (Transformation|SetRelativeRotation _pivotscene (Math|Interpolation|RInterpTo (Variables|/Script/Engine.SceneComponent|GetRelativeRotation _pivotscene) (Math|Rotator|MakeRotator 0.0 0.0 (.Yaw (Math|Rotator|BreakRotator (Math|Rotator|FindLookatRotation (Transformation|GetWorldLocation _pivotscene) (Transformation|GetActorLocation (Variables|Cache|GetTargetPlayer)))))) DeltaSeconds (Variables|Alert|GetTrackingSpeed)) false false)
        (Variables|State|SetCurrentState "NewEnumerator1")
        (Rendering|Components|Light|SetLightColor (Variables|Default|GetSpotLight) (Variables|Visual|GetAlertColor) true)
        (else
          (Variables|State|SetCurrentState "NewEnumerator0")
          (Rendering|Components|Light|SetLightColor (Variables|Default|GetSpotLight) (Variables|Visual|GetPatrolColor) true)
          ;[0.15 0.15 0.15 0.5] CCTV_HedMove
          (bind _scanalpha (Timeline|ScanTimeline PlayFromStart)
            (:Update
              (if (Utilities|Enum|Equal(Enum) (Variables|State|GetCurrentState) "NewEnumerator0")
                (Transformation|SetRelativeRotation (Variables|Default|GetPivotScene) (Math|Rotator|CombineRotators (Variables|Cache|GetInitialPivotRotation) (Math|Rotator|MakeRotator 0.0 0.0 (* _scanalpha (Variables|Patrol|GetScanAngle)))) false false)))))))))

(fn ConstructionScript)

(fn IsPlayerinSight
  (bind _targetplayer (Variables|Cache|GetTargetPlayer))
  (bind _spotlight (Variables|Default|GetSpotLight))
  (bind _returnvalue (Transformation|GetActorLocation _targetplayer))
  (bind _returnvalue_2 (Transformation|GetWorldLocation _spotlight))
  (bind _outhit (Collision|LineTraceByChannel _returnvalue_2 _returnvalue "TraceTypeQuery1" false 0 "None"))
  (return (and (and (<= (Math|Vector|Distance(Vector) _returnvalue _returnvalue_2) (Variables|Detection|GetDetectionRange)) (<= (Class|KismetMathLibrary|DegAcos (Math|Vector|DotProduct (Math|Vector|Normalize (- _returnvalue _returnvalue_2)) (Math|Vector|GetForwardVector _spotlight))) (Variables|Detection|GetDetectionConeAngle))) (== (.HitActor (Collision|BreakHitResult _outhit)) (Variables|Cache|GetTargetPlayer)))))