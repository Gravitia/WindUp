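; Two-part switch, likely for two players, that hides a target mesh when it and its paired switch are both active.
; Overlapping the Trigger sets IsActivated, then checks PairSwitch's flag before calling VisiblityOff on TargetMesh.
; Ending the overlap clears IsActivated before testing it, so the VisiblityOn branch that would restore the mesh never runs as written.
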(event OnComponentBeginOverlap(Trigger)
  (params (OverlappedComponent :type Primitive%20Component%20Object%20Reference) (OtherActor :type Actor%20Object%20Reference) (OtherComp :type Primitive%20Component%20Object%20Reference) (OtherBodyIndex :type Integer) (bFromSweep :type Boolean) (SweepResult :type Hit%20Result%20Structure%20%28by%20ref%29))
  (Variables|Default|SetIsActivated%20 true)
  (if (Variables|Default|GetIsActivated%20)
    (if (Variables|/Game/01_Blueprint/InteractiveObject/BP_2POffSwitch_02.BP_2POffSwitch_02_C|GetIsActivated%20 (Variables|Default|GetPairSwitch))
      (Default|VisiblityOff (Variables|Default|GetTargetMesh)))))

(event OnComponentEndOverlap(Trigger)
  (params (OverlappedComponent :type Primitive%20Component%20Object%20Reference) (OtherActor :type Actor%20Object%20Reference) (OtherComp :type Primitive%20Component%20Object%20Reference) (OtherBodyIndex :type Integer))
  (Variables|Default|SetIsActivated%20 false)
  (if (Variables|Default|GetIsActivated%20)
    (if (Variables|/Game/01_Blueprint/InteractiveObject/BP_2POffSwitch_02.BP_2POffSwitch_02_C|GetIsActivated%20 (Variables|Default|GetPairSwitch))
      (Default|Visiblityon (Variables|Default|GetTargetMesh)))))

(fn ConstructionScript)