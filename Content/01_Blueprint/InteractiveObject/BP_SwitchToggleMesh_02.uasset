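; Interactive object that toggles between an on mesh and an off mesh, as a switch-controlled element.
; VisiblityOn shows MeshOn with query and physics collision and hides MeshOff, while VisiblityOff reverses visibility and disables MeshOn's collision.
; MeshOff's collision is never changed.
; BeginPlay applies the on state only when IsVisible is set, otherwise leaving the component defaults in place.
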(event Custom|VisiblityOn
  (Rendering|SetVisibility (Variables|Default|GetMeshOff) false false)
  (Rendering|SetVisibility (Variables|Default|GetMeshOn) true false)
  (Collision|SetCollisionEnabled (Variables|Default|GetMeshOn) "QueryAndPhysics"))

(event Custom|VisiblityOff
  (Rendering|SetVisibility (Variables|Default|GetMeshOff) true false)
  (Rendering|SetVisibility (Variables|Default|GetMeshOn) false false)
  (Collision|SetCollisionEnabled (Variables|Default|GetMeshOn) "NoCollision"))

(event EventBeginPlay
  (if (Variables|Default|GetIsVisible)
    (CallFunction|Visiblityon)))

(fn ConstructionScript)