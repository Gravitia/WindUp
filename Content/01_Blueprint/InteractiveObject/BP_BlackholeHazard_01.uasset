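; BP_BlackholeHazard_01 is a physics-simulated interactive object that periodically returns to its starting transform.
; On BeginPlay, the authority stores the initial transform and starts a looping ResetTime timer.
; Each tick of that timer skips the reset while InBlackhole is set; otherwise it toggles physics off, teleports the mesh actor home, re-enables physics and sets the timer again.
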(event Custom|TeleportToInit
  (bind _staticmesh (Variables|Default|GetStaticMesh))
  (if (not (Variables|Default|GetbInBlackhole))
    (Physics|SetSimulatePhysics _staticmesh false)
    (Transformation|SetActorTransform (Variables|Default|GetInitTransform) false true)
    (Physics|SetSimulatePhysics _staticmesh true)
    (Utilities|Time|SetTimerbyEvent (delegate Custom|TeleportToInit) (Variables|Default|GetResetTime) true)))

(event EventBeginPlay
  (Networking|SwitchHasAuthority
    (:Authority
      (Variables|Default|SetInitTransform (Transformation|GetActorTransform))
      (Utilities|Time|SetTimerbyEvent (delegate Custom|TeleportToInit) (Variables|Default|GetResetTime) true))))

(fn ConstructionScript)