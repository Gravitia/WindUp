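; Interactive-object fire windmill that repeatedly rotates its static mesh through a 90-degree pitch sweep.
; BeginPlay advances PropAngle once, then starts a timeline whose track lerps the mesh's relative rotation up to that angle, keeping yaw constant.
; A two-second Delay on the timeline's Update pin restarts it from the beginning, replaying the same arc because the angle never advances again.
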(event EventBeginPlay
  (bind _a_z__yaw_ (Variables|Default|GetA%20Z%20%28Yaw%29))
  (Variables|Default|SetProp%20Angle (+ (Variables|Default|GetProp%20Angle) 9e+01))
  (bind _newtrack_0 (Timeline|Timeline PlayFromStart)
    (:Update
      (Transformation|SetRelativeRotation (Variables|Default|GetStaticMesh) (Math|Rotator|Lerp(Rotator) (Math|Rotator|MakeRotator 0.0 (- (Variables|Default|GetProp%20Angle) 9e+01) _a_z__yaw_) (Math|Rotator|MakeRotator 0.0 (Variables|Default|GetProp%20Angle) _a_z__yaw_) _newtrack_0) false false)
      (Utilities|FlowControl|Delay 2.0)
      (Timeline|Timeline PlayFromStart))))

(fn ConstructionScript)