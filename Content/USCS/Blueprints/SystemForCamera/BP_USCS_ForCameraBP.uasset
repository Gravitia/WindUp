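; Camera zone actor for the USCS spline camera system, handing the view to SceneCamera when the player enters either of two influence volumes.
; Activation copies spline, blend, rotation, clamp and lag settings onto SceneCamera, with optional fade-in.
; Zones share state through references to all instances and other camera Blueprints to detect switches and avoid redundant transitions.
; Optional Tick-driven rail depth moves CameraSpline relative to the player's closest point on SplineDepth.
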(event OnComponentBeginOverlap(ZoneInfluenceA)
  (params (OverlappedComponent :type Primitive%20Component%20Object%20Reference) (OtherActor :type Actor%20Object%20Reference) (OtherComp :type Primitive%20Component%20Object%20Reference) (OtherBodyIndex :type Integer) (bFromSweep :type Boolean) (SweepResult :type Hit%20Result%20Structure%20%28by%20ref%29))
  (bind _scenecamera (Variables|PARAMETERS:|GetSceneCamera))
  (bind _splineraildepthon_ (Variables|PARAMETERS:|GetSplineRailDepthOn?))
  (bind _usefadein (Variables|PARAMETRS:FadeIn:|GetUseFadeIn))
  (Utilities|IsPlayerCharacter/Pawn? OtherActor
    (:true
      (bind _displayname (CallFunction|GetUSCSDisplayName))
      (Variables|Default|SetCurrentUSCS_OverlappedA _displayname)
      (Variables|Default|SetIsActivated? true)
      (Utilities|FlowControl|Sequence
        (:then_0
          (Utilities|FlowControl|Sequence
            (:then_0
              (for _array_element (Variables|Default|GetCharacterCameraBP_Ref)
                (Default|BacktoUscs _array_element)))
            (:then_1
              (for _array_element_2 (Variables|Default|GetCameraStaticBP_Ref)
                (Default|BacktoUscs _array_element_2)))
            (:then_2
              (CallFunction|BacktoUscs))))
        (:then_1
          (Actor|Tick|SetActorTickEnabled (or (or _splineraildepthon_ _usefadein) (and _splineraildepthon_ _usefadein)))
          (if (Variables|PARAMETRS:FadeIn:|GetUseFadeIn)
            (if (Utilities|Enum|Equal(Enum) (Variables|Default|GetCurrentUSCS_OverlappedA) (Variables|Default|GetCurrentUSCS_OverlappedB))
              (if (Variables|Default|GetIs%20SwitchBP?)
                (bind _bc_fadeincamerabp (CallFunction|BCFadeinCameraParameters (Variables|PARAMETERS:|GetSceneCamera) (Variables|PARAMETRS:FadeIn:|GetUseFadeIn) (Variables|PARAMETRS:FadeIn:|GetDisable%20Player%20Input%20Controller) (Variables|PARAMETRS:FadeIn:|GetPre%20Fade%20Time) (Variables|PARAMETRS:FadeIn:|GetPre%20Fade%20Color) (Variables|PARAMETRS:FadeIn:|GetPre%20Fade%20Should%20Fade%20Audio) (Variables|PARAMETRS:FadeIn:|GetFade%20Time) (Variables|PARAMETRS:FadeIn:|GetFade%20Color) (Variables|PARAMETRS:FadeIn:|GetFade%20from%20Alpha%28X%29%20to%20Alpha%28Y%29) (Variables|PARAMETRS:FadeIn:|GetShould%20Fade%20Audio?) (Variables|PARAMETRS:FadeIn:|GetHold%20When%20Finished?) :!label _label))
                (Default|BCFadeinSetting _bc_fadeincamerabp))
              (else
                (goto _label))))
          (Variables|/Game/USCS/Blueprints/SystemForCamera/BP_CameraBP.BP_CameraBP_C|SetSpline (Variables|PARAMETERS:|GetSceneCamera) (Variables|Default|GetCameraSpline))
          (Variables|/Game/USCS/Blueprints/SystemForCamera/BP_CameraBP.BP_CameraBP_C|SetIsStartGameCamera? _scenecamera (Variables|PARAMETERS:|GetIsGameStartCamera?))
          (Variables|/Game/USCS/Blueprints/SystemForCamera/BP_CameraBP.BP_CameraBP_C|SetInstantCameraView _scenecamera (Variables|PARAMETERS:|GetInstantCameraView%28NoBlend%29))
          (Variables|/Game/USCS/Blueprints/SystemForCamera/BP_CameraBP.BP_CameraBP_C|SetGameStartCameraBlendTime _scenecamera (Variables|PARAMETERS:|GetGame%20Start%20Camera%20Blend%20Time))
          (Variables|/Game/USCS/Blueprints/SystemForCamera/BP_CameraBP.BP_CameraBP_C|SetSnapCameraSpline? _scenecamera (Variables|PARAMETERS:|GetSnapCameraSpline?))
          (Variables|/Game/USCS/Blueprints/SystemForCamera/BP_CameraBP.BP_CameraBP_C|SetSnapCameraSplineDistance%20Offset _scenecamera (Variables|PARAMETERS:|GetSnapCameraSplineDistanceOffset))
          (Variables|/Game/USCS/Blueprints/SystemForCamera/BP_CameraBP.BP_CameraBP_C|SetInterpSpeedLocation _scenecamera (Variables|PARAMETERS:|GetInterp%20Speed%20Location))
          (Variables|/Game/USCS/Blueprints/SystemForCamera/BP_CameraBP.BP_CameraBP_C|SetInterpSpeedRotation _scenecamera (Variables|PARAMETERS:|GetInterp%20Speed%20Rotation))
          (Variables|/Game/USCS/Blueprints/SystemForCamera/BP_CameraBP.BP_CameraBP_C|SetLookAtPlayer? _scenecamera (Variables|PARAMETERS:|GetTrackingPlayer%28CameraRotation%29))
          (Variables|/Game/USCS/Blueprints/SystemForCamera/BP_CameraBP.BP_CameraBP_C|SetLookAtPlayerOffset _scenecamera (Variables|PARAMETERS:|GetTrackingPlayerOffset))
          (Variables|/Game/USCS/Blueprints/SystemForCamera/BP_CameraBP.BP_CameraBP_C|SetUseCameraOffset _scenecamera (Variables|PARAMETERS:|GetUseCameraOffset))
          (Variables|/Game/USCS/Blueprints/SystemForCamera/BP_CameraBP.BP_CameraBP_C|SetBlend%20TimeFromOtherCamera _scenecamera (Variables|PARAMETERS:|GetBlendTimeFromOtherCamera))
          (Variables|/Game/USCS/Blueprints/SystemForCamera/BP_CameraBP.BP_CameraBP_C|SetCameraOffset _scenecamera (Variables|PARAMETERS:|GetCameraOffset))
          (Variables|/Game/USCS/Blueprints/SystemForCamera/BP_CameraBP.BP_CameraBP_C|SetConstraintX,Y,Z_Rotation _scenecamera (Variables|PARAMETERS:|GetConstraint%20X,Y,Z%20Rotation))
          (Variables|/Game/USCS/Blueprints/SystemForCamera/BP_CameraBP.BP_CameraBP_C|SetAntiCameraJitter _scenecamera (Variables|PARAMETERS:SceneCameraSetting:|GetCameraAntiJitter))
          (Variables|/Game/USCS/Blueprints/SystemForCamera/BP_CameraBP.BP_CameraBP_C|SetDebugClampAngles? _scenecamera (Variables|PARAMETERS:|GetDebug%20Clamp%20Angles?))
          (Variables|/Game/USCS/Blueprints/SystemForCamera/BP_CameraBP.BP_CameraBP_C|SetCanControlCameraRotationV? _scenecamera (Variables|PARAMETERS:SceneCameraController:|GetCan%20Control%20Camera%20Rotation%20V?))
          (Variables|/Game/USCS/Blueprints/SystemForCamera/BP_CameraBP.BP_CameraBP_C|SetReverseAxisV? _scenecamera (Variables|PARAMETERS:SceneCameraController:|GetReverse%20Control%20Axis%20V?))
          (Variables|/Game/USCS/Blueprints/SystemForCamera/BP_CameraBP.BP_CameraBP_C|SetAngleMinV: _scenecamera (Variables|PARAMETERS:SceneCameraController:|GetAngle%20Min%20V:))
          (Variables|/Game/USCS/Blueprints/SystemForCamera/BP_CameraBP.BP_CameraBP_C|SetAngleMaxV: _scenecamera (Variables|PARAMETERS:SceneCameraController:|GetAngle%20Max%20V:))
          (Variables|/Game/USCS/Blueprints/SystemForCamera/BP_CameraBP.BP_CameraBP_C|SetCanControlCameraRotationH? _scenecamera (Variables|PARAMETERS:SceneCameraController:|GetCan%20Control%20Camera%20Rotation%20H?))
          (Variables|/Game/USCS/Blueprints/SystemForCamera/BP_CameraBP.BP_CameraBP_C|SetReverseAxisH? _scenecamera (Variables|PARAMETERS:SceneCameraController:|GetReverse%20Control%20Axis%20H?))
          (Variables|/Game/USCS/Blueprints/SystemForCamera/BP_CameraBP.BP_CameraBP_C|SetAngleMinH: _scenecamera (Variables|PARAMETERS:SceneCameraController:|GetAngle%20Min%20H:))
          (Variables|/Game/USCS/Blueprints/SystemForCamera/BP_CameraBP.BP_CameraBP_C|SetAngleMaxH: _scenecamera (Variables|PARAMETERS:SceneCameraController:|GetAngle%20Max%20H:))
          (Variables|/Game/USCS/Blueprints/SystemForCamera/BP_CameraBP.BP_CameraBP_C|SetClampX _scenecamera (Variables|PARAMETERS:|GetClampSlopeL/R))
          (Variables|/Game/USCS/Blueprints/SystemForCamera/BP_CameraBP.BP_CameraBP_C|SetClampY _scenecamera (Variables|PARAMETERS:|GetClampAngleDown/Up))
          (Variables|/Game/USCS/Blueprints/SystemForCamera/BP_CameraBP.BP_CameraBP_C|SetClampZ _scenecamera (- (Variables|PARAMETERS:|GetClampAngleL/R) 9e+01))
          (Variables|/Game/USCS/Blueprints/SystemForCamera/BP_CameraBP.BP_CameraBP_C|SetUsePawnControlRotationn _scenecamera (Variables|PARAMETERS:SceneCameraSetting:|GetUsePawnControlRotation))
          (Variables|/Game/USCS/Blueprints/SystemForCamera/BP_CameraBP.BP_CameraBP_C|SetInherittPitch _scenecamera (Variables|PARAMETERS:SceneCameraSetting:|GetInherit%20Pitch))
          (Variables|/Game/USCS/Blueprints/SystemForCamera/BP_CameraBP.BP_CameraBP_C|SetInherittYaw _scenecamera (Variables|PARAMETERS:SceneCameraSetting:|GetInherit%20Yaw))
          (Variables|/Game/USCS/Blueprints/SystemForCamera/BP_CameraBP.BP_CameraBP_C|SetInherittRoll _scenecamera (Variables|PARAMETERS:SceneCameraSetting:|GetInherit%20Roll))
          (Variables|/Game/USCS/Blueprints/SystemForCamera/BP_CameraBP.BP_CameraBP_C|SetCamera%20Spring%20Lag _scenecamera (Variables|PARAMETERS:SceneCameraLag:|GetEnable%20Camera%20Lag))
          (Variables|/Game/USCS/Blueprints/SystemForCamera/BP_CameraBP.BP_CameraBP_C|SetCamera%20Spring%20Lag%20Rotation _scenecamera (Variables|PARAMETERS:SceneCameraLag:|GetEnable%20Camera%20Rotation%20Lag))
          (Variables|/Game/USCS/Blueprints/SystemForCamera/BP_CameraBP.BP_CameraBP_C|SetCamera%20Spring%20Lag%20Speed _scenecamera (Variables|PARAMETERS:SceneCameraLag:|GetCamera%20Lag%20Speed))
          (Variables|/Game/USCS/Blueprints/SystemForCamera/BP_CameraBP.BP_CameraBP_C|SetCamera%20Spring%20Lag%20Rotation%20Speed _scenecamera (Variables|PARAMETERS:SceneCameraLag:|GetCamera%20Rotation%20Lag%20Speed))
          (Variables|/Game/USCS/Blueprints/SystemForCamera/BP_CameraBP.BP_CameraBP_C|SetCamera%20Lag%20Maxx%20Distance _scenecamera (Variables|PARAMETERS:SceneCameraLag:|GetCamera%20Lag%20Max%20Distance))
          (if (Variables|/Game/USCS/Blueprints/SystemForCamera/BP_CameraBP.BP_CameraBP_C|GetIsCameraInitiated? (Variables|PARAMETERS:|GetSceneCamera))
            (if (Variables|Default|GetPreviousZoneInfluWasA_UscsZoneInflu)
              (for (_array_element_3 _array_index) (Variables|Default|GetUscsForCameraBP_Ref) :!label _label_2
                (if (Variables|BP_USCS_ForCameraBP_C|GetIsActivated? _array_element_3)
                  (Variables|BP_USCS_ForCameraBP_C|SetCurrentUSCS_ForCameraBP_Index _array_element_3 _array_index)
                  (if (not (== (Variables|Default|GetCurrentUSCS_ForCameraBP_Index) (Variables|Default|GetPreviousUSCS_ForCameraBP_Index)))
                    (if (Variables|PARAMETERS:|GetInstantCameraView%28NoBlend%29)
                      (Default|BacktoCameraBP (Variables|PARAMETERS:|GetSceneCamera)))
                    (for _array_element_4 (Variables|Default|GetUscsForCameraBP_Ref)
                      (Variables|BP_USCS_ForCameraBP_C|SetPreviousUSCS_ForCameraBP_Index _array_element_4 (Variables|Default|GetCurrentUSCS_ForCameraBP_Index))))
                  (else
                    (Variables|BP_USCS_ForCameraBP_C|SetCurrentUSCS_ForCameraBP_Index _array_element_3 -1)
                    (Variables|BP_USCS_ForCameraBP_C|SetPreviousUSCS_ForCameraBP_Index _array_element_3 -1))))
              (else
                (if (Variables|PARAMETERS:|GetIsGameStartCamera?) :!label _label_3
                  (Utilities|FlowControl|Sequence
                    (:then_0
                      (Utilities|FlowControl|Delay 0.2)
                      (Variables|PARAMETERS:|SetIsGameStartCamera? false))
                    (:then_1
                      (Default|BacktoCameraBP (Variables|PARAMETERS:|GetSceneCamera) :!label _label_4)
                      (Variables|Default|SetPreviousZoneInfluWasA_UscsZoneInflu true)
                      (goto _label_2)))
                  (else
                    (goto _label_4)))))
            (else
              (goto _label_3))))))))

(event OnComponentBeginOverlap(ZoneInfluenceB)
  (params (OverlappedComponent :type Primitive%20Component%20Object%20Reference) (OtherActor :type Actor%20Object%20Reference) (OtherComp :type Primitive%20Component%20Object%20Reference) (OtherBodyIndex :type Integer) (bFromSweep :type Boolean) (SweepResult :type Hit%20Result%20Structure%20%28by%20ref%29))
  (bind _scenecamera (Variables|PARAMETERS:|GetSceneCamera))
  (bind _splineraildepthon_ (Variables|PARAMETERS:|GetSplineRailDepthOn?))
  (bind _usefadein (Variables|PARAMETRS:FadeIn:|GetUseFadeIn))
  (Utilities|IsPlayerCharacter/Pawn? OtherActor
    (:true
      (bind _displayname (CallFunction|GetUSCSDisplayName))
      (Variables|Default|SetCurrentUSCS_OverlappedB _displayname)
      (Variables|Default|SetIsActivated? true)
      (Utilities|FlowControl|Sequence
        (:then_0
          (Utilities|FlowControl|Sequence
            (:then_0
              (for _array_element (Variables|Default|GetCharacterCameraBP_Ref)
                (Default|BacktoUscs _array_element)))
            (:then_1
              (for _array_element_2 (Variables|Default|GetCameraStaticBP_Ref)
                (Default|BacktoUscs _array_element_2)))
            (:then_2
              (CallFunction|BacktoUscs))))
        (:then_1
          (Actor|Tick|SetActorTickEnabled (or (or _splineraildepthon_ _usefadein) (and _splineraildepthon_ _usefadein)))
          (if (Variables|PARAMETRS:FadeIn:|GetUseFadeIn)
            (if (Utilities|Enum|Equal(Enum) (Variables|Default|GetCurrentUSCS_OverlappedA) (Variables|Default|GetCurrentUSCS_OverlappedB))
              (if (Variables|Default|GetIs%20SwitchBP?)
                (bind _bc_fadeincamerabp (CallFunction|BCFadeinCameraParameters (Variables|PARAMETERS:|GetSceneCamera) (Variables|PARAMETRS:FadeIn:|GetUseFadeIn) (Variables|PARAMETRS:FadeIn:|GetDisable%20Player%20Input%20Controller) (Variables|PARAMETRS:FadeIn:|GetPre%20Fade%20Time) (Variables|PARAMETRS:FadeIn:|GetPre%20Fade%20Color) (Variables|PARAMETRS:FadeIn:|GetPre%20Fade%20Should%20Fade%20Audio) (Variables|PARAMETRS:FadeIn:|GetFade%20Time) (Variables|PARAMETRS:FadeIn:|GetFade%20Color) (Variables|PARAMETRS:FadeIn:|GetFade%20from%20Alpha%28X%29%20to%20Alpha%28Y%29) (Variables|PARAMETRS:FadeIn:|GetShould%20Fade%20Audio?) (Variables|PARAMETRS:FadeIn:|GetHold%20When%20Finished?) :!label _label))
                (Default|BCFadeinSetting _bc_fadeincamerabp))
              (else
                (goto _label))))
          (Variables|/Game/USCS/Blueprints/SystemForCamera/BP_CameraBP.BP_CameraBP_C|SetSpline (Variables|PARAMETERS:|GetSceneCamera) (Variables|Default|GetCameraSpline))
          (Variables|/Game/USCS/Blueprints/SystemForCamera/BP_CameraBP.BP_CameraBP_C|SetIsStartGameCamera? _scenecamera (Variables|PARAMETERS:|GetIsGameStartCamera?))
          (Variables|/Game/USCS/Blueprints/SystemForCamera/BP_CameraBP.BP_CameraBP_C|SetInstantCameraView _scenecamera (Variables|PARAMETERS:|GetInstantCameraView%28NoBlend%29))
          (Variables|/Game/USCS/Blueprints/SystemForCamera/BP_CameraBP.BP_CameraBP_C|SetGameStartCameraBlendTime _scenecamera (Variables|PARAMETERS:|GetGame%20Start%20Camera%20Blend%20Time))
          (Variables|/Game/USCS/Blueprints/SystemForCamera/BP_CameraBP.BP_CameraBP_C|SetSnapCameraSpline? _scenecamera (Variables|PARAMETERS:|GetSnapCameraSpline?))
          (Variables|/Game/USCS/Blueprints/SystemForCamera/BP_CameraBP.BP_CameraBP_C|SetSnapCameraSplineDistance%20Offset _scenecamera (Variables|PARAMETERS:|GetSnapCameraSplineDistanceOffset))
          (Variables|/Game/USCS/Blueprints/SystemForCamera/BP_CameraBP.BP_CameraBP_C|SetInterpSpeedLocation _scenecamera (Variables|PARAMETERS:|GetInterp%20Speed%20Location))
          (Variables|/Game/USCS/Blueprints/SystemForCamera/BP_CameraBP.BP_CameraBP_C|SetInterpSpeedRotation _scenecamera (Variables|PARAMETERS:|GetInterp%20Speed%20Rotation))
          (Variables|/Game/USCS/Blueprints/SystemForCamera/BP_CameraBP.BP_CameraBP_C|SetLookAtPlayer? _scenecamera (Variables|PARAMETERS:|GetTrackingPlayer%28CameraRotation%29))
          (Variables|/Game/USCS/Blueprints/SystemForCamera/BP_CameraBP.BP_CameraBP_C|SetLookAtPlayerOffset _scenecamera (Variables|PARAMETERS:|GetTrackingPlayerOffset))
          (Variables|/Game/USCS/Blueprints/SystemForCamera/BP_CameraBP.BP_CameraBP_C|SetUseCameraOffset _scenecamera (Variables|PARAMETERS:|GetUseCameraOffset))
          (Variables|/Game/USCS/Blueprints/SystemForCamera/BP_CameraBP.BP_CameraBP_C|SetBlend%20TimeFromOtherCamera _scenecamera (Variables|PARAMETERS:|GetBlendTimeFromOtherCamera))
          (Variables|/Game/USCS/Blueprints/SystemForCamera/BP_CameraBP.BP_CameraBP_C|SetCameraOffset _scenecamera (Variables|PARAMETERS:|GetCameraOffset))
          (Variables|/Game/USCS/Blueprints/SystemForCamera/BP_CameraBP.BP_CameraBP_C|SetConstraintX,Y,Z_Rotation _scenecamera (Variables|PARAMETERS:|GetConstraint%20X,Y,Z%20Rotation))
          (Variables|/Game/USCS/Blueprints/SystemForCamera/BP_CameraBP.BP_CameraBP_C|SetAntiCameraJitter _scenecamera (Variables|PARAMETERS:SceneCameraSetting:|GetCameraAntiJitter))
          (Variables|/Game/USCS/Blueprints/SystemForCamera/BP_CameraBP.BP_CameraBP_C|SetDebugClampAngles? _scenecamera (Variables|PARAMETERS:|GetDebug%20Clamp%20Angles?))
          (Variables|/Game/USCS/Blueprints/SystemForCamera/BP_CameraBP.BP_CameraBP_C|SetCanControlCameraRotationV? _scenecamera (Variables|PARAMETERS:SceneCameraController:|GetCan%20Control%20Camera%20Rotation%20V?))
          (Variables|/Game/USCS/Blueprints/SystemForCamera/BP_CameraBP.BP_CameraBP_C|SetReverseAxisV? _scenecamera (Variables|PARAMETERS:SceneCameraController:|GetReverse%20Control%20Axis%20V?))
          (Variables|/Game/USCS/Blueprints/SystemForCamera/BP_CameraBP.BP_CameraBP_C|SetAngleMinV: _scenecamera (Variables|PARAMETERS:SceneCameraController:|GetAngle%20Min%20V:))
          (Variables|/Game/USCS/Blueprints/SystemForCamera/BP_CameraBP.BP_CameraBP_C|SetAngleMaxV: _scenecamera (Variables|PARAMETERS:SceneCameraController:|GetAngle%20Max%20V:))
          (Variables|/Game/USCS/Blueprints/SystemForCamera/BP_CameraBP.BP_CameraBP_C|SetCanControlCameraRotationH? _scenecamera (Variables|PARAMETERS:SceneCameraController:|GetCan%20Control%20Camera%20Rotation%20H?))
          (Variables|/Game/USCS/Blueprints/SystemForCamera/BP_CameraBP.BP_CameraBP_C|SetReverseAxisH? _scenecamera (Variables|PARAMETERS:SceneCameraController:|GetReverse%20Control%20Axis%20H?))
          (Variables|/Game/USCS/Blueprints/SystemForCamera/BP_CameraBP.BP_CameraBP_C|SetAngleMinH: _scenecamera (Variables|PARAMETERS:SceneCameraController:|GetAngle%20Min%20H:))
          (Variables|/Game/USCS/Blueprints/SystemForCamera/BP_CameraBP.BP_CameraBP_C|SetAngleMaxH: _scenecamera (Variables|PARAMETERS:SceneCameraController:|GetAngle%20Max%20H:))
          (Variables|/Game/USCS/Blueprints/SystemForCamera/BP_CameraBP.BP_CameraBP_C|SetClampX _scenecamera (Variables|PARAMETERS:|GetClampSlopeL/R))
          (Variables|/Game/USCS/Blueprints/SystemForCamera/BP_CameraBP.BP_CameraBP_C|SetClampY _scenecamera (Variables|PARAMETERS:|GetClampAngleDown/Up))
          (Variables|/Game/USCS/Blueprints/SystemForCamera/BP_CameraBP.BP_CameraBP_C|SetClampZ _scenecamera (- (Variables|PARAMETERS:|GetClampAngleL/R) 9e+01))
          (Variables|/Game/USCS/Blueprints/SystemForCamera/BP_CameraBP.BP_CameraBP_C|SetUsePawnControlRotationn _scenecamera (Variables|PARAMETERS:SceneCameraSetting:|GetUsePawnControlRotation))
          (Variables|/Game/USCS/Blueprints/SystemForCamera/BP_CameraBP.BP_CameraBP_C|SetInherittPitch _scenecamera (Variables|PARAMETERS:SceneCameraSetting:|GetInherit%20Pitch))
          (Variables|/Game/USCS/Blueprints/SystemForCamera/BP_CameraBP.BP_CameraBP_C|SetInherittYaw _scenecamera (Variables|PARAMETERS:SceneCameraSetting:|GetInherit%20Yaw))
          (Variables|/Game/USCS/Blueprints/SystemForCamera/BP_CameraBP.BP_CameraBP_C|SetInherittRoll _scenecamera (Variables|PARAMETERS:SceneCameraSetting:|GetInherit%20Roll))
          (Variables|/Game/USCS/Blueprints/SystemForCamera/BP_CameraBP.BP_CameraBP_C|SetCamera%20Spring%20Lag _scenecamera (Variables|PARAMETERS:SceneCameraLag:|GetEnable%20Camera%20Lag))
          (Variables|/Game/USCS/Blueprints/SystemForCamera/BP_CameraBP.BP_CameraBP_C|SetCamera%20Spring%20Lag%20Rotation _scenecamera (Variables|PARAMETERS:SceneCameraLag:|GetEnable%20Camera%20Rotation%20Lag))
          (Variables|/Game/USCS/Blueprints/SystemForCamera/BP_CameraBP.BP_CameraBP_C|SetCamera%20Spring%20Lag%20Speed _scenecamera (Variables|PARAMETERS:SceneCameraLag:|GetCamera%20Lag%20Speed))
          (Variables|/Game/USCS/Blueprints/SystemForCamera/BP_CameraBP.BP_CameraBP_C|SetCamera%20Spring%20Lag%20Rotation%20Speed _scenecamera (Variables|PARAMETERS:SceneCameraLag:|GetCamera%20Rotation%20Lag%20Speed))
          (Variables|/Game/USCS/Blueprints/SystemForCamera/BP_CameraBP.BP_CameraBP_C|SetCamera%20Lag%20Maxx%20Distance _scenecamera (Variables|PARAMETERS:SceneCameraLag:|GetCamera%20Lag%20Max%20Distance))
          (if (Variables|/Game/USCS/Blueprints/SystemForCamera/BP_CameraBP.BP_CameraBP_C|GetIsCameraInitiated? (Variables|PARAMETERS:|GetSceneCamera))
            (if (Variables|Default|GetPreviousZoneInfluWasA_UscsZoneInflu)
              (for (_array_element_3 _array_index) (Variables|Default|GetUscsForCameraBP_Ref) :!label _label_2
                (if (Variables|BP_USCS_ForCameraBP_C|GetIsActivated? _array_element_3)
                  (Variables|BP_USCS_ForCameraBP_C|SetCurrentUSCS_ForCameraBP_Index _array_element_3 _array_index)
                  (if (not (== (Variables|Default|GetCurrentUSCS_ForCameraBP_Index) (Variables|Default|GetPreviousUSCS_ForCameraBP_Index)))
                    (if (Variables|PARAMETERS:|GetInstantCameraView%28NoBlend%29)
                      (Default|BacktoCameraBP (Variables|PARAMETERS:|GetSceneCamera)))
                    (for _array_element_4 (Variables|Default|GetUscsForCameraBP_Ref)
                      (Variables|BP_USCS_ForCameraBP_C|SetPreviousUSCS_ForCameraBP_Index _array_element_4 (Variables|Default|GetCurrentUSCS_ForCameraBP_Index))))
                  (else
                    (Variables|BP_USCS_ForCameraBP_C|SetCurrentUSCS_ForCameraBP_Index _array_element_3 -1)
                    (Variables|BP_USCS_ForCameraBP_C|SetPreviousUSCS_ForCameraBP_Index _array_element_3 -1))))
              (else
                (if (Variables|PARAMETERS:|GetIsGameStartCamera?) :!label _label_3
                  (Utilities|FlowControl|Sequence
                    (:then_0
                      (Utilities|FlowControl|Delay 0.2)
                      (Variables|PARAMETERS:|SetIsGameStartCamera? false))
                    (:then_1
                      (Default|BacktoCameraBP (Variables|PARAMETERS:|GetSceneCamera) :!label _label_4)
                      (Variables|Default|SetPreviousZoneInfluWasA_UscsZoneInflu true)
                      (goto _label_2)))
                  (else
                    (goto _label_4)))))
            (else
              (goto _label_3))))))))

(event Custom|Initalize%20USCS
  (bind _scenecamera (Variables|PARAMETERS:|GetSceneCamera))
  (bind _splineraildepthon_ (Variables|PARAMETERS:|GetSplineRailDepthOn?))
  (bind _usefadein (Variables|PARAMETRS:FadeIn:|GetUseFadeIn))
  (Variables|Default|SetIs%20SwitchBP? false)
  (Utilities|FlowControl|Sequence
    (:then_0
      (Variables|Default|SetIsOverlappingBP_ZoneInfluencerActivator? false)
      (Actor|Tick|SetActorTickEnabled false)
      (Utilities|FlowControl|Sequence
        (:then_0
          (Utilities|FlowControl|Delay 0.0)
          (Variables|Default|SetIsInsideZoneInfluencer? (CallFunction|PlayerIsoverlappingOneZoneInfluencer))
          (if (Variables|Default|GetIsInsideZoneInfluencer?)
            (Variables|Default|SetPreviousZoneInfluWasA_UscsZoneInflu true)
            (bind _displayname (CallFunction|GetUSCSDisplayName))
            (Variables|Default|SetCurrentUSCS_OverlappedA _displayname)
            (Variables|Default|SetCurrentUSCS_OverlappedB _displayname)
            (Variables|Default|SetIsActivated? true)
            (Utilities|FlowControl|Sequence
              (:then_0
                (Actor|Tick|SetActorTickEnabled (or (or _splineraildepthon_ _usefadein) (and _splineraildepthon_ _usefadein)) :!label _label)
                (if (Variables|PARAMETRS:FadeIn:|GetUseFadeIn)
                  (if (Utilities|Enum|Equal(Enum) (Variables|Default|GetCurrentUSCS_OverlappedA) (Variables|Default|GetCurrentUSCS_OverlappedB))
                    (if (Variables|Default|GetIs%20SwitchBP?)
                      (bind _bc_fadeincamerabp (CallFunction|BCFadeinCameraParameters (Variables|PARAMETERS:|GetSceneCamera) (Variables|PARAMETRS:FadeIn:|GetUseFadeIn) (Variables|PARAMETRS:FadeIn:|GetDisable%20Player%20Input%20Controller) (Variables|PARAMETRS:FadeIn:|GetPre%20Fade%20Time) (Variables|PARAMETRS:FadeIn:|GetPre%20Fade%20Color) (Variables|PARAMETRS:FadeIn:|GetPre%20Fade%20Should%20Fade%20Audio) (Variables|PARAMETRS:FadeIn:|GetFade%20Time) (Variables|PARAMETRS:FadeIn:|GetFade%20Color) (Variables|PARAMETRS:FadeIn:|GetFade%20from%20Alpha%28X%29%20to%20Alpha%28Y%29) (Variables|PARAMETRS:FadeIn:|GetShould%20Fade%20Audio?) (Variables|PARAMETRS:FadeIn:|GetHold%20When%20Finished?) :!label _label_2))
                      (Default|BCFadeinSetting _bc_fadeincamerabp))
                    (else
                      (goto _label_2))))
                (Variables|/Game/USCS/Blueprints/SystemForCamera/BP_CameraBP.BP_CameraBP_C|SetSpline (Variables|PARAMETERS:|GetSceneCamera) (Variables|Default|GetCameraSpline))
                (Variables|/Game/USCS/Blueprints/SystemForCamera/BP_CameraBP.BP_CameraBP_C|SetIsStartGameCamera? _scenecamera (Variables|PARAMETERS:|GetIsGameStartCamera?))
                (Variables|/Game/USCS/Blueprints/SystemForCamera/BP_CameraBP.BP_CameraBP_C|SetInstantCameraView _scenecamera (Variables|PARAMETERS:|GetInstantCameraView%28NoBlend%29))
                (Variables|/Game/USCS/Blueprints/SystemForCamera/BP_CameraBP.BP_CameraBP_C|SetGameStartCameraBlendTime _scenecamera (Variables|PARAMETERS:|GetGame%20Start%20Camera%20Blend%20Time))
                (Variables|/Game/USCS/Blueprints/SystemForCamera/BP_CameraBP.BP_CameraBP_C|SetSnapCameraSpline? _scenecamera (Variables|PARAMETERS:|GetSnapCameraSpline?))
                (Variables|/Game/USCS/Blueprints/SystemForCamera/BP_CameraBP.BP_CameraBP_C|SetSnapCameraSplineDistance%20Offset _scenecamera (Variables|PARAMETERS:|GetSnapCameraSplineDistanceOffset))
                (Variables|/Game/USCS/Blueprints/SystemForCamera/BP_CameraBP.BP_CameraBP_C|SetInterpSpeedLocation _scenecamera (Variables|PARAMETERS:|GetInterp%20Speed%20Location))
                (Variables|/Game/USCS/Blueprints/SystemForCamera/BP_CameraBP.BP_CameraBP_C|SetInterpSpeedRotation _scenecamera (Variables|PARAMETERS:|GetInterp%20Speed%20Rotation))
                (Variables|/Game/USCS/Blueprints/SystemForCamera/BP_CameraBP.BP_CameraBP_C|SetLookAtPlayer? _scenecamera (Variables|PARAMETERS:|GetTrackingPlayer%28CameraRotation%29))
                (Variables|/Game/USCS/Blueprints/SystemForCamera/BP_CameraBP.BP_CameraBP_C|SetLookAtPlayerOffset _scenecamera (Variables|PARAMETERS:|GetTrackingPlayerOffset))
                (Variables|/Game/USCS/Blueprints/SystemForCamera/BP_CameraBP.BP_CameraBP_C|SetUseCameraOffset _scenecamera (Variables|PARAMETERS:|GetUseCameraOffset))
                (Variables|/Game/USCS/Blueprints/SystemForCamera/BP_CameraBP.BP_CameraBP_C|SetBlend%20TimeFromOtherCamera _scenecamera (Variables|PARAMETERS:|GetBlendTimeFromOtherCamera))
                (Variables|/Game/USCS/Blueprints/SystemForCamera/BP_CameraBP.BP_CameraBP_C|SetCameraOffset _scenecamera (Variables|PARAMETERS:|GetCameraOffset))
                (Variables|/Game/USCS/Blueprints/SystemForCamera/BP_CameraBP.BP_CameraBP_C|SetConstraintX,Y,Z_Rotation _scenecamera (Variables|PARAMETERS:|GetConstraint%20X,Y,Z%20Rotation))
                (Variables|/Game/USCS/Blueprints/SystemForCamera/BP_CameraBP.BP_CameraBP_C|SetAntiCameraJitter _scenecamera (Variables|PARAMETERS:SceneCameraSetting:|GetCameraAntiJitter))
                (Variables|/Game/USCS/Blueprints/SystemForCamera/BP_CameraBP.BP_CameraBP_C|SetDebugClampAngles? _scenecamera (Variables|PARAMETERS:|GetDebug%20Clamp%20Angles?))
                (Variables|/Game/USCS/Blueprints/SystemForCamera/BP_CameraBP.BP_CameraBP_C|SetCanControlCameraRotationV? _scenecamera (Variables|PARAMETERS:SceneCameraController:|GetCan%20Control%20Camera%20Rotation%20V?))
                (Variables|/Game/USCS/Blueprints/SystemForCamera/BP_CameraBP.BP_CameraBP_C|SetReverseAxisV? _scenecamera (Variables|PARAMETERS:SceneCameraController:|GetReverse%20Control%20Axis%20V?))
                (Variables|/Game/USCS/Blueprints/SystemForCamera/BP_CameraBP.BP_CameraBP_C|SetAngleMinV: _scenecamera (Variables|PARAMETERS:SceneCameraController:|GetAngle%20Min%20V:))
                (Variables|/Game/USCS/Blueprints/SystemForCamera/BP_CameraBP.BP_CameraBP_C|SetAngleMaxV: _scenecamera (Variables|PARAMETERS:SceneCameraController:|GetAngle%20Max%20V:))
                (Variables|/Game/USCS/Blueprints/SystemForCamera/BP_CameraBP.BP_CameraBP_C|SetCanControlCameraRotationH? _scenecamera (Variables|PARAMETERS:SceneCameraController:|GetCan%20Control%20Camera%20Rotation%20H?))
                (Variables|/Game/USCS/Blueprints/SystemForCamera/BP_CameraBP.BP_CameraBP_C|SetReverseAxisH? _scenecamera (Variables|PARAMETERS:SceneCameraController:|GetReverse%20Control%20Axis%20H?))
                (Variables|/Game/USCS/Blueprints/SystemForCamera/BP_CameraBP.BP_CameraBP_C|SetAngleMinH: _scenecamera (Variables|PARAMETERS:SceneCameraController:|GetAngle%20Min%20H:))
                (Variables|/Game/USCS/Blueprints/SystemForCamera/BP_CameraBP.BP_CameraBP_C|SetAngleMaxH: _scenecamera (Variables|PARAMETERS:SceneCameraController:|GetAngle%20Max%20H:))
                (Variables|/Game/USCS/Blueprints/SystemForCamera/BP_CameraBP.BP_CameraBP_C|SetClampX _scenecamera (Variables|PARAMETERS:|GetClampSlopeL/R))
                (Variables|/Game/USCS/Blueprints/SystemForCamera/BP_CameraBP.BP_CameraBP_C|SetClampY _scenecamera (Variables|PARAMETERS:|GetClampAngleDown/Up))
                (Variables|/Game/USCS/Blueprints/SystemForCamera/BP_CameraBP.BP_CameraBP_C|SetClampZ _scenecamera (- (Variables|PARAMETERS:|GetClampAngleL/R) 9e+01))
                (Variables|/Game/USCS/Blueprints/SystemForCamera/BP_CameraBP.BP_CameraBP_C|SetUsePawnControlRotationn _scenecamera (Variables|PARAMETERS:SceneCameraSetting:|GetUsePawnControlRotation))
                (Variables|/Game/USCS/Blueprints/SystemForCamera/BP_CameraBP.BP_CameraBP_C|SetInherittPitch _scenecamera (Variables|PARAMETERS:SceneCameraSetting:|GetInherit%20Pitch))
                (Variables|/Game/USCS/Blueprints/SystemForCamera/BP_CameraBP.BP_CameraBP_C|SetInherittYaw _scenecamera (Variables|PARAMETERS:SceneCameraSetting:|GetInherit%20Yaw))
                (Variables|/Game/USCS/Blueprints/SystemForCamera/BP_CameraBP.BP_CameraBP_C|SetInherittRoll _scenecamera (Variables|PARAMETERS:SceneCameraSetting:|GetInherit%20Roll))
                (Variables|/Game/USCS/Blueprints/SystemForCamera/BP_CameraBP.BP_CameraBP_C|SetCamera%20Spring%20Lag _scenecamera (Variables|PARAMETERS:SceneCameraLag:|GetEnable%20Camera%20Lag))
                (Variables|/Game/USCS/Blueprints/SystemForCamera/BP_CameraBP.BP_CameraBP_C|SetCamera%20Spring%20Lag%20Rotation _scenecamera (Variables|PARAMETERS:SceneCameraLag:|GetEnable%20Camera%20Rotation%20Lag))
                (Variables|/Game/USCS/Blueprints/SystemForCamera/BP_CameraBP.BP_CameraBP_C|SetCamera%20Spring%20Lag%20Speed _scenecamera (Variables|PARAMETERS:SceneCameraLag:|GetCamera%20Lag%20Speed))
                (Variables|/Game/USCS/Blueprints/SystemForCamera/BP_CameraBP.BP_CameraBP_C|SetCamera%20Spring%20Lag%20Rotation%20Speed _scenecamera (Variables|PARAMETERS:SceneCameraLag:|GetCamera%20Rotation%20Lag%20Speed))
                (Variables|/Game/USCS/Blueprints/SystemForCamera/BP_CameraBP.BP_CameraBP_C|SetCamera%20Lag%20Maxx%20Distance _scenecamera (Variables|PARAMETERS:SceneCameraLag:|GetCamera%20Lag%20Max%20Distance))
                (if (Variables|/Game/USCS/Blueprints/SystemForCamera/BP_CameraBP.BP_CameraBP_C|GetIsCameraInitiated? (Variables|PARAMETERS:|GetSceneCamera))
                  (if (Variables|Default|GetPreviousZoneInfluWasA_UscsZoneInflu)
                    (for (_array_element _array_index) (Variables|Default|GetUscsForCameraBP_Ref) :!label _label_3
                      (if (Variables|BP_USCS_ForCameraBP_C|GetIsActivated? _array_element)
                        (Variables|BP_USCS_ForCameraBP_C|SetCurrentUSCS_ForCameraBP_Index _array_element _array_index)
                        (if (not (== (Variables|Default|GetCurrentUSCS_ForCameraBP_Index) (Variables|Default|GetPreviousUSCS_ForCameraBP_Index)))
                          (if (Variables|PARAMETERS:|GetInstantCameraView%28NoBlend%29)
                            (Default|BacktoCameraBP (Variables|PARAMETERS:|GetSceneCamera)))
                          (for _array_element_2 (Variables|Default|GetUscsForCameraBP_Ref)
                            (Variables|BP_USCS_ForCameraBP_C|SetPreviousUSCS_ForCameraBP_Index _array_element_2 (Variables|Default|GetCurrentUSCS_ForCameraBP_Index))))
                        (else
                          (Variables|BP_USCS_ForCameraBP_C|SetCurrentUSCS_ForCameraBP_Index _array_element -1)
                          (Variables|BP_USCS_ForCameraBP_C|SetPreviousUSCS_ForCameraBP_Index _array_element -1))))
                    (else
                      (if (Variables|PARAMETERS:|GetIsGameStartCamera?) :!label _label_4
                        (Utilities|FlowControl|Sequence
                          (:then_0
                            (Utilities|FlowControl|Delay 0.2)
                            (Variables|PARAMETERS:|SetIsGameStartCamera? false))
                          (:then_1
                            (Default|BacktoCameraBP (Variables|PARAMETERS:|GetSceneCamera) :!label _label_5)
                            (Variables|Default|SetPreviousZoneInfluWasA_UscsZoneInflu true)
                            (goto _label_3)))
                        (else
                          (goto _label_5)))))
                  (else
                    (goto _label_4))))
              (:then_1
                (goto _label_5)))
            (else
              (Variables|Default|SetPreviousZoneInfluWasA_UscsZoneInflu false)
              (if (Variables|PARAMETERS:|GetIsGameStartCamera?)
                (Variables|Default|SetIsActivated? true)
                (goto _label)
                (else
                  (Variables|Default|SetIsActivated? false)
                  (for _array_element_3 (Variables|Default|GetUscsForCameraBP_Ref)
                    (Variables|BP_USCS_ForCameraBP_C|SetPreviousZoneInfluWasA_UscsZoneInflu _array_element_3 true)))))))
        (:then_1
          (bind _outactors (Actor|GetAllActorsOfClass "BP_USCS_ForCameraBP_C"))
          (Variables|Default|SetUscsForCameraBP_Ref _outactors))))
    (:then_1
      (for (_array_element_4 _array_index_2) (Variables|Default|GetUscsForCameraBP_Ref)
        (Variables|BP_USCS_ForCameraBP_C|SetCurrentUSCS_ForCameraBP_Index _array_element_4 _array_index_2)
        (Variables|BP_USCS_ForCameraBP_C|SetPreviousUSCS_ForCameraBP_Index _array_element_4 _array_index_2)))))

(event Custom|ForceGlobalActivation
  (bind _scenecamera (Variables|PARAMETERS:|GetSceneCamera))
  (bind _splineraildepthon_ (Variables|PARAMETERS:|GetSplineRailDepthOn?))
  (bind _usefadein (Variables|PARAMETRS:FadeIn:|GetUseFadeIn))
  (Utilities|FlowControl|Sequence
    (:then_0
      (Variables|Default|SetIsOverlappingBP_ZoneInfluencerActivator? false)
      (Actor|Tick|SetActorTickEnabled false)
      (Utilities|FlowControl|Sequence
        (:then_0
          (Utilities|FlowControl|Delay 0.0)
          (Variables|Default|SetIsInsideZoneInfluencer? (CallFunction|PlayerIsoverlappingOneZoneInfluencer))
          (if (Variables|Default|GetIsInsideZoneInfluencer?)
            (Variables|Default|SetPreviousZoneInfluWasA_UscsZoneInflu true)
            (bind _displayname (CallFunction|GetUSCSDisplayName))
            (Variables|Default|SetCurrentUSCS_OverlappedA _displayname)
            (Variables|Default|SetCurrentUSCS_OverlappedB _displayname)
            (Variables|Default|SetIsActivated? true)
            (Utilities|FlowControl|Sequence
              (:then_0
                (Actor|Tick|SetActorTickEnabled (or (or _splineraildepthon_ _usefadein) (and _splineraildepthon_ _usefadein)) :!label _label)
                (if (Variables|PARAMETRS:FadeIn:|GetUseFadeIn)
                  (if (Utilities|Enum|Equal(Enum) (Variables|Default|GetCurrentUSCS_OverlappedA) (Variables|Default|GetCurrentUSCS_OverlappedB))
                    (if (Variables|Default|GetIs%20SwitchBP?)
                      (bind _bc_fadeincamerabp (CallFunction|BCFadeinCameraParameters (Variables|PARAMETERS:|GetSceneCamera) (Variables|PARAMETRS:FadeIn:|GetUseFadeIn) (Variables|PARAMETRS:FadeIn:|GetDisable%20Player%20Input%20Controller) (Variables|PARAMETRS:FadeIn:|GetPre%20Fade%20Time) (Variables|PARAMETRS:FadeIn:|GetPre%20Fade%20Color) (Variables|PARAMETRS:FadeIn:|GetPre%20Fade%20Should%20Fade%20Audio) (Variables|PARAMETRS:FadeIn:|GetFade%20Time) (Variables|PARAMETRS:FadeIn:|GetFade%20Color) (Variables|PARAMETRS:FadeIn:|GetFade%20from%20Alpha%28X%29%20to%20Alpha%28Y%29) (Variables|PARAMETRS:FadeIn:|GetShould%20Fade%20Audio?) (Variables|PARAMETRS:FadeIn:|GetHold%20When%20Finished?) :!label _label_2))
                      (Default|BCFadeinSetting _bc_fadeincamerabp))
                    (else
                      (goto _label_2))))
                (Variables|/Game/USCS/Blueprints/SystemForCamera/BP_CameraBP.BP_CameraBP_C|SetSpline (Variables|PARAMETERS:|GetSceneCamera) (Variables|Default|GetCameraSpline))
                (Variables|/Game/USCS/Blueprints/SystemForCamera/BP_CameraBP.BP_CameraBP_C|SetIsStartGameCamera? _scenecamera (Variables|PARAMETERS:|GetIsGameStartCamera?))
                (Variables|/Game/USCS/Blueprints/SystemForCamera/BP_CameraBP.BP_CameraBP_C|SetInstantCameraView _scenecamera (Variables|PARAMETERS:|GetInstantCameraView%28NoBlend%29))
                (Variables|/Game/USCS/Blueprints/SystemForCamera/BP_CameraBP.BP_CameraBP_C|SetGameStartCameraBlendTime _scenecamera (Variables|PARAMETERS:|GetGame%20Start%20Camera%20Blend%20Time))
                (Variables|/Game/USCS/Blueprints/SystemForCamera/BP_CameraBP.BP_CameraBP_C|SetSnapCameraSpline? _scenecamera (Variables|PARAMETERS:|GetSnapCameraSpline?))
                (Variables|/Game/USCS/Blueprints/SystemForCamera/BP_CameraBP.BP_CameraBP_C|SetSnapCameraSplineDistance%20Offset _scenecamera (Variables|PARAMETERS:|GetSnapCameraSplineDistanceOffset))
                (Variables|/Game/USCS/Blueprints/SystemForCamera/BP_CameraBP.BP_CameraBP_C|SetInterpSpeedLocation _scenecamera (Variables|PARAMETERS:|GetInterp%20Speed%20Location))
                (Variables|/Game/USCS/Blueprints/SystemForCamera/BP_CameraBP.BP_CameraBP_C|SetInterpSpeedRotation _scenecamera (Variables|PARAMETERS:|GetInterp%20Speed%20Rotation))
                (Variables|/Game/USCS/Blueprints/SystemForCamera/BP_CameraBP.BP_CameraBP_C|SetLookAtPlayer? _scenecamera (Variables|PARAMETERS:|GetTrackingPlayer%28CameraRotation%29))
                (Variables|/Game/USCS/Blueprints/SystemForCamera/BP_CameraBP.BP_CameraBP_C|SetLookAtPlayerOffset _scenecamera (Variables|PARAMETERS:|GetTrackingPlayerOffset))
                (Variables|/Game/USCS/Blueprints/SystemForCamera/BP_CameraBP.BP_CameraBP_C|SetUseCameraOffset _scenecamera (Variables|PARAMETERS:|GetUseCameraOffset))
                (Variables|/Game/USCS/Blueprints/SystemForCamera/BP_CameraBP.BP_CameraBP_C|SetBlend%20TimeFromOtherCamera _scenecamera (Variables|PARAMETERS:|GetBlendTimeFromOtherCamera))
                (Variables|/Game/USCS/Blueprints/SystemForCamera/BP_CameraBP.BP_CameraBP_C|SetCameraOffset _scenecamera (Variables|PARAMETERS:|GetCameraOffset))
                (Variables|/Game/USCS/Blueprints/SystemForCamera/BP_CameraBP.BP_CameraBP_C|SetConstraintX,Y,Z_Rotation _scenecamera (Variables|PARAMETERS:|GetConstraint%20X,Y,Z%20Rotation))
                (Variables|/Game/USCS/Blueprints/SystemForCamera/BP_CameraBP.BP_CameraBP_C|SetAntiCameraJitter _scenecamera (Variables|PARAMETERS:SceneCameraSetting:|GetCameraAntiJitter))
                (Variables|/Game/USCS/Blueprints/SystemForCamera/BP_CameraBP.BP_CameraBP_C|SetDebugClampAngles? _scenecamera (Variables|PARAMETERS:|GetDebug%20Clamp%20Angles?))
                (Variables|/Game/USCS/Blueprints/SystemForCamera/BP_CameraBP.BP_CameraBP_C|SetCanControlCameraRotationV? _scenecamera (Variables|PARAMETERS:SceneCameraController:|GetCan%20Control%20Camera%20Rotation%20V?))
                (Variables|/Game/USCS/Blueprints/SystemForCamera/BP_CameraBP.BP_CameraBP_C|SetReverseAxisV? _scenecamera (Variables|PARAMETERS:SceneCameraController:|GetReverse%20Control%20Axis%20V?))
                (Variables|/Game/USCS/Blueprints/SystemForCamera/BP_CameraBP.BP_CameraBP_C|SetAngleMinV: _scenecamera (Variables|PARAMETERS:SceneCameraController:|GetAngle%20Min%20V:))
                (Variables|/Game/USCS/Blueprints/SystemForCamera/BP_CameraBP.BP_CameraBP_C|SetAngleMaxV: _scenecamera (Variables|PARAMETERS:SceneCameraController:|GetAngle%20Max%20V:))
                (Variables|/Game/USCS/Blueprints/SystemForCamera/BP_CameraBP.BP_CameraBP_C|SetCanControlCameraRotationH? _scenecamera (Variables|PARAMETERS:SceneCameraController:|GetCan%20Control%20Camera%20Rotation%20H?))
                (Variables|/Game/USCS/Blueprints/SystemForCamera/BP_CameraBP.BP_CameraBP_C|SetReverseAxisH? _scenecamera (Variables|PARAMETERS:SceneCameraController:|GetReverse%20Control%20Axis%20H?))
                (Variables|/Game/USCS/Blueprints/SystemForCamera/BP_CameraBP.BP_CameraBP_C|SetAngleMinH: _scenecamera (Variables|PARAMETERS:SceneCameraController:|GetAngle%20Min%20H:))
                (Variables|/Game/USCS/Blueprints/SystemForCamera/BP_CameraBP.BP_CameraBP_C|SetAngleMaxH: _scenecamera (Variables|PARAMETERS:SceneCameraController:|GetAngle%20Max%20H:))
                (Variables|/Game/USCS/Blueprints/SystemForCamera/BP_CameraBP.BP_CameraBP_C|SetClampX _scenecamera (Variables|PARAMETERS:|GetClampSlopeL/R))
                (Variables|/Game/USCS/Blueprints/SystemForCamera/BP_CameraBP.BP_CameraBP_C|SetClampY _scenecamera (Variables|PARAMETERS:|GetClampAngleDown/Up))
                (Variables|/Game/USCS/Blueprints/SystemForCamera/BP_CameraBP.BP_CameraBP_C|SetClampZ _scenecamera (- (Variables|PARAMETERS:|GetClampAngleL/R) 9e+01))
                (Variables|/Game/USCS/Blueprints/SystemForCamera/BP_CameraBP.BP_CameraBP_C|SetUsePawnControlRotationn _scenecamera (Variables|PARAMETERS:SceneCameraSetting:|GetUsePawnControlRotation))
                (Variables|/Game/USCS/Blueprints/SystemForCamera/BP_CameraBP.BP_CameraBP_C|SetInherittPitch _scenecamera (Variables|PARAMETERS:SceneCameraSetting:|GetInherit%20Pitch))
                (Variables|/Game/USCS/Blueprints/SystemForCamera/BP_CameraBP.BP_CameraBP_C|SetInherittYaw _scenecamera (Variables|PARAMETERS:SceneCameraSetting:|GetInherit%20Yaw))
                (Variables|/Game/USCS/Blueprints/SystemForCamera/BP_CameraBP.BP_CameraBP_C|SetInherittRoll _scenecamera (Variables|PARAMETERS:SceneCameraSetting:|GetInherit%20Roll))
                (Variables|/Game/USCS/Blueprints/SystemForCamera/BP_CameraBP.BP_CameraBP_C|SetCamera%20Spring%20Lag _scenecamera (Variables|PARAMETERS:SceneCameraLag:|GetEnable%20Camera%20Lag))
                (Variables|/Game/USCS/Blueprints/SystemForCamera/BP_CameraBP.BP_CameraBP_C|SetCamera%20Spring%20Lag%20Rotation _scenecamera (Variables|PARAMETERS:SceneCameraLag:|GetEnable%20Camera%20Rotation%20Lag))
                (Variables|/Game/USCS/Blueprints/SystemForCamera/BP_CameraBP.BP_CameraBP_C|SetCamera%20Spring%20Lag%20Speed _scenecamera (Variables|PARAMETERS:SceneCameraLag:|GetCamera%20Lag%20Speed))
                (Variables|/Game/USCS/Blueprints/SystemForCamera/BP_CameraBP.BP_CameraBP_C|SetCamera%20Spring%20Lag%20Rotation%20Speed _scenecamera (Variables|PARAMETERS:SceneCameraLag:|GetCamera%20Rotation%20Lag%20Speed))
                (Variables|/Game/USCS/Blueprints/SystemForCamera/BP_CameraBP.BP_CameraBP_C|SetCamera%20Lag%20Maxx%20Distance _scenecamera (Variables|PARAMETERS:SceneCameraLag:|GetCamera%20Lag%20Max%20Distance))
                (if (Variables|/Game/USCS/Blueprints/SystemForCamera/BP_CameraBP.BP_CameraBP_C|GetIsCameraInitiated? (Variables|PARAMETERS:|GetSceneCamera))
                  (if (Variables|Default|GetPreviousZoneInfluWasA_UscsZoneInflu)
                    (for (_array_element _array_index) (Variables|Default|GetUscsForCameraBP_Ref) :!label _label_3
                      (if (Variables|BP_USCS_ForCameraBP_C|GetIsActivated? _array_element)
                        (Variables|BP_USCS_ForCameraBP_C|SetCurrentUSCS_ForCameraBP_Index _array_element _array_index)
                        (if (not (== (Variables|Default|GetCurrentUSCS_ForCameraBP_Index) (Variables|Default|GetPreviousUSCS_ForCameraBP_Index)))
                          (if (Variables|PARAMETERS:|GetInstantCameraView%28NoBlend%29)
                            (Default|BacktoCameraBP (Variables|PARAMETERS:|GetSceneCamera)))
                          (for _array_element_2 (Variables|Default|GetUscsForCameraBP_Ref)
                            (Variables|BP_USCS_ForCameraBP_C|SetPreviousUSCS_ForCameraBP_Index _array_element_2 (Variables|Default|GetCurrentUSCS_ForCameraBP_Index))))
                        (else
                          (Variables|BP_USCS_ForCameraBP_C|SetCurrentUSCS_ForCameraBP_Index _array_element -1)
                          (Variables|BP_USCS_ForCameraBP_C|SetPreviousUSCS_ForCameraBP_Index _array_element -1))))
                    (else
                      (if (Variables|PARAMETERS:|GetIsGameStartCamera?) :!label _label_4
                        (Utilities|FlowControl|Sequence
                          (:then_0
                            (Utilities|FlowControl|Delay 0.2)
                            (Variables|PARAMETERS:|SetIsGameStartCamera? false))
                          (:then_1
                            (Default|BacktoCameraBP (Variables|PARAMETERS:|GetSceneCamera) :!label _label_5)
                            (Variables|Default|SetPreviousZoneInfluWasA_UscsZoneInflu true)
                            (goto _label_3)))
                        (else
                          (goto _label_5)))))
                  (else
                    (goto _label_4))))
              (:then_1
                (goto _label_5)))
            (else
              (Variables|Default|SetPreviousZoneInfluWasA_UscsZoneInflu false)
              (if (Variables|PARAMETERS:|GetIsGameStartCamera?)
                (Variables|Default|SetIsActivated? true)
                (goto _label)
                (else
                  (Variables|Default|SetIsActivated? false)
                  (for _array_element_3 (Variables|Default|GetUscsForCameraBP_Ref)
                    (Variables|BP_USCS_ForCameraBP_C|SetPreviousZoneInfluWasA_UscsZoneInflu _array_element_3 true)))))))
        (:then_1
          (bind _outactors (Actor|GetAllActorsOfClass "BP_USCS_ForCameraBP_C"))
          (Variables|Default|SetUscsForCameraBP_Ref _outactors))))
    (:then_1
      (for (_array_element_4 _array_index_2) (Variables|Default|GetUscsForCameraBP_Ref)
        (Variables|BP_USCS_ForCameraBP_C|SetCurrentUSCS_ForCameraBP_Index _array_element_4 _array_index_2)
        (Variables|BP_USCS_ForCameraBP_C|SetPreviousUSCS_ForCameraBP_Index _array_element_4 _array_index_2)))))

(event Custom|OverlapBP_ZoneInfluencerActivator
  (bind _scenecamera (Variables|PARAMETERS:|GetSceneCamera))
  (bind _splineraildepthon_ (Variables|PARAMETERS:|GetSplineRailDepthOn?))
  (bind _usefadein (Variables|PARAMETRS:FadeIn:|GetUseFadeIn))
  (Actor|Tick|SetActorTickEnabled (or (or _splineraildepthon_ _usefadein) (and _splineraildepthon_ _usefadein)))
  (if (Variables|PARAMETRS:FadeIn:|GetUseFadeIn)
    (if (Utilities|Enum|Equal(Enum) (Variables|Default|GetCurrentUSCS_OverlappedA) (Variables|Default|GetCurrentUSCS_OverlappedB))
      (if (Variables|Default|GetIs%20SwitchBP?)
        (bind _bc_fadeincamerabp (CallFunction|BCFadeinCameraParameters (Variables|PARAMETERS:|GetSceneCamera) (Variables|PARAMETRS:FadeIn:|GetUseFadeIn) (Variables|PARAMETRS:FadeIn:|GetDisable%20Player%20Input%20Controller) (Variables|PARAMETRS:FadeIn:|GetPre%20Fade%20Time) (Variables|PARAMETRS:FadeIn:|GetPre%20Fade%20Color) (Variables|PARAMETRS:FadeIn:|GetPre%20Fade%20Should%20Fade%20Audio) (Variables|PARAMETRS:FadeIn:|GetFade%20Time) (Variables|PARAMETRS:FadeIn:|GetFade%20Color) (Variables|PARAMETRS:FadeIn:|GetFade%20from%20Alpha%28X%29%20to%20Alpha%28Y%29) (Variables|PARAMETRS:FadeIn:|GetShould%20Fade%20Audio?) (Variables|PARAMETRS:FadeIn:|GetHold%20When%20Finished?) :!label _label))
        (Default|BCFadeinSetting _bc_fadeincamerabp))
      (else
        (goto _label))))
  (Variables|/Game/USCS/Blueprints/SystemForCamera/BP_CameraBP.BP_CameraBP_C|SetSpline (Variables|PARAMETERS:|GetSceneCamera) (Variables|Default|GetCameraSpline))
  (Variables|/Game/USCS/Blueprints/SystemForCamera/BP_CameraBP.BP_CameraBP_C|SetIsStartGameCamera? _scenecamera (Variables|PARAMETERS:|GetIsGameStartCamera?))
  (Variables|/Game/USCS/Blueprints/SystemForCamera/BP_CameraBP.BP_CameraBP_C|SetInstantCameraView _scenecamera (Variables|PARAMETERS:|GetInstantCameraView%28NoBlend%29))
  (Variables|/Game/USCS/Blueprints/SystemForCamera/BP_CameraBP.BP_CameraBP_C|SetGameStartCameraBlendTime _scenecamera (Variables|PARAMETERS:|GetGame%20Start%20Camera%20Blend%20Time))
  (Variables|/Game/USCS/Blueprints/SystemForCamera/BP_CameraBP.BP_CameraBP_C|SetSnapCameraSpline? _scenecamera (Variables|PARAMETERS:|GetSnapCameraSpline?))
  (Variables|/Game/USCS/Blueprints/SystemForCamera/BP_CameraBP.BP_CameraBP_C|SetSnapCameraSplineDistance%20Offset _scenecamera (Variables|PARAMETERS:|GetSnapCameraSplineDistanceOffset))
  (Variables|/Game/USCS/Blueprints/SystemForCamera/BP_CameraBP.BP_CameraBP_C|SetInterpSpeedLocation _scenecamera (Variables|PARAMETERS:|GetInterp%20Speed%20Location))
  (Variables|/Game/USCS/Blueprints/SystemForCamera/BP_CameraBP.BP_CameraBP_C|SetInterpSpeedRotation _scenecamera (Variables|PARAMETERS:|GetInterp%20Speed%20Rotation))
  (Variables|/Game/USCS/Blueprints/SystemForCamera/BP_CameraBP.BP_CameraBP_C|SetLookAtPlayer? _scenecamera (Variables|PARAMETERS:|GetTrackingPlayer%28CameraRotation%29))
  (Variables|/Game/USCS/Blueprints/SystemForCamera/BP_CameraBP.BP_CameraBP_C|SetLookAtPlayerOffset _scenecamera (Variables|PARAMETERS:|GetTrackingPlayerOffset))
  (Variables|/Game/USCS/Blueprints/SystemForCamera/BP_CameraBP.BP_CameraBP_C|SetUseCameraOffset _scenecamera (Variables|PARAMETERS:|GetUseCameraOffset))
  (Variables|/Game/USCS/Blueprints/SystemForCamera/BP_CameraBP.BP_CameraBP_C|SetBlend%20TimeFromOtherCamera _scenecamera (Variables|PARAMETERS:|GetBlendTimeFromOtherCamera))
  (Variables|/Game/USCS/Blueprints/SystemForCamera/BP_CameraBP.BP_CameraBP_C|SetCameraOffset _scenecamera (Variables|PARAMETERS:|GetCameraOffset))
  (Variables|/Game/USCS/Blueprints/SystemForCamera/BP_CameraBP.BP_CameraBP_C|SetConstraintX,Y,Z_Rotation _scenecamera (Variables|PARAMETERS:|GetConstraint%20X,Y,Z%20Rotation))
  (Variables|/Game/USCS/Blueprints/SystemForCamera/BP_CameraBP.BP_CameraBP_C|SetAntiCameraJitter _scenecamera (Variables|PARAMETERS:SceneCameraSetting:|GetCameraAntiJitter))
  (Variables|/Game/USCS/Blueprints/SystemForCamera/BP_CameraBP.BP_CameraBP_C|SetDebugClampAngles? _scenecamera (Variables|PARAMETERS:|GetDebug%20Clamp%20Angles?))
  (Variables|/Game/USCS/Blueprints/SystemForCamera/BP_CameraBP.BP_CameraBP_C|SetCanControlCameraRotationV? _scenecamera (Variables|PARAMETERS:SceneCameraController:|GetCan%20Control%20Camera%20Rotation%20V?))
  (Variables|/Game/USCS/Blueprints/SystemForCamera/BP_CameraBP.BP_CameraBP_C|SetReverseAxisV? _scenecamera (Variables|PARAMETERS:SceneCameraController:|GetReverse%20Control%20Axis%20V?))
  (Variables|/Game/USCS/Blueprints/SystemForCamera/BP_CameraBP.BP_CameraBP_C|SetAngleMinV: _scenecamera (Variables|PARAMETERS:SceneCameraController:|GetAngle%20Min%20V:))
  (Variables|/Game/USCS/Blueprints/SystemForCamera/BP_CameraBP.BP_CameraBP_C|SetAngleMaxV: _scenecamera (Variables|PARAMETERS:SceneCameraController:|GetAngle%20Max%20V:))
  (Variables|/Game/USCS/Blueprints/SystemForCamera/BP_CameraBP.BP_CameraBP_C|SetCanControlCameraRotationH? _scenecamera (Variables|PARAMETERS:SceneCameraController:|GetCan%20Control%20Camera%20Rotation%20H?))
  (Variables|/Game/USCS/Blueprints/SystemForCamera/BP_CameraBP.BP_CameraBP_C|SetReverseAxisH? _scenecamera (Variables|PARAMETERS:SceneCameraController:|GetReverse%20Control%20Axis%20H?))
  (Variables|/Game/USCS/Blueprints/SystemForCamera/BP_CameraBP.BP_CameraBP_C|SetAngleMinH: _scenecamera (Variables|PARAMETERS:SceneCameraController:|GetAngle%20Min%20H:))
  (Variables|/Game/USCS/Blueprints/SystemForCamera/BP_CameraBP.BP_CameraBP_C|SetAngleMaxH: _scenecamera (Variables|PARAMETERS:SceneCameraController:|GetAngle%20Max%20H:))
  (Variables|/Game/USCS/Blueprints/SystemForCamera/BP_CameraBP.BP_CameraBP_C|SetClampX _scenecamera (Variables|PARAMETERS:|GetClampSlopeL/R))
  (Variables|/Game/USCS/Blueprints/SystemForCamera/BP_CameraBP.BP_CameraBP_C|SetClampY _scenecamera (Variables|PARAMETERS:|GetClampAngleDown/Up))
  (Variables|/Game/USCS/Blueprints/SystemForCamera/BP_CameraBP.BP_CameraBP_C|SetClampZ _scenecamera (- (Variables|PARAMETERS:|GetClampAngleL/R) 9e+01))
  (Variables|/Game/USCS/Blueprints/SystemForCamera/BP_CameraBP.BP_CameraBP_C|SetUsePawnControlRotationn _scenecamera (Variables|PARAMETERS:SceneCameraSetting:|GetUsePawnControlRotation))
  (Variables|/Game/USCS/Blueprints/SystemForCamera/BP_CameraBP.BP_CameraBP_C|SetInherittPitch _scenecamera (Variables|PARAMETERS:SceneCameraSetting:|GetInherit%20Pitch))
  (Variables|/Game/USCS/Blueprints/SystemForCamera/BP_CameraBP.BP_CameraBP_C|SetInherittYaw _scenecamera (Variables|PARAMETERS:SceneCameraSetting:|GetInherit%20Yaw))
  (Variables|/Game/USCS/Blueprints/SystemForCamera/BP_CameraBP.BP_CameraBP_C|SetInherittRoll _scenecamera (Variables|PARAMETERS:SceneCameraSetting:|GetInherit%20Roll))
  (Variables|/Game/USCS/Blueprints/SystemForCamera/BP_CameraBP.BP_CameraBP_C|SetCamera%20Spring%20Lag _scenecamera (Variables|PARAMETERS:SceneCameraLag:|GetEnable%20Camera%20Lag))
  (Variables|/Game/USCS/Blueprints/SystemForCamera/BP_CameraBP.BP_CameraBP_C|SetCamera%20Spring%20Lag%20Rotation _scenecamera (Variables|PARAMETERS:SceneCameraLag:|GetEnable%20Camera%20Rotation%20Lag))
  (Variables|/Game/USCS/Blueprints/SystemForCamera/BP_CameraBP.BP_CameraBP_C|SetCamera%20Spring%20Lag%20Speed _scenecamera (Variables|PARAMETERS:SceneCameraLag:|GetCamera%20Lag%20Speed))
  (Variables|/Game/USCS/Blueprints/SystemForCamera/BP_CameraBP.BP_CameraBP_C|SetCamera%20Spring%20Lag%20Rotation%20Speed _scenecamera (Variables|PARAMETERS:SceneCameraLag:|GetCamera%20Rotation%20Lag%20Speed))
  (Variables|/Game/USCS/Blueprints/SystemForCamera/BP_CameraBP.BP_CameraBP_C|SetCamera%20Lag%20Maxx%20Distance _scenecamera (Variables|PARAMETERS:SceneCameraLag:|GetCamera%20Lag%20Max%20Distance))
  (if (Variables|/Game/USCS/Blueprints/SystemForCamera/BP_CameraBP.BP_CameraBP_C|GetIsCameraInitiated? (Variables|PARAMETERS:|GetSceneCamera))
    (if (Variables|Default|GetPreviousZoneInfluWasA_UscsZoneInflu)
      (for (_array_element _array_index) (Variables|Default|GetUscsForCameraBP_Ref) :!label _label_2
        (if (Variables|BP_USCS_ForCameraBP_C|GetIsActivated? _array_element)
          (Variables|BP_USCS_ForCameraBP_C|SetCurrentUSCS_ForCameraBP_Index _array_element _array_index)
          (if (not (== (Variables|Default|GetCurrentUSCS_ForCameraBP_Index) (Variables|Default|GetPreviousUSCS_ForCameraBP_Index)))
            (if (Variables|PARAMETERS:|GetInstantCameraView%28NoBlend%29)
              (Default|BacktoCameraBP (Variables|PARAMETERS:|GetSceneCamera)))
            (for _array_element_2 (Variables|Default|GetUscsForCameraBP_Ref)
              (Variables|BP_USCS_ForCameraBP_C|SetPreviousUSCS_ForCameraBP_Index _array_element_2 (Variables|Default|GetCurrentUSCS_ForCameraBP_Index))))
          (else
            (Variables|BP_USCS_ForCameraBP_C|SetCurrentUSCS_ForCameraBP_Index _array_element -1)
            (Variables|BP_USCS_ForCameraBP_C|SetPreviousUSCS_ForCameraBP_Index _array_element -1))))
      (else
        (if (Variables|PARAMETERS:|GetIsGameStartCamera?) :!label _label_3
          (Utilities|FlowControl|Sequence
            (:then_0
              (Utilities|FlowControl|Delay 0.2)
              (Variables|PARAMETERS:|SetIsGameStartCamera? false))
            (:then_1
              (Default|BacktoCameraBP (Variables|PARAMETERS:|GetSceneCamera) :!label _label_4)
              (Variables|Default|SetPreviousZoneInfluWasA_UscsZoneInflu true)
              (goto _label_2)))
          (else
            (goto _label_4)))))
    (else
      (goto _label_3))))

(event EventBacktoCamera-StaticBP
  (Actor|Tick|SetActorTickEnabled false)
  (Variables|Default|SetPreviousZoneInfluWasA_UscsZoneInflu false)
  (Variables|Default|SetCurrentUSCS_OverlappedA "A")
  (Variables|Default|SetCurrentUSCS_OverlappedB "B")
  (Variables|Default|SetIsActivated? false))

(event EventBeginPlay
  (bind _scenecamera (Variables|PARAMETERS:|GetSceneCamera))
  (bind _splineraildepthon_ (Variables|PARAMETERS:|GetSplineRailDepthOn?))
  (bind _usefadein (Variables|PARAMETRS:FadeIn:|GetUseFadeIn))
  (Variables|Default|SetIs%20SwitchBP? false)
  (Utilities|FlowControl|Sequence
    (:then_0
      (Variables|Default|SetIsOverlappingBP_ZoneInfluencerActivator? false)
      (Actor|Tick|SetActorTickEnabled false)
      (Utilities|FlowControl|Sequence
        (:then_0
          (Utilities|FlowControl|Delay 0.0)
          (Variables|Default|SetIsInsideZoneInfluencer? (CallFunction|PlayerIsoverlappingOneZoneInfluencer))
          (if (Variables|Default|GetIsInsideZoneInfluencer?)
            (Variables|Default|SetPreviousZoneInfluWasA_UscsZoneInflu true)
            (bind _displayname (CallFunction|GetUSCSDisplayName))
            (Variables|Default|SetCurrentUSCS_OverlappedA _displayname)
            (Variables|Default|SetCurrentUSCS_OverlappedB _displayname)
            (Variables|Default|SetIsActivated? true)
            (Utilities|FlowControl|Sequence
              (:then_0
                (Actor|Tick|SetActorTickEnabled (or (or _splineraildepthon_ _usefadein) (and _splineraildepthon_ _usefadein)) :!label _label)
                (if (Variables|PARAMETRS:FadeIn:|GetUseFadeIn)
                  (if (Utilities|Enum|Equal(Enum) (Variables|Default|GetCurrentUSCS_OverlappedA) (Variables|Default|GetCurrentUSCS_OverlappedB))
                    (if (Variables|Default|GetIs%20SwitchBP?)
                      (bind _bc_fadeincamerabp (CallFunction|BCFadeinCameraParameters (Variables|PARAMETERS:|GetSceneCamera) (Variables|PARAMETRS:FadeIn:|GetUseFadeIn) (Variables|PARAMETRS:FadeIn:|GetDisable%20Player%20Input%20Controller) (Variables|PARAMETRS:FadeIn:|GetPre%20Fade%20Time) (Variables|PARAMETRS:FadeIn:|GetPre%20Fade%20Color) (Variables|PARAMETRS:FadeIn:|GetPre%20Fade%20Should%20Fade%20Audio) (Variables|PARAMETRS:FadeIn:|GetFade%20Time) (Variables|PARAMETRS:FadeIn:|GetFade%20Color) (Variables|PARAMETRS:FadeIn:|GetFade%20from%20Alpha%28X%29%20to%20Alpha%28Y%29) (Variables|PARAMETRS:FadeIn:|GetShould%20Fade%20Audio?) (Variables|PARAMETRS:FadeIn:|GetHold%20When%20Finished?) :!label _label_2))
                      (Default|BCFadeinSetting _bc_fadeincamerabp))
                    (else
                      (goto _label_2))))
                (Variables|/Game/USCS/Blueprints/SystemForCamera/BP_CameraBP.BP_CameraBP_C|SetSpline (Variables|PARAMETERS:|GetSceneCamera) (Variables|Default|GetCameraSpline))
                (Variables|/Game/USCS/Blueprints/SystemForCamera/BP_CameraBP.BP_CameraBP_C|SetIsStartGameCamera? _scenecamera (Variables|PARAMETERS:|GetIsGameStartCamera?))
                (Variables|/Game/USCS/Blueprints/SystemForCamera/BP_CameraBP.BP_CameraBP_C|SetInstantCameraView _scenecamera (Variables|PARAMETERS:|GetInstantCameraView%28NoBlend%29))
                (Variables|/Game/USCS/Blueprints/SystemForCamera/BP_CameraBP.BP_CameraBP_C|SetGameStartCameraBlendTime _scenecamera (Variables|PARAMETERS:|GetGame%20Start%20Camera%20Blend%20Time))
                (Variables|/Game/USCS/Blueprints/SystemForCamera/BP_CameraBP.BP_CameraBP_C|SetSnapCameraSpline? _scenecamera (Variables|PARAMETERS:|GetSnapCameraSpline?))
                (Variables|/Game/USCS/Blueprints/SystemForCamera/BP_CameraBP.BP_CameraBP_C|SetSnapCameraSplineDistance%20Offset _scenecamera (Variables|PARAMETERS:|GetSnapCameraSplineDistanceOffset))
                (Variables|/Game/USCS/Blueprints/SystemForCamera/BP_CameraBP.BP_CameraBP_C|SetInterpSpeedLocation _scenecamera (Variables|PARAMETERS:|GetInterp%20Speed%20Location))
                (Variables|/Game/USCS/Blueprints/SystemForCamera/BP_CameraBP.BP_CameraBP_C|SetInterpSpeedRotation _scenecamera (Variables|PARAMETERS:|GetInterp%20Speed%20Rotation))
                (Variables|/Game/USCS/Blueprints/SystemForCamera/BP_CameraBP.BP_CameraBP_C|SetLookAtPlayer? _scenecamera (Variables|PARAMETERS:|GetTrackingPlayer%28CameraRotation%29))
                (Variables|/Game/USCS/Blueprints/SystemForCamera/BP_CameraBP.BP_CameraBP_C|SetLookAtPlayerOffset _scenecamera (Variables|PARAMETERS:|GetTrackingPlayerOffset))
                (Variables|/Game/USCS/Blueprints/SystemForCamera/BP_CameraBP.BP_CameraBP_C|SetUseCameraOffset _scenecamera (Variables|PARAMETERS:|GetUseCameraOffset))
                (Variables|/Game/USCS/Blueprints/SystemForCamera/BP_CameraBP.BP_CameraBP_C|SetBlend%20TimeFromOtherCamera _scenecamera (Variables|PARAMETERS:|GetBlendTimeFromOtherCamera))
                (Variables|/Game/USCS/Blueprints/SystemForCamera/BP_CameraBP.BP_CameraBP_C|SetCameraOffset _scenecamera (Variables|PARAMETERS:|GetCameraOffset))
                (Variables|/Game/USCS/Blueprints/SystemForCamera/BP_CameraBP.BP_CameraBP_C|SetConstraintX,Y,Z_Rotation _scenecamera (Variables|PARAMETERS:|GetConstraint%20X,Y,Z%20Rotation))
                (Variables|/Game/USCS/Blueprints/SystemForCamera/BP_CameraBP.BP_CameraBP_C|SetAntiCameraJitter _scenecamera (Variables|PARAMETERS:SceneCameraSetting:|GetCameraAntiJitter))
                (Variables|/Game/USCS/Blueprints/SystemForCamera/BP_CameraBP.BP_CameraBP_C|SetDebugClampAngles? _scenecamera (Variables|PARAMETERS:|GetDebug%20Clamp%20Angles?))
                (Variables|/Game/USCS/Blueprints/SystemForCamera/BP_CameraBP.BP_CameraBP_C|SetCanControlCameraRotationV? _scenecamera (Variables|PARAMETERS:SceneCameraController:|GetCan%20Control%20Camera%20Rotation%20V?))
                (Variables|/Game/USCS/Blueprints/SystemForCamera/BP_CameraBP.BP_CameraBP_C|SetReverseAxisV? _scenecamera (Variables|PARAMETERS:SceneCameraController:|GetReverse%20Control%20Axis%20V?))
                (Variables|/Game/USCS/Blueprints/SystemForCamera/BP_CameraBP.BP_CameraBP_C|SetAngleMinV: _scenecamera (Variables|PARAMETERS:SceneCameraController:|GetAngle%20Min%20V:))
                (Variables|/Game/USCS/Blueprints/SystemForCamera/BP_CameraBP.BP_CameraBP_C|SetAngleMaxV: _scenecamera (Variables|PARAMETERS:SceneCameraController:|GetAngle%20Max%20V:))
                (Variables|/Game/USCS/Blueprints/SystemForCamera/BP_CameraBP.BP_CameraBP_C|SetCanControlCameraRotationH? _scenecamera (Variables|PARAMETERS:SceneCameraController:|GetCan%20Control%20Camera%20Rotation%20H?))
                (Variables|/Game/USCS/Blueprints/SystemForCamera/BP_CameraBP.BP_CameraBP_C|SetReverseAxisH? _scenecamera (Variables|PARAMETERS:SceneCameraController:|GetReverse%20Control%20Axis%20H?))
                (Variables|/Game/USCS/Blueprints/SystemForCamera/BP_CameraBP.BP_CameraBP_C|SetAngleMinH: _scenecamera (Variables|PARAMETERS:SceneCameraController:|GetAngle%20Min%20H:))
                (Variables|/Game/USCS/Blueprints/SystemForCamera/BP_CameraBP.BP_CameraBP_C|SetAngleMaxH: _scenecamera (Variables|PARAMETERS:SceneCameraController:|GetAngle%20Max%20H:))
                (Variables|/Game/USCS/Blueprints/SystemForCamera/BP_CameraBP.BP_CameraBP_C|SetClampX _scenecamera (Variables|PARAMETERS:|GetClampSlopeL/R))
                (Variables|/Game/USCS/Blueprints/SystemForCamera/BP_CameraBP.BP_CameraBP_C|SetClampY _scenecamera (Variables|PARAMETERS:|GetClampAngleDown/Up))
                (Variables|/Game/USCS/Blueprints/SystemForCamera/BP_CameraBP.BP_CameraBP_C|SetClampZ _scenecamera (- (Variables|PARAMETERS:|GetClampAngleL/R) 9e+01))
                (Variables|/Game/USCS/Blueprints/SystemForCamera/BP_CameraBP.BP_CameraBP_C|SetUsePawnControlRotationn _scenecamera (Variables|PARAMETERS:SceneCameraSetting:|GetUsePawnControlRotation))
                (Variables|/Game/USCS/Blueprints/SystemForCamera/BP_CameraBP.BP_CameraBP_C|SetInherittPitch _scenecamera (Variables|PARAMETERS:SceneCameraSetting:|GetInherit%20Pitch))
                (Variables|/Game/USCS/Blueprints/SystemForCamera/BP_CameraBP.BP_CameraBP_C|SetInherittYaw _scenecamera (Variables|PARAMETERS:SceneCameraSetting:|GetInherit%20Yaw))
                (Variables|/Game/USCS/Blueprints/SystemForCamera/BP_CameraBP.BP_CameraBP_C|SetInherittRoll _scenecamera (Variables|PARAMETERS:SceneCameraSetting:|GetInherit%20Roll))
                (Variables|/Game/USCS/Blueprints/SystemForCamera/BP_CameraBP.BP_CameraBP_C|SetCamera%20Spring%20Lag _scenecamera (Variables|PARAMETERS:SceneCameraLag:|GetEnable%20Camera%20Lag))
                (Variables|/Game/USCS/Blueprints/SystemForCamera/BP_CameraBP.BP_CameraBP_C|SetCamera%20Spring%20Lag%20Rotation _scenecamera (Variables|PARAMETERS:SceneCameraLag:|GetEnable%20Camera%20Rotation%20Lag))
                (Variables|/Game/USCS/Blueprints/SystemForCamera/BP_CameraBP.BP_CameraBP_C|SetCamera%20Spring%20Lag%20Speed _scenecamera (Variables|PARAMETERS:SceneCameraLag:|GetCamera%20Lag%20Speed))
                (Variables|/Game/USCS/Blueprints/SystemForCamera/BP_CameraBP.BP_CameraBP_C|SetCamera%20Spring%20Lag%20Rotation%20Speed _scenecamera (Variables|PARAMETERS:SceneCameraLag:|GetCamera%20Rotation%20Lag%20Speed))
                (Variables|/Game/USCS/Blueprints/SystemForCamera/BP_CameraBP.BP_CameraBP_C|SetCamera%20Lag%20Maxx%20Distance _scenecamera (Variables|PARAMETERS:SceneCameraLag:|GetCamera%20Lag%20Max%20Distance))
                (if (Variables|/Game/USCS/Blueprints/SystemForCamera/BP_CameraBP.BP_CameraBP_C|GetIsCameraInitiated? (Variables|PARAMETERS:|GetSceneCamera))
                  (if (Variables|Default|GetPreviousZoneInfluWasA_UscsZoneInflu)
                    (for (_array_element _array_index) (Variables|Default|GetUscsForCameraBP_Ref) :!label _label_3
                      (if (Variables|BP_USCS_ForCameraBP_C|GetIsActivated? _array_element)
                        (Variables|BP_USCS_ForCameraBP_C|SetCurrentUSCS_ForCameraBP_Index _array_element _array_index)
                        (if (not (== (Variables|Default|GetCurrentUSCS_ForCameraBP_Index) (Variables|Default|GetPreviousUSCS_ForCameraBP_Index)))
                          (if (Variables|PARAMETERS:|GetInstantCameraView%28NoBlend%29)
                            (Default|BacktoCameraBP (Variables|PARAMETERS:|GetSceneCamera)))
                          (for _array_element_2 (Variables|Default|GetUscsForCameraBP_Ref)
                            (Variables|BP_USCS_ForCameraBP_C|SetPreviousUSCS_ForCameraBP_Index _array_element_2 (Variables|Default|GetCurrentUSCS_ForCameraBP_Index))))
                        (else
                          (Variables|BP_USCS_ForCameraBP_C|SetCurrentUSCS_ForCameraBP_Index _array_element -1)
                          (Variables|BP_USCS_ForCameraBP_C|SetPreviousUSCS_ForCameraBP_Index _array_element -1))))
                    (else
                      (if (Variables|PARAMETERS:|GetIsGameStartCamera?) :!label _label_4
                        (Utilities|FlowControl|Sequence
                          (:then_0
                            (Utilities|FlowControl|Delay 0.2)
                            (Variables|PARAMETERS:|SetIsGameStartCamera? false))
                          (:then_1
                            (Default|BacktoCameraBP (Variables|PARAMETERS:|GetSceneCamera) :!label _label_5)
                            (Variables|Default|SetPreviousZoneInfluWasA_UscsZoneInflu true)
                            (goto _label_3)))
                        (else
                          (goto _label_5)))))
                  (else
                    (goto _label_4))))
              (:then_1
                (goto _label_5)))
            (else
              (Variables|Default|SetPreviousZoneInfluWasA_UscsZoneInflu false)
              (if (Variables|PARAMETERS:|GetIsGameStartCamera?)
                (Variables|Default|SetIsActivated? true)
                (goto _label)
                (else
                  (Variables|Default|SetIsActivated? false)
                  (for _array_element_3 (Variables|Default|GetUscsForCameraBP_Ref)
                    (Variables|BP_USCS_ForCameraBP_C|SetPreviousZoneInfluWasA_UscsZoneInflu _array_element_3 true)))))))
        (:then_1
          (bind _outactors (Actor|GetAllActorsOfClass "BP_USCS_ForCameraBP_C"))
          (Variables|Default|SetUscsForCameraBP_Ref _outactors))))
    (:then_1
      (for (_array_element_4 _array_index_2) (Variables|Default|GetUscsForCameraBP_Ref)
        (Variables|BP_USCS_ForCameraBP_C|SetCurrentUSCS_ForCameraBP_Index _array_element_4 _array_index_2)
        (Variables|BP_USCS_ForCameraBP_C|SetPreviousUSCS_ForCameraBP_Index _array_element_4 _array_index_2)))))

(event EventTick
  (params (DeltaSeconds :type Float%20%28single-precision%29))
  (Utilities|FlowControl|Sequence
    (:then_0
      (if (Variables|PARAMETERS:|GetSplineRailDepthOn?)
        (if (Variables|/Game/USCS/Blueprints/SystemForCamera/BP_CameraBP.BP_CameraBP_C|GetLookAtPlayer? (Variables|PARAMETERS:|GetSceneCamera))
          (Transformation|SetWorldLocation (Variables|Default|GetCameraSpline) (+ (Spline|FindLocationClosesttoWorldLocation (Variables|Default|GetSplineDepth) (Transformation|GetActorLocation (CallFunction|GetPlayerType(PawnorCharacter))) "World") (Variables|PARAMETERS:|GetSplineRailDepthDistance)) false false))))
    (:then_1
      (if (Variables|Default|GetPreviousZoneInfluWasA_UscsZoneInflu)
        (if (Variables|PARAMETRS:FadeIn:|GetUseFadeIn)
          (bind _displayname (CallFunction|GetUSCSDisplayName))
          (Variables|Default|SetCurrentUSCS_OverlappedA _displayname)
          (Variables|Default|SetCurrentUSCS_OverlappedB _displayname))
        (else
          (Variables|Default|SetCurrentUSCS_OverlappedA "A")
          (Variables|Default|SetCurrentUSCS_OverlappedB "B"))))))

(event EventBacktoCamera-CharacterBP
  (Actor|Tick|SetActorTickEnabled false)
  (Variables|Default|SetPreviousZoneInfluWasA_UscsZoneInflu false)
  (Variables|Default|SetCurrentUSCS_OverlappedA "A")
  (Variables|Default|SetCurrentUSCS_OverlappedB "B")
  (Variables|Default|SetIsActivated? false))

(fn ConstructionScript)

(fn PlayerIsoverlappingOneZoneInfluencer
  (bind _returnvalue (CallFunction|GetPlayerType(PawnorCharacter)))
  (return (or (Collision|IsOverlappingActor (Variables|Default|GetZoneInfluenceA) _returnvalue :!class /Script/Engine.PrimitiveComponent) (Collision|IsOverlappingActor (Variables|Default|GetZoneInfluenceB) _returnvalue :!class /Script/Engine.PrimitiveComponent))))

(fn GetUSCSDisplayName
  (bind _uscsforcamerabp_ref (Variables|Default|GetUscsForCameraBP_Ref))
  (for (_array_element _array_index) _uscsforcamerabp_ref
    (if (CallFunction|PlayerIsoverlappingOneZoneInfluencer _array_element)
      (return (Utilities|GetDisplayName (Utilities|Array|Get(acopy) _uscsforcamerabp_ref _array_index)) _array_index))))