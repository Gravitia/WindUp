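; BP_CollapseTruck is an interactive truck that tilts and collapses when the player character enters its trigger box.
; A timeline pitches the truck from its BeginPlay rotation to 10 degrees while shaking the camera every update.
; A delay started from those updates then enables physics on the truck and three pencil components and destroys a merged component.
; A second timeline for tipping further to 90 degrees is never run.
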(event OnComponentBeginOverlap(Box)
  (params (OverlappedComponent :type Primitive%20Component%20Object%20Reference) (OtherActor :type Actor%20Object%20Reference) (OtherComp :type Primitive%20Component%20Object%20Reference) (OtherBodyIndex :type Integer) (bFromSweep :type Boolean) (SweepResult :type Hit%20Result%20Structure%20%28by%20ref%29))
  (Utilities|Casting|CastToBP_CharacterPlayer OtherActor)
  (bind _rotation (Timeline|Timeline Play)
    (:Update
      (Transformation|SetRelativeRotation (Variables|Default|GetTruck) (Math|Rotator|MakeRotator 0.0 (.pitch (.rotation (Math|Transform|Lerp(Transform) (Math|Transform|MakeTransform "0, 0, 0" (Math|Rotator|MakeRotator 0.0 (.pitch (stale EventBeginPlay _output_get)) 0.0) "1.000000,1.000000,1.000000") (Math|Transform|MakeTransform "0, 0, 0" (Math|Rotator|MakeRotator 0.0 1e+01 0.0) "1.000000,1.000000,1.000000") _rotation))) 0.0) false false)
      (CameraShakes|StartCameraShake (Game|GetPlayerCameraManager 0) "/Game/01_Blueprint/Camera/BP_CameraShake.BP_CameraShake_C" 0.5 "CameraLocal" "0, 0, 0")
      (Utilities|FlowControl|Delay 5.0)
      (Physics|SetSimulatePhysics (Variables|Default|GetTruck) true)
      (Components|DestroyComponent (Variables|Default|GetMerge_F0CB2F15)))))

(event EventBeginPlay
  (bind _output_get (Variables|Default|SetTruckRotation (Transformation|GetWorldRotation (Variables|Default|GetTruck)))))

(fn ConstructionScript)