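; BP_HazardShooter is an interactive hazard emitter that repeatedly fires an actor of a configurable class from a target component.
; A looping timer, started on BeginPlay, spawns the actor at SpawnTarget along its forward vector and prints a debug message.
; Each spawn gets a random scale per axis, so proportions can be non-uniform.
; The Destroy_Area component destroys any BP_BlackholeHazard_02 that begins overlapping it.
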(event OnComponentBeginOverlap(Destroy_Area)
  (params (OverlappedComponent :type Primitive%20Component%20Object%20Reference) (OtherActor :type Actor%20Object%20Reference) (OtherComp :type Primitive%20Component%20Object%20Reference) (OtherBodyIndex :type Integer) (bFromSweep :type Boolean) (SweepResult :type Hit%20Result%20Structure%20%28by%20ref%29))
  (bind _asbp_blackhole_hazard_02 (Utilities|Casting|CastToBP_BlackholeHazard_02 OtherActor))
  (Actor|DestroyActor _asbp_blackhole_hazard_02))

(event Custom|Shoot
  (bind _scalemin (Variables|Default|GetScaleMin))
  (bind _scalemax (Variables|Default|GetScaleMax))
  (bind _spawntarget (Variables|Default|GetSpawnTarget))
  (bind _returnvalue (Math|Random|RandomFloatinRange _scalemin _scalemax))
  (Game|SpawnActorfromClass (Variables|Default|GetClass) (Math|Transform|MakeTransform (Transformation|GetWorldLocation _spawntarget) (Math|Conversions|RotationFromXVector (Math|Vector|GetForwardVector _spawntarget)) (Math|Vector|MakeVector _returnvalue _returnvalue _returnvalue)) "Undefined" "MultiplyWithRoot" 0 0)
  (Development|PrintText "Ball Shoot"))

(event EventBeginPlay
  (Utilities|Time|SetTimerbyEvent (delegate Custom|Shoot) (Variables|Default|GetLoop%20Delay) true))

(fn ConstructionScript)